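; BP_LightFixture01b_tunnel is a light fixture actor for the underground tunnel map that sets the color temperature of its PointLight.
; The construction script applies either a fixed Temperature or a random value within a min-max range.
; The random value can come from a seeded stream for repeatable results or from an unseeded roll.
; The event graph holds no runtime logic.
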(event `self.ReceiveTick`
  (params (DeltaSeconds :type "Float (single-precision)")))

(fn `UserConstructionScript`
  (bind _min_max_temperature_ (`self.Min Max Temperature `))
  (bind _max_temperature_ (`self.Max Temperature `))
  (if (`self.Use Random Temperature in Range`)
    (`LightComponent.SetTemperature` (`self.PointLight`) (`KismetMathLibrary.SelectFloat` (`KismetMathLibrary.RandomFloatInRangeFromStream` (`self.Seed`) _min_max_temperature_ _max_temperature_) (`KismetMathLibrary.RandomFloatInRange` _min_max_temperature_ _max_temperature_) (`self.Use Random Seed`)))
    (else
      (`LightComponent.SetTemperature` (`self.PointLight`) (`self.Temperature`)))))