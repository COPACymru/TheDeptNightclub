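; Configurable parent flashlight actor that can be switched on and off through TurnOn and TurnOff.
; Its construction script sets mesh and colors, attaches a point or spot light plus an optional second spot at lamp sockets, and builds an optional lens flare billboard.
; SetIntensity drives lights and emissive materials, optionally scaling spot brightness by inverse squared cone angle.
; The second light follows its own ON2 flag, and flare intensity is set only at construction.
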(event `TurnOn`
  (set `self.ON` true)
  (`self.Set Intensity`))

(event `TurnOff`
  (set `self.ON` false)
  (`self.Set Intensity`))

(fn `Set Cone Angle`
  (bind _light_source_1_spot (`self.Light Source 1_Spot`))
  (bind _outer_cone_angle (`self.Outer Cone Angle`))
  (if (not (`self.PointLight`))
    (`SpotLightComponent.SetOuterConeAngle` _light_source_1_spot _outer_cone_angle)
    (`SpotLightComponent.SetInnerConeAngle` _light_source_1_spot (* _outer_cone_angle (`self.Inner Cone Angle Multiplier`)))
    (`self.Set Intensity`)))

(fn `Set Intensity`
  (bind _light_source_2 (`self.Light Source 2`))
  (bind _intensity (`self.Intensity`))
  (bind _returnvalue (`KismetMathLibrary.Conv_BoolToDouble` (`self.ON`)))
  (bind _returnvalue_2 (* (`self.Intensity 2`) (`KismetMathLibrary.Conv_BoolToDouble` (`self.ON2`))))
  (`MeshComponent.SetScalarParameterValueOnMaterials` (`self.Static Mesh Flashlight`) "Emissive" (* (`self.Intensity`) (`self.Emissive Intensity Multiplier`) _returnvalue))
  (`LightComponent.SetIntensity` (select `bool` (`self.PointLight`) :`false` (`self.Light Source 1_Spot`) :`true` (`self.Light Source 1_Point`) :!type "PointLightComponent Object Reference") (* (select `bool` (and (`self.Intensity depends on Cone Angle`) (not (`self.PointLight`))) :`false` _intensity :`true` (* (/ _intensity (`KismetMathLibrary.Square` (`self.Outer Cone Angle`))) 2500.0)) _returnvalue))
  ;[1 1 1] Second Light
  (`/Engine/EditorBlueprintResources/StandardMacros.IsValid` _light_source_2
    (:`Is Valid`
      (`LightComponent.SetIntensity` _light_source_2 _returnvalue_2)
      (`MeshComponent.SetScalarParameterValueOnMaterials` (`self.Static Mesh Flashlight`) "Emissive2" (* _returnvalue_2 (`self.Emissive Intensity Multiplier`))))))

(fn `UserConstructionScript`
  (bind _static_mesh_flashlight (`self.Static Mesh Flashlight`))
  (bind _static_mesh_flashlight_2 (`self.Static Mesh Flashlight`))
  (bind _materialbillboard (`self.MaterialBillboard`))
  (bind _returnvalue (`KismetMathLibrary.Conv_ColorToLinearColor` (`self.Light Color`)))
  (`|ExecutionSequence`
    (:`then_0`
      ;[1 1 1] Set Mesh
      (`StaticMeshComponent.SetStaticMesh` _static_mesh_flashlight_2 (`self.Mesh`))
      (`MeshComponent.SetVectorParameterValueOnMaterials` _static_mesh_flashlight_2 "Color" (`KismetMathLibrary.Conv_LinearColorToVector` (`KismetMathLibrary.Conv_ColorToLinearColor` (`self.Color`))))
      (`MeshComponent.SetVectorParameterValueOnMaterials` _static_mesh_flashlight_2 "LightColor" (`KismetMathLibrary.Conv_LinearColorToVector` (`KismetMathLibrary.Conv_ColorToLinearColor` (`self.Light Color`))))
      (`PrimitiveComponent.SetCastShadow` (`self.Static Mesh Flashlight`) (`self.Mesh Cast Shadow`)))
    (:`then_1`
      ;[1 1 1] Add Light Source
      (`|ExecutionSequence`
        (:`then_0`
          (if (`self.PointLight`)
            (bind _returnvalue_2 (`AddComponent|NODE_AddPointLightComponent-0` :`bManualAttachment` true))
            (set `self.Light Source 1_Point` _returnvalue_2)
            (`SceneComponent.K2_AttachToComponent` _returnvalue_2 _static_mesh_flashlight "Lamp" "KeepRelative" "KeepRelative" "KeepRelative" true)
            (`LightComponent.SetLightColor` _returnvalue_2 _returnvalue true)
            (else
              (bind _returnvalue_3 (`AddComponent|NODE_AddSpotLightComponent-0`))
              (set `self.Light Source 1_Spot` _returnvalue_3)
              (`SceneComponent.K2_AttachToComponent` _returnvalue_3 _static_mesh_flashlight "Lamp" "KeepRelative" "KeepRelative" "KeepRelative" true)
              (`LightComponent.SetLightColor` _returnvalue_3 _returnvalue true)
              (`self.Set Cone Angle`)
              (`/Engine/EditorBlueprintResources/StandardMacros.IsValid` (`self.Spotlight Beam Texture`)
                (:`Is Valid`
                  (bind _returnvalue_4 (`KismetMaterialLibrary.CreateDynamicMaterialInstance` (`LightComponent.LightFunctionMaterial` _returnvalue_3)))
                  (`MaterialInstanceDynamic.SetTextureParameterValue` _returnvalue_4 "Texture" (`self.Spotlight Beam Texture`))
                  (`LightComponent.SetLightFunctionMaterial` _returnvalue_3 _returnvalue_4))
                (:`Is Not Valid`
                  (`LightComponent.SetLightFunctionMaterial` _returnvalue_3 null))))))
        (:`then_1`)))
    (:`then_2`
      (if (`self.Second Light`)
        (bind _returnvalue_5 (`AddComponent|NODE_AddSpotLightComponent-1`))
        (bind _output_get (set `self.Light Source 2` _returnvalue_5))
        (`SceneComponent.K2_AttachToComponent` _output_get (`self.Static Mesh Flashlight`) "Lamp2" "KeepRelative" "KeepRelative" "KeepRelative" true)
        (`LightComponent.SetLightColor` _output_get (`KismetMathLibrary.Conv_ColorToLinearColor` (`self.Light Color`)) true)))
    (:`then_3`
      (`self.Set Intensity`))
    (:`then_4`
      (if (`self.LensFlare`)
        (bind _returnvalue_6 (`KismetMaterialLibrary.CreateDynamicMaterialInstance` "/Game/MainMenuLevelAssets/Flashlights_Pack/Materials/M_Flashlight_LensFlare_b.M_Flashlight_LensFlare_b"))
        (set `self.Flare_Material` _returnvalue_6)
        (`MaterialInstanceDynamic.SetVectorParameterValue` _returnvalue_6 "LightColor" (`KismetMathLibrary.Conv_ColorToLinearColor` (`self.Light Color`)))
        (`MaterialInstanceDynamic.SetScalarParameterValue` _returnvalue_6 "Intensity" (* (`self.Intensity`) (`self.Emissive Intensity Multiplier`) (`KismetMathLibrary.Conv_BoolToDouble` (`self.ON`)) (`self.Flare Intensity`)))
        (`PrimitiveComponent.SetMaterial` _materialbillboard 0 _returnvalue_6)
        (else
          (`ActorComponent.K2_DestroyComponent` _materialbillboard))))))