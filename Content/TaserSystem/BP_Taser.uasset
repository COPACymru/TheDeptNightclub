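; Taser weapon actor that fires wired probes, tases actors carrying a TaserSystem component, and toggles a flashlight and red lights.
; FireTaser predicts a dropping projectile path, then attaches two cable wires to the hit component or a spawned BP_MissedShot.
; StopTasing releases the target, clears wires and sound, and requires a reload.
; A looping timeline flashes the bottom light until fired, and restarts on reload.
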(event `self.ReceiveBeginPlay`
  (`self.Flash Light`))

(event `Flash Light`
  ;[1 1 1] Flash the bottom red light
  (bind (_direction _flash_track) (`Timeline|Timeline_0` :!via `PlayFromStart` :!label _label)
    (:`Update`
      (`LightComponent.SetIntensity` (`self.Bottom Light`) _flash_track))
    (:`Finished`
      (if (`self.ShouldFlash?`)
        (goto _label :!via `PlayFromStart`)))))

(event `Fire Taser`
  (bind _firing_ref (`self.Firing REF`))
  ;[1 1 1] Only shoot if there is a cartridge
  (if (not (`self.NeedsReloading?`))
    ;[1 1 1] Spawn taser loop SFX
    (bind _returnvalue (`GameplayStatics.SpawnSoundAttached` "/Game/TaserSystem/SFX/Taser_Loop_Cue.Taser_Loop_Cue" (`self.Taser`) "None" (0.0 0.0 0.0) (struct) "KeepRelativeOffset" false 1.0 1.0 0.0 null null))
    (set `self.Taser Loop` _returnvalue)
    (set `self.ShouldFlash?` false)
    ;[1 1 1] Calculate projectile drop (TIP: MODIFY THE SPEED VARIABLE TO CHANGE THE DROP | SET "DRAW DEBUG TYPE" TO "FOR DURATION" TO SEE IT IN-GAME
    (bind (_predictresult _returnvalue_2) (`GameplayStatics.Blueprint_PredictProjectilePath_Advanced` (make `PredictProjectilePathParams` :`StartLocation` (`SceneComponent.K2_GetComponentLocation` _firing_ref) :`LaunchVelocity` (* (`SceneComponent.GetForwardVector` _firing_ref) (`self.Speed`)) :`bTraceWithCollision` true :`MaxSimTime` 10.0 :`TraceChannel` "ECC_Visibility" :`ActorsToIgnore` (`|MakeArray` self :!type "Actor Object Reference") :`SimFrequency` 250.0)))
    ;[1 1 1] Only tase actors that contain the "Taser System" component
    (if _returnvalue_2
      (bind (_bblockinghit _binitialoverlap _time _distance _location _impactpoint _normal _impactnormal _physmat _hitactor _hitcomponent _hitbonename) (`GameplayStatics.BreakHitResult` (`.HitResult` (break `PredictProjectilePathResult` _predictresult))))
      (`/Engine/EditorBlueprintResources/StandardMacros.IsValid` _hitactor
        (:`Is Valid`
          (bind _returnvalue_3 (`self.GetComponentByClass` _hitactor "/Game/TaserSystem/TaserSystem.TaserSystem_C"))
          (`/Engine/EditorBlueprintResources/StandardMacros.IsValid` _returnvalue_3
            (:`Is Valid`
              (set `self.Target` _returnvalue_3) ; Set the actor to the target that is being tased
              ;[1 1 1] Attach the wire
              (bind _returnvalue_4 (`AddComponent|NODE_AddCableComponent-2` :`RelativeTransform` (`KismetMathLibrary.MakeTransform` (6.1 1.8 0.6))))
              (bind _output_get (set `self.Wire 1` _returnvalue_4))
              (`CableComponent.SetAttachEndToComponent` _output_get _hitcomponent _hitbonename)
              (bind _returnvalue_5 (`AddComponent|NODE_AddCableComponent-3` :`RelativeTransform` (`KismetMathLibrary.MakeTransform` (6.1 1.8 3.6))))
              (bind _output_get_2 (set `self.Wire 2` _returnvalue_5))
              (`CableComponent.SetAttachEndToComponent` _output_get_2 _hitcomponent _hitbonename)
              (`/Game/TaserSystem/TaserSystem.Be Tased` (`self.Target`)))
            (:`Is Not Valid`
              ;[1 1 1] Attach the wire to a missed shot (The taser didn't hit an actor with the "TaserSystem" component
              (bind _returnvalue_6 (`|SpawnActorFromClass` "/Game/TaserSystem/BP_MissedShot.BP_MissedShot_C" (`KismetMathLibrary.MakeTransform` _location) "Undefined" "OverrideRootScale" null null))
              (set `self.MissedShot REF` _returnvalue_6)
              (bind _returnvalue_7 (`AddComponent|NODE_AddCableComponent-4` :`RelativeTransform` (`KismetMathLibrary.MakeTransform` (6.1 1.8 0.6))))
              (bind _output_get_3 (set `self.Wire 1` _returnvalue_7))
              (`CableComponent.SetAttachEndTo` _output_get_3 (`self.MissedShot REF`) "None" "None")
              (bind _returnvalue_8 (`AddComponent|NODE_AddCableComponent-5` :`RelativeTransform` (`KismetMathLibrary.MakeTransform` (6.1 1.8 3.6))))
              (bind _output_get_4 (set `self.Wire 2` _returnvalue_8))
              (`CableComponent.SetAttachEndTo` _returnvalue_8 (`self.MissedShot REF`) "None" "None")
              (set `CableComponent.EndLocation` (0.0 0.0 15.0) _output_get_4))))))))

(event `Turn On Flashlight`
  ;[1 1 1] Flashlight on/off
  (`SceneComponent.SetVisibility` (`self.Flashlight`) true false))

(event `Turn On Red Lights`
  ;[1 1 1] Red lights on/off
  (`SceneComponent.SetVisibility` (`self.Top Light`) true false)
  (`SceneComponent.SetVisibility` (`self.Bottom Light`) true false))

(event `Turn Off Flashlight`
  ;[1 1 1] Flashlight on/off
  (`SceneComponent.SetVisibility` (`self.Flashlight`) false false))

(event `Turn Off Red Lights`
  ;[1 1 1] Red lights on/off
  (`SceneComponent.SetVisibility` (`self.Top Light`) false false)
  (`SceneComponent.SetVisibility` (`self.Bottom Light`) false false))

(event `Stop Tasing`
  ;[1 1 1] Stop tasing
  (if (not (`self.NeedsReloading?`))
    (set `self.NeedsReloading?` true)
    (bind _taser_loop (`self.Taser Loop`)
      (:`then`
        (`AudioComponent.Stop` _taser_loop))
      (:`else`
        _))
    (bind _target (`self.Target`)
      (:`then`
        (`/Game/TaserSystem/TaserSystem.Stop Being Tased` _target)
        (set `self.Target` null))
      (:`else`
        _))
    (bind _wire_1 (`self.Wire 1`)
      (:`then`
        (`ActorComponent.K2_DestroyComponent` _wire_1)
        (`ActorComponent.K2_DestroyComponent` (`self.Wire 2`))
        (set `self.Wire 1` null)
        (set `self.Wire 2` null)
        (bind _missedshot_ref (`self.MissedShot REF`)
          (:`then`
            (`self.K2_DestroyActor` _missedshot_ref))
          (:`else`)))
      (:`else`))))

(event `Reload Taser`
  ;[1 1 1] Reload
  ;;[1 1 1] Only reload if there isn't a cartridge
  (if (`self.NeedsReloading?`)
    (set `self.NeedsReloading?` false)
    (set `self.ShouldFlash?` true)
    (`self.Flash Light`)))

(fn `UserConstructionScript`
  (bind _flashlight (`self.Flashlight`))
  (bind _top_light (`self.Top Light`))
  (`|ExecutionSequence`
    (:`then_0`
      ;[1 1 1] Toggle red lights
      (if (`self.HaveRedLights?`)
        (`SceneComponent.SetHiddenInGame` _top_light false false)
        (`SceneComponent.SetHiddenInGame` (`self.Bottom Light`) false false)
        (else
          (`SceneComponent.SetHiddenInGame` _top_light true false)
          (`SceneComponent.SetHiddenInGame` (`self.Bottom Light`) true false))))
    (:`then_1`
      ;[1 1 1] Toggle flashlight
      (if (`self.HaveFlashlight?`)
        (`SceneComponent.SetHiddenInGame` _flashlight false false)
        (else
          (`SceneComponent.SetHiddenInGame` _flashlight true false))))))