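; BP_Door is an interactable door in the QA interrogation room that swings open and closed.
; Interact toggles the closed state, records that the door has been opened and plays the same sound cue either way.
; A timeline drives the door's relative yaw, playing forward to open and reversing to close.
; Box overlaps show or hide a prompt widget and call SetInteractionTypeMessage on the overlapping actor, passing true on both enter and exit.
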(event `Open Door`
  (bind (_direction _door_track) (`Timeline|Open Door T` :!label _label)
    (:`Update`
      (`SceneComponent.K2_SetRelativeRotation` (`self.Door`) (`KismetMathLibrary.MakeRotator` 0.0 0.0 _door_track) false false))))

(event `Close Door`
  (goto _label :!via `Reverse`))

(event `self.Box.OnComponentBeginOverlap`
  (params (OverlappedComponent :type "PrimitiveComponent Object Reference") (OtherActor :type "Actor Object Reference") (OtherComp :type "PrimitiveComponent Object Reference") (OtherBodyIndex :type Integer) (bFromSweep :type Boolean) (SweepResult :type "HitResult Structure (by ref)"))
  (message `/Game/GameFiles/GameBlueprints/InteractInterface.Set Interaction Type` OtherActor true)
  (`SceneComponent.SetVisibility` (`self.Widget`) true false))

(event `self.Box.OnComponentEndOverlap`
  (params (OverlappedComponent :type "PrimitiveComponent Object Reference") (OtherActor :type "Actor Object Reference") (OtherComp :type "PrimitiveComponent Object Reference") (OtherBodyIndex :type Integer))
  (message `/Game/GameFiles/GameBlueprints/InteractInterface.Set Interaction Type` OtherActor true)
  (`SceneComponent.SetVisibility` (`self.Widget`) false false))

(fn `Interact`
  (params (Interactor :type "Character Object Reference") (`Camera Trans Time` :type "Float (double-precision)"))
  (returns (`Did Interact?` :type Boolean))
  (if (`self.Door Closed`)
    (`self.Open Door`)
    (set `self.Door Closed` false)
    (set `self.BeenOpened?` true)
    (else
      (`self.Close Door`)
      (set `self.Door Closed` true)))
  (`GameplayStatics.PlaySoundAtLocation` "/Game/GameFiles/SFX/DoorOpen_Cue.DoorOpen_Cue" (`self.K2_GetActorLocation`) (struct) 1.0 1.0 0.0 null null null null)
  (return false))

(fn `UserConstructionScript`)