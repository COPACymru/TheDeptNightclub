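; Barmaid NPC, apparently Shannon, who offers a single conversation through an interaction.
; BeginPlay adds a SpeakToShannon prompt widget to the viewport, while a sphere overlap toggles a separate widget component and sets the player's interaction message on entry.
; Interact starts the dialogue component's conversation and hides that widget component.
; All of this except widget creation is gated by CanTalk, which clears when the conversation ends.
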(event `self.ReceiveBeginPlay`
  (bind _returnvalue (`|CreateWidget` "/Game/GameFiles/UI/Prompts/SpeakToShannon.SpeakToShannon_C"))
  (bind _output_get (set `self.Prompt Widget` _returnvalue))
  (`UserWidget.AddToViewport` _output_get 0))

(event `self.Sphere.OnComponentBeginOverlap`
  (params (OverlappedComponent :type "PrimitiveComponent Object Reference") (OtherActor :type "Actor Object Reference") (OtherComp :type "PrimitiveComponent Object Reference") (OtherBodyIndex :type Integer) (bFromSweep :type Boolean) (SweepResult :type "HitResult Structure (by ref)"))
  (if (`self.CanTalk?`)
    (message `/Game/GameFiles/GameBlueprints/InteractInterface.Set Interaction Type` (`GameplayStatics.GetPlayerCharacter` 0) true)
    (`SceneComponent.SetVisibility` (`self.Widget`) true false)))

(event `self.Sphere.OnComponentEndOverlap`
  (params (OverlappedComponent :type "PrimitiveComponent Object Reference") (OtherActor :type "Actor Object Reference") (OtherComp :type "PrimitiveComponent Object Reference") (OtherBodyIndex :type Integer))
  (if (`self.CanTalk?`)
    (`SceneComponent.SetVisibility` (`self.Widget`) false false)))

(event `/Game/GameFiles/DialogueSystemV2/BPI_DialougeComponentV2.On Conversation End`
  (set `self.CanTalk?` false))

(fn `Interact`
  (params (Interactor :type "Character Object Reference") (`Camera Trans Time` :type "Float (double-precision)"))
  (returns (`Did Interact?` :type Boolean))
  (if (`self.CanTalk?`)
    (`/Game/GameFiles/DialogueSystemV2/DialogueComponentV2.Start Conversation` (`self.DialogueComponentV2`) 0.0)
    (`SceneComponent.SetVisibility` (`self.Widget`) false false)
    (return true)))

(fn `UserConstructionScript`)