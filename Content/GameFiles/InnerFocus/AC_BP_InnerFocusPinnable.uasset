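; Actor component for pinnable objects in InnerFocus that keeps cable ends attached to its owner's pin point.
; Each tick it sets every valid cable in Pins to end at the owner's location plus RelativePinLocation, converted into BP_IF_MasterBoard's local space.
; An invalid entry is removed and ends that tick's loop.
; PlaceCable applies the same attachment to a given cable, relative to a supplied target actor.
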(event `self.ReceiveTick`
  (params (DeltaSeconds :type "Float (single-precision)"))
  (bind _pins (`self.Pins`))
  (for (_array_element _array_index) _pins
    (`/Engine/EditorBlueprintResources/StandardMacros.IsValid` _array_element
      (:`Is Valid`
        (bind _returnvalue (`GameplayStatics.GetActorOfClass` "/Game/GameFiles/InnerFocus/BP_IF_MasterBoard.BP_IF_MasterBoard_C"))
        (set `CableComponent.EndLocation` (`KismetMathLibrary.InverseTransformLocation` (`Actor.GetTransform` _returnvalue) (+ (`Actor.K2_GetActorLocation` (`self.GetOwner`)) (`self.RelativePinLocation`))) _array_element)
        (set `CableComponent.bAttachEnd` true _array_element))
      (:`Is Not Valid`
        (`KismetArrayLibrary.Array_Remove` _pins _array_index)
        (break)))))

(fn `Place Cable`
  (params (`Cable Ref` :type "CableComponent Object Reference") (Target :type "Actor Object Reference"))
  (set `CableComponent.EndLocation` (`KismetMathLibrary.InverseTransformLocation` (`Actor.GetTransform` Target) (+ (`Actor.K2_GetActorLocation` (`self.GetOwner`)) (`self.RelativePinLocation`))) `Cable Ref`)
  (set `CableComponent.bAttachEnd` true `Cable Ref`))