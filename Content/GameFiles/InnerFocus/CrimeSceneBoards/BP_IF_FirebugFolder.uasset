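; Firebug case folder actor on the Inner Focus crime scene board that owns the Firebug evidence list widget, created on BeginPlay.
; Escape hides the folder and list, then hands visibility and input to the evidence folder (full version, with optional note or pin tutorial) or master board (tech demo).
; The master board path also reloads evidence, shows polaroids and text, and re-enables camera movement.
; Left click traces for evidence folder components but triggers nothing.
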(event `self.ReceiveBeginPlay`
  ;[1 1 1] Create evidence list
  (bind _returnvalue (`|CreateWidget` "/Game/GameFiles/InnerFocus/UI/W_IF_EvidenceListFIREBUG.W_IF_EvidenceListFIREBUG_C"))
  (set `self.Evidence List` _returnvalue)
  (`GameplayStatics.SetViewportMouseCaptureMode` "CapturePermanently_IncludingInitialMouseDown"))

(event `Key|LeftMouseButton`
  (params (Key :type "Key Structure"))
  (bind (_worldlocation _worlddirection) (`PlayerController.DeprojectMousePositionToWorld` (`GameplayStatics.GetPlayerController` 0)))
  ;[1 1 1] Click on screen
  (:`Pressed`
    (if (`self.CanClick?`)
      (bind (_outhit _returnvalue) (`KismetSystemLibrary.LineTraceSingle` :`Start` _worldlocation :`End` (+ _worldlocation (* _worlddirection 2000.0)) :`TraceChannel` "TraceTypeQuery1" :`bIgnoreSelf` false))
      (if _returnvalue
        (if (`KismetStringLibrary.Contains` (`KismetSystemLibrary.GetDisplayName` (`.HitComponent` (`GameplayStatics.BreakHitResult` _outhit))) "Evidence_Folder")
          _)))))

(event `Key|Escape`
  (params (Key :type "Key Structure"))
  (bind _returnvalue (`GameplayStatics.GetPlayerController` 0))
  (bind _returnvalue_2 (`GameplayStatics.GetPlayerController` 0))
  (bind _returnvalue_3 (`GameplayStatics.GetGameInstance`))
  (bind _evidence_list (`self.Evidence List`))
  (bind _evidence_list_2 (`self.Evidence List`))
  (:`Pressed`
    (bind _game_version (message `/Game/GameFiles/GameBlueprints/BPI_GameInstance.Get Game Version` (`GameplayStatics.GetGameInstance`)))
    ;[1 1 1] Open evidence folder
    (switch `/Game/GameFiles/GameBlueprints/GameVersionEnum` _game_version
      (:`NewEnumerator0`
        (`GameplayStatics.GetActorOfClass` "/Game/GameFiles/InnerFocus/BP_IF_MasterBoard.BP_IF_MasterBoard_C")
        (bind _returnvalue_4 (`GameplayStatics.GetActorOfClass` "/Game/GameFiles/InnerFocus/BP_IF_EvidenceFolder.BP_IF_EvidenceFolder_C"))
        (`self.SetActorHiddenInGame` _returnvalue_4 false)
        (`self.SetActorHiddenInGame` true)
        (`self.EnableInput` _returnvalue_4 _returnvalue)
        (`self.DisableInput` self _returnvalue)
        (`Widget.RemoveFromParent` _evidence_list_2)
        (`Widget.SetVisibility` (`/Game/GameFiles/InnerFocus/UI/W_IF_EvidenceListFIREBUG.EvidenceInfoBox` _evidence_list_2) "Hidden")
        (`WidgetBlueprintLibrary.SetInputMode_GameOnly` (`GameplayStatics.GetPlayerController` 0))
        (`GameplayStatics.SetViewportMouseCaptureMode` "CapturePermanently_IncludingInitialMouseDown")
        ;[1 1 1] Add note and/or pin tutorials
        (bind _should_play_if_note_tut_ (message `/Game/GameFiles/GameBlueprints/BPI_GameInstance.Get Should Play IF Note Tut` _returnvalue_3))
        (if _should_play_if_note_tut_
          (bind _returnvalue_5 (`|CreateWidget` "/Game/GameFiles/InnerFocus/UI/W_IF_NoteTut.W_IF_NoteTut_C"))
          (`UserWidget.AddToViewport` _returnvalue_5 0)
          (else
            (bind _should_play_if_pin_tut (message `/Game/GameFiles/GameBlueprints/BPI_GameInstance.Get Should Play IF Pin Tut` _returnvalue_3))
            (if _should_play_if_pin_tut
              (bind _returnvalue_6 (`|CreateWidget` "/Game/GameFiles/InnerFocus/UI/W_IF_PinTut.W_IF_PinTut_C"))
              (`UserWidget.AddToViewport` _returnvalue_6 0)))))
      (:`NewEnumerator3`
        ;[1 1 1] Open master board
        (bind _returnvalue_7 (`GameplayStatics.GetActorOfClass` "/Game/GameFiles/InnerFocus/BP_IF_MasterBoard.BP_IF_MasterBoard_C"))
        (`/Game/GameFiles/InnerFocus/BP_IF_MasterBoard.Clear Evidence On Board` _returnvalue_7)
        (`/Game/GameFiles/InnerFocus/BP_IF_MasterBoard.Load Evidence On Board` _returnvalue_7)
        (`self.SetActorHiddenInGame` _returnvalue_7 false)
        (`self.SetActorHiddenInGame` true)
        (`/Game/GameFiles/InnerFocus/BP_IF_MasterBoard.Show Polaroids` _returnvalue_7)
        (bind _returnvalue_8 (`GameplayStatics.GetActorOfClass` "/Game/GameFiles/InnerFocus/BP_InnerFocusComponent.BP_InnerFocusComponent_C"))
        (set `/Game/GameFiles/InnerFocus/BP_InnerFocusComponent.CanMoveCamera?` true _returnvalue_8)
        (bind _outactors (`GameplayStatics.GetAllActorsOfClass` "/Game/GameFiles/InnerFocus/Evidence/BP_IF_Text.BP_IF_Text_C"))
        (for _array_element _outactors
          (`self.SetActorHiddenInGame` _array_element false))
        (`self.EnableInput` _returnvalue_7 _returnvalue_2)
        (`self.DisableInput` self _returnvalue_2)
        (`Widget.RemoveFromParent` _evidence_list)
        (`Widget.SetVisibility` (`/Game/GameFiles/InnerFocus/UI/W_IF_EvidenceListFIREBUG.EvidenceInfoBox` _evidence_list) "Hidden")
        (`WidgetBlueprintLibrary.SetInputMode_GameOnly` (`GameplayStatics.GetPlayerController` 0))
        (`GameplayStatics.SetViewportMouseCaptureMode` "CapturePermanently_IncludingInitialMouseDown")))))

(fn `UserConstructionScript`)