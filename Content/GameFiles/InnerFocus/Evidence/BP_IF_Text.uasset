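; Sticky note actor in the InnerFocus Evidence set that displays wrapped text on a post-it mesh.
; On BeginPlay it tints the note material with its Colour and randomly picks a flat or bent mesh.
; WrapText splits InputText by character count, regardless of word boundaries, into up to seven line variables.
; After a short delay, it combines those lines through FormatText and sets the TextRender.
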(event `self.ReceiveBeginPlay`
  (bind (_colour_r _colour_g _colour_b) (break `LinearColor` (`self.Colour`)))
  ;[1 1 1] Set sticky note colour and if bent or not
  (`MeshComponent.SetVectorParameterValueOnMaterials` (`self.Note`) "Colour" (`KismetMathLibrary.MakeVector` _colour_r _colour_g _colour_b))
  (`StaticMeshComponent.SetStaticMesh` (`self.Note`) (select `bool` (`KismetMathLibrary.RandomBool`) :`false` "/Game/GameFiles/InnerFocus/Evidence/Mesh/Postit_Note_Clean.Postit_Note_Clean" :`true` "/Game/GameFiles/InnerFocus/Evidence/Mesh/Postit_Note_Clean_Bent.Postit_Note_Clean_Bent" :!type "StaticMesh Object Reference")))

(event `Wrap Text`
  (bind _temp_line (`self.Temp Line`))
  (bind _temp_line_2 (`self.Temp Line`))
  ;[1 1 1] Auto-wrap text in notes
  ; Total of 119 characters, over 7 lines with 17 characters in each line
  (for _array_element (`KismetStringLibrary.GetCharacterArrayFromString` (`KismetTextLibrary.Conv_TextToString` (`self.Input Text`)))
    (`/Engine/EditorBlueprintResources/StandardMacros.IncrementInt` (`self.Current Character`)
      (:`  `
        (if (== (`self.Total Characters`) 253)
          (break)
          (else
            (set `self.Temp Line` (`KismetStringLibrary.Concat_StrStr` (`self.Temp Line`) _array_element))
            (if (== (`self.Current Character`) 23)
              (set `self.Current Character` 0)
              (bind _result (`/Engine/EditorBlueprintResources/StandardMacros.IncrementInt` (`self.Current Line`) :!label _label)
                (:`  `
                  (switch `int` _result
                    (:`0`
                      (set `self.Line 0` _temp_line_2))
                    (:`1`
                      (set `self.Line 1` _temp_line_2))
                    (:`2`
                      (set `self.Line 2` _temp_line_2))
                    (:`3`
                      (set `self.Line 3` _temp_line_2))
                    (:`4`
                      (set `self.Line 4` _temp_line))
                    (:`5`
                      (set `self.Line 5` _temp_line))
                    (:`6`
                      (set `self.Line 6` _temp_line)))
                  (set `self.Temp Line` "")))))))))
  (`|ExecutionSequence`
    (:`then_0`
      (goto _label))
    (:`then_1`
      (`KismetSystemLibrary.Delay` 0.2)
      (`TextRenderComponent.K2_SetText` (`self.TextRender`) (`|FormatText` "{Line 0} \n{Line 1} \n{Line 2} \n{Line 3} \n{Line 4} \n{Line 5} \n{Line 6}" (`self.Line 0`) (`self.Line 1`) (`self.Line 2`) (`self.Line 3`) (`self.Line 4`) (`self.Line 5`) (`self.Line 6`))))))

(fn `UserConstructionScript`)