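; Evidence folder screen actor in the Inner Focus board system, where clicking a case folder opens its evidence view.
; Left click traces from the cursor and, when the hit component is named Firebug Folder, shows BP_IF_FirebugFolder with its evidence list widget.
; Escape returns to BP_IF_MasterBoard, reloading its evidence, unhiding text actors and showing any pending note or pin tutorial.
; Screens switch by toggling actor visibility and input.
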(event `self.ReceiveBeginPlay`
  (`GameplayStatics.SetViewportMouseCaptureMode` "CapturePermanently_IncludingInitialMouseDown"))

(event `Key|LeftMouseButton`
  (params (Key :type "Key Structure"))
  (bind (_worldlocation _worlddirection) (`PlayerController.DeprojectMousePositionToWorld` (`GameplayStatics.GetPlayerController` 0)))
  ;[1 1 1] Click on screen
  (:`Pressed`
    (if (`self.CanClick?`)
      (bind (_outhit _returnvalue) (`KismetSystemLibrary.LineTraceSingle` :`Start` _worldlocation :`End` (+ _worldlocation (* _worlddirection 2000.0)) :`TraceChannel` "TraceTypeQuery1" :`bIgnoreSelf` false))
      (if _returnvalue
        (if (`KismetStringLibrary.Contains` (`KismetSystemLibrary.GetDisplayName` (`.HitComponent` (`GameplayStatics.BreakHitResult` _outhit))) "Firebug Folder")
          (`self.Open Firebug Folder`))))))

(event `Key|Escape`
  (params (Key :type "Key Structure"))
  (bind _returnvalue (`GameplayStatics.GetPlayerController` 0))
  (bind _returnvalue_2 (`GameplayStatics.GetGameInstance`))
  ;[1 1 1] Open master board
  (:`Pressed`
    (bind _returnvalue_3 (`GameplayStatics.GetActorOfClass` "/Game/GameFiles/InnerFocus/BP_IF_MasterBoard.BP_IF_MasterBoard_C"))
    (`/Game/GameFiles/InnerFocus/BP_IF_MasterBoard.Clear Evidence On Board` _returnvalue_3)
    (`/Game/GameFiles/InnerFocus/BP_IF_MasterBoard.Load Evidence On Board` _returnvalue_3)
    (`self.SetActorHiddenInGame` _returnvalue_3 false)
    (`self.SetActorHiddenInGame` true)
    (`self.EnableInput` _returnvalue_3 _returnvalue)
    (`self.DisableInput` self _returnvalue)
    (bind _outactors (`GameplayStatics.GetAllActorsOfClass` "/Game/GameFiles/InnerFocus/Evidence/BP_IF_Text.BP_IF_Text_C"))
    (for _array_element _outactors
      (`self.SetActorHiddenInGame` _array_element false))
    ;[1 1 1] Add note and/or pin tutorials
    (bind _should_play_if_note_tut_ (message `/Game/GameFiles/GameBlueprints/BPI_GameInstance.Get Should Play IF Note Tut` _returnvalue_2))
    (if _should_play_if_note_tut_
      (bind _returnvalue_4 (`|CreateWidget` "/Game/GameFiles/InnerFocus/UI/W_IF_NoteTut.W_IF_NoteTut_C"))
      (`UserWidget.AddToViewport` _returnvalue_4 0)
      (else
        (bind _should_play_if_pin_tut (message `/Game/GameFiles/GameBlueprints/BPI_GameInstance.Get Should Play IF Pin Tut` _returnvalue_2))
        (if _should_play_if_pin_tut
          (bind _returnvalue_5 (`|CreateWidget` "/Game/GameFiles/InnerFocus/UI/W_IF_PinTut.W_IF_PinTut_C"))
          (`UserWidget.AddToViewport` _returnvalue_5 0))))))

(event `Open Firebug Folder`
  (bind _returnvalue (`GameplayStatics.GetPlayerController` 0))
  ;[1 1 1] Open evidence board
  (`GameplayStatics.GetActorOfClass` "/Game/GameFiles/InnerFocus/BP_IF_MasterBoard.BP_IF_MasterBoard_C")
  (bind _returnvalue_2 (`GameplayStatics.GetActorOfClass` "/Game/GameFiles/InnerFocus/CrimeSceneBoards/BP_IF_FirebugFolder.BP_IF_FirebugFolder_C"))
  (`self.SetActorHiddenInGame` _returnvalue_2 false)
  (`self.SetActorHiddenInGame` true)
  (`self.EnableInput` _returnvalue_2 _returnvalue)
  (`self.DisableInput` self _returnvalue)
  (bind _evidence_list (`/Game/GameFiles/InnerFocus/CrimeSceneBoards/BP_IF_FirebugFolder.Evidence List` _returnvalue_2))
  (`UserWidget.AddToViewport` _evidence_list 0)
  (`WidgetBlueprintLibrary.SetInputMode_GameAndUIEx` (`GameplayStatics.GetPlayerController` 0) _evidence_list "DoNotLock" false)
  (`GameplayStatics.SetViewportMouseCaptureMode` "CapturePermanently_IncludingInitialMouseDown"))

(fn `UserConstructionScript`)