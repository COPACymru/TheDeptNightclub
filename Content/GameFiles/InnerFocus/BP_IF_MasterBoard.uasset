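; Interactive evidence board for Inner Focus mode, where the player arranges evidence, links it with pin strings and opens the evidence folder.
; Cursor line traces route clicks by hit component name to dragging, double-click info or a right-click dropdown.
; Pin strings are runtime cable components following the cursor through a Delay loop, mapped by ID for removal.
; Evidence spawns from GameInstance data at saved transforms and is destroyed on exit.
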(event `Remove Cable`
  (params (ID :type "Float (double-precision) (by ref)"))
  (bind _value (`BlueprintMapLibrary.Map_Find` (`self.Cable REF`) ID))
  ;[1 1 1] Remove cable
  (`/Engine/EditorBlueprintResources/StandardMacros.IsValid` _value
    (:`Is Valid`
      (`ActorComponent.K2_DestroyComponent` _value))))

(event `self.ReceiveBeginPlay`
  (bind _returnvalue (`|CreateWidget` "/Game/GameFiles/InnerFocus/UI/W_IF_DropDownMenu.W_IF_DropDownMenu_C"))
  (set `self.Drop Down Menu` _returnvalue)
  (`GameplayStatics.SetViewportMouseCaptureMode` "CapturePermanently_IncludingInitialMouseDown")
  (bind _returnvalue_2 (`|CreateWidget` "/Game/GameFiles/InnerFocus/UI/W_IF_Controls.W_IF_Controls_C"))
  (set `self.Controls Widget` _returnvalue_2)
  (bind _returnvalue_3 (`|CreateWidget` "/Game/GameFiles/InnerFocus/UI/W_IF_EvidenceInfo.W_IF_EvidenceInfo_C"))
  (set `self.W_EvidenceInfo` _returnvalue_3))

(event `Create Left Click Widget`
  (bind _returnvalue (`|CreateWidget` "/Game/GameFiles/InnerFocus/UI/W_LeftClick.W_LeftClick_C"))
  (bind _output_get (set `self.W_LeftClick` _returnvalue))
  (`UserWidget.AddToViewport` _output_get 0))

(event `Drag Second Pin`
  (bind (_worldlocation _worlddirection) (`PlayerController.DeprojectMousePositionToWorld` (`GameplayStatics.GetPlayerController` 0)))
  ;[1 1 1] Drag out second pin string
  (if (`self.IsPlacingPinString?`) :!label _label
    (bind (_outhit _returnvalue) (`KismetSystemLibrary.LineTraceSingle` :`Start` _worldlocation :`End` (+ _worldlocation (* _worlddirection 2000.0)) :`TraceChannel` "TraceTypeQuery1" :`bIgnoreSelf` false))
    (if _returnvalue
      (set `CableComponent.EndLocation` (`KismetMathLibrary.InverseTransformLocation` (`self.GetTransform`) (`.Location` (`GameplayStatics.BreakHitResult` _outhit))) (stale `Add First Pin String` _returnvalue))
      (set `CableComponent.bAttachEnd` true (stale `Add First Pin String` _returnvalue))
      (`KismetSystemLibrary.Delay` 0.05)
      (`self.Drag Second Pin`))))

(event `Search For Item To Remvoe`
  (bind (_worldlocation _worlddirection) (`PlayerController.DeprojectMousePositionToWorld` (`GameplayStatics.GetPlayerController` 0)))
  ;[1 1 1] Search for item to remove that player has right clicked on
  (bind (_outhit _returnvalue) (`KismetSystemLibrary.LineTraceSingle` _worldlocation (+ _worldlocation (* _worlddirection 2000.0)) "TraceTypeQuery1"))
  (if _returnvalue
    (bind (_bblockinghit _binitialoverlap _time _distance _location _impactpoint _normal _impactnormal _physmat _hitactor _hitcomponent) (`GameplayStatics.BreakHitResult` _outhit))
    (bind _returnvalue_2 (`KismetSystemLibrary.GetDisplayName` _hitcomponent))
    (if (or (`KismetStringLibrary.Contains` _returnvalue_2 "Note") (`KismetStringLibrary.Contains` _returnvalue_2 "Pin String"))
      (`/Engine/EditorBlueprintResources/StandardMacros.IsValid` _hitactor
        (:`Is Valid`
          (set `self.Actor To Remove` _hitactor)
          (`Widget.SetIsEnabled` (`/Game/GameFiles/InnerFocus/UI/W_IF_DropDownMenu.RemoveButton` (`self.Drop Down Menu`)) true)
          ;;[1 1 1] Remove "remove" tut
          (bind _removetut (`self.RemoveTut`)
            (:`then`
              (`Widget.RemoveFromParent` _removetut)
              (set `self.RemoveTut` null))
            (:`else`)))
        (:`Is Not Valid`
          (set `self.Actor To Remove` null :!label _label_2)))
      (else
        (goto _label_2)))
    (else
      (goto _label_2))))

(event `Add First Pin String`
  (params (`Start Transform` :type "Transform Structure"))
  (bind _temppinstringstartloc (`self.TempPinStringStartLoc`))
  ;[1 1 1] Attach first pin string
  (bind _returnvalue (`AddComponent|NODE_AddCableComponent-1` :`RelativeTransform` (`KismetMathLibrary.MakeTransform` _temppinstringstartloc)))
  (`self.Spawn First Pin String REF` _temppinstringstartloc _returnvalue)
  (set `self.IsPlacingPinString?` true)
  (`Widget.RemoveFromParent` (`self.Drop Down Menu`))
  (goto _label))

(event `Key|RightMouseButton`
  (params (Key :type "Key Structure"))
  (bind _returnvalue (`WidgetLayoutLibrary.GetViewportScale`))
  (bind _drop_down_menu (`self.Drop Down Menu`))
  ;[1 1 1] Add drop down menu on right click
  (:`Pressed`
    (bind _returnvalue_2 (`GameplayStatics.GetActorOfClass` "/Game/GameFiles/InnerFocus/BP_InnerFocusComponent.BP_InnerFocusComponent_C"))
    (if (`/Game/GameFiles/InnerFocus/BP_InnerFocusComponent.CanExit?` _returnvalue_2)
      (if (not (`self.IsPlacingPinString?`))
        (`self.Get Clicked Location`)
        (`UserWidget.AddToViewport` _drop_down_menu 0)
        (bind _returnvalue_3 (`WidgetLayoutLibrary.GetMousePositionOnViewport`))
        (`UserWidget.SetPositionInViewport` _drop_down_menu (`KismetMathLibrary.MakeVector2D` (* (`KismetMathLibrary.BreakVector2D` _returnvalue_3) _returnvalue) (* (`.Y` (`KismetMathLibrary.BreakVector2D` _returnvalue_3)) _returnvalue)) true)
        (`self.Search For Item To Remvoe`)))))

(event `Key|LeftMouseButton`
  (params (Key :type "Key Structure"))
  (bind _returnvalue (`WidgetLayoutLibrary.GetViewportScale`))
  (bind _w_evidenceinfo (`self.W_EvidenceInfo`))
  (bind (_worldlocation _worlddirection) (`PlayerController.DeprojectMousePositionToWorld` (`GameplayStatics.GetPlayerController` 0)))
  (bind (_worldlocation_2 _worlddirection_2) (`PlayerController.DeprojectMousePositionToWorld` (`GameplayStatics.GetPlayerController` 0)))
  ;[1 1 1] Click on screen
  (:`Pressed`
    (if (`self.CanClick?`)
      (bind (_outhit _returnvalue_2) (`KismetSystemLibrary.LineTraceSingle` :`Start` _worldlocation :`End` (+ _worldlocation (* _worlddirection 2000.0)) :`TraceChannel` "TraceTypeQuery1" :`bIgnoreSelf` false))
      (if _returnvalue_2
        (if (`self.IsPlacingPinString?`)
          (bind (_bblockinghit _binitialoverlap _time _distance _location _impactpoint _normal _impactnormal _physmat _hitactor _hitcomponent) (`GameplayStatics.BreakHitResult` _outhit))
          (bind _returnvalue_3 (`KismetSystemLibrary.GetDisplayName` _hitcomponent))
          (bind _returnvalue_4 (`KismetStringLibrary.Contains` _returnvalue_3 "Evidence Image"))
          (bind _returnvalue_5 (or _returnvalue_4 (`KismetStringLibrary.Contains` _returnvalue_3 "Note")))
          ;[0 0.1112 1] Attaching the cable to the evidence (if the pin is placed on the evidence)
          (if _returnvalue_5
            (bind _returnvalue_6 (`self.GetComponentByClass` _hitactor "/Game/GameFiles/InnerFocus/AC_BP_InnerFocusPinnable.AC_BP_InnerFocusPinnable_C"))
            (`/Engine/EditorBlueprintResources/StandardMacros.IsValid` _returnvalue_6
              (:`Is Valid`
                (`KismetArrayLibrary.Array_AddUnique` (`/Game/GameFiles/InnerFocus/AC_BP_InnerFocusPinnable.Pins` _returnvalue_6) (stale `Add First Pin String` _returnvalue))
                (`/Game/GameFiles/InnerFocus/AC_BP_InnerFocusPinnable.Place Cable` _returnvalue_6 (stale `Add First Pin String` _returnvalue) self)
                (set `self.IsPlacingPinString?` false))
              (:`Is Not Valid`
                ;[1 1 1] Attach second pin string
                (set `CableComponent.EndLocation` (`KismetMathLibrary.InverseTransformLocation` (`self.GetTransform`) _location) (stale `Add First Pin String` _returnvalue) :!label _label_3)
                (set `CableComponent.bAttachEnd` true (stale `Add First Pin String` _returnvalue))
                (set `self.IsPlacingPinString?` false)))
            (else
              (goto _label_3)))
          (`self.Spawn Second Pin String REF` _location)
          ;[1 1 1] Remove pin string and note tutorial
          (`/Engine/EditorBlueprintResources/StandardMacros.DoOnce` false
            (:`Completed`
              (bind _returnvalue_7 (`|CreateWidget` "/Game/GameFiles/InnerFocus/UI/W_IF_RemovePinTut.W_IF_RemovePinTut_C"))
              (bind _output_get (set `self.RemoveTut` _returnvalue_7))
              (`UserWidget.AddToViewport` _output_get 0)))
          (elif (`KismetStringLibrary.Contains` _returnvalue_3 "Evidence Folder")
            (`self.Open Evidence Board`)
            (else
              ;[1 1 1] Drag to move evidence around
              (if _returnvalue_5
                (set `self.Evidence To Move` _hitactor)
                (bind _result (`/Engine/EditorBlueprintResources/StandardMacros.IncrementInt` (`self.TimesPressed`))
                  (:`  `
                    (if (and (== _result 2) _returnvalue_4)
                      ;[1 1 1] Add evidence info to screen (on double click of evidence)
                      (if (not (`self.IsPlacingPinString?`))
                        (bind _asbp_if_evidence_master (cast `/Game/GameFiles/InnerFocus/Evidence/BP_IF_Evidence_Master` (`self.Evidence To Move`)))
                        (set `/Game/GameFiles/InnerFocus/UI/W_IF_EvidenceInfo.Evidence Info` (`/Game/GameFiles/InnerFocus/Evidence/BP_IF_Evidence_Master.Evidence Info` _asbp_if_evidence_master) _w_evidenceinfo)
                        (`UserWidget.AddToViewport` _w_evidenceinfo 0)
                        (bind _returnvalue_8 (`WidgetLayoutLibrary.GetMousePositionOnViewport`))
                        (`UserWidget.SetPositionInViewport` _w_evidenceinfo (`KismetMathLibrary.MakeVector2D` (* (`KismetMathLibrary.BreakVector2D` _returnvalue_8) _returnvalue) (* (`.Y` (`KismetMathLibrary.BreakVector2D` _returnvalue_8)) _returnvalue)) true))
                      (else
                        (`|ExecutionSequence`
                          (:`then_0`
                            (bind (_outhit_2 _returnvalue_9) (`KismetSystemLibrary.LineTraceSingle` :`Start` _worldlocation_2 :`End` (+ _worldlocation_2 (* _worlddirection_2 2000.0)) :`TraceChannel` "TraceTypeQuery1" :`bIgnoreSelf` false :!label _label_4))
                            (if _returnvalue_9
                              (bind (_bblockinghit_2 _binitialoverlap_2 _time_2 _distance_2 _location_2) (`GameplayStatics.BreakHitResult` _outhit_2))
                              (`self.K2_SetActorLocation` (`self.Evidence To Move`) (`KismetMathLibrary.MakeVector` (.x _location_2) -5128.05658 (.z _location_2)) false false))
                            (`KismetSystemLibrary.Delay` 0.02)
                            (if (`PlayerController.IsInputKeyDown` (`GameplayStatics.GetPlayerController` 0) "LeftMouseButton")
                              (goto _label_4)
                              (else
                                (bind _asbp_if_evidence_master_2 (cast `/Game/GameFiles/InnerFocus/Evidence/BP_IF_Evidence_Master` (`self.Evidence To Move`)))
                                (`KismetArrayLibrary.Array_Set` (`self.Evidence Spawn Transforms`) (`/Game/GameFiles/InnerFocus/Evidence/BP_IF_Evidence_Master.Index` _asbp_if_evidence_master_2) (`KismetMathLibrary.MakeTransform` (`KismetMathLibrary.MakeVector` (.x _location_2) -5128.05658 (.z _location_2)) (struct :`Yaw` 90.0))))))
                          (:`then_1`
                            (`KismetSystemLibrary.RetriggerableDelay` 0.2)
                            (set `self.TimesPressed` 0)))))))))))))))

(event `Open Evidence Board`
  (bind _returnvalue (`GameplayStatics.GetPlayerController` 0))
  (bind _returnvalue_2 (`GameplayStatics.GetPlayerController` 0))
  (`|ExecutionSequence`
    (:`then_0`
      (bind _game_version (message `/Game/GameFiles/GameBlueprints/BPI_GameInstance.Get Game Version` (`GameplayStatics.GetGameInstance`)))
      (switch `/Game/GameFiles/GameBlueprints/GameVersionEnum` _game_version
        (:`NewEnumerator0`
          ;[1 1 1] Open evidence board
          (bind _returnvalue_3 (`GameplayStatics.GetActorOfClass` "/Game/GameFiles/InnerFocus/BP_IF_EvidenceFolder.BP_IF_EvidenceFolder_C"))
          (`self.SetActorHiddenInGame` _returnvalue_3 false)
          (`self.SetActorHiddenInGame` true)
          (`self.EnableInput` _returnvalue_3 _returnvalue_2)
          (`self.DisableInput` self _returnvalue_2)
          (bind _outactors (`GameplayStatics.GetAllActorsOfClass` "/Game/GameFiles/InnerFocus/Evidence/BP_IF_Text.BP_IF_Text_C"))
          (for _array_element _outactors
            (`self.SetActorHiddenInGame` _array_element true)))
        (:`NewEnumerator3`
          ;[1 1 1] Open firebug evidence board
          (`GameplayStatics.GetActorOfClass` "BP_IF_MasterBoard_C")
          (bind _returnvalue_4 (`GameplayStatics.GetActorOfClass` "/Game/GameFiles/InnerFocus/CrimeSceneBoards/BP_IF_FirebugFolder.BP_IF_FirebugFolder_C"))
          (`self.SetActorHiddenInGame` _returnvalue_4 false)
          (`self.SetActorHiddenInGame` true)
          (`self.Hide Polaroids`)
          (bind _returnvalue_5 (`GameplayStatics.GetActorOfClass` "/Game/GameFiles/InnerFocus/BP_InnerFocusComponent.BP_InnerFocusComponent_C"))
          (set `/Game/GameFiles/InnerFocus/BP_InnerFocusComponent.CanMoveCamera?` false _returnvalue_5)
          (`/Game/GameFiles/InnerFocus/BP_InnerFocusComponent.Reset camera` _returnvalue_5)
          (`self.EnableInput` _returnvalue_4 _returnvalue)
          (`self.DisableInput` self _returnvalue)
          (bind _evidence_list (`/Game/GameFiles/InnerFocus/CrimeSceneBoards/BP_IF_FirebugFolder.Evidence List` _returnvalue_4))
          (`UserWidget.AddToViewport` _evidence_list 0)
          (`WidgetBlueprintLibrary.SetInputMode_GameAndUIEx` (`GameplayStatics.GetPlayerController` 0) _evidence_list "DoNotLock" false)
          (`GameplayStatics.SetViewportMouseCaptureMode` "CapturePermanently_IncludingInitialMouseDown")
          (bind _outactors_2 (`GameplayStatics.GetAllActorsOfClass` "/Game/GameFiles/InnerFocus/Evidence/BP_IF_Text.BP_IF_Text_C"))
          (for _array_element_2 _outactors_2
            (`self.SetActorHiddenInGame` _array_element_2 true)))))
    (:`then_1`
      ;[1 1 1] Add evidence tutorial
      (`/Engine/EditorBlueprintResources/StandardMacros.DoOnce` false
        (:`Completed`
          (bind _returnvalue_6 (`|CreateWidget` "/Game/GameFiles/InnerFocus/UI/W_InnerFocusEvidenceTut.W_InnerFocusEvidenceTut_C"))
          (`UserWidget.AddToViewport` _returnvalue_6 0)
          (`/Game/GameFiles/InnerFocus/UI/W_LeftClick.Fade Off` (`self.W_LeftClick`)))))))

(event `Key|Escape` :consume false
  (params (Key :type "Key Structure"))
  ;[1 1 1] Exit inner focus
  (:`Pressed`
    (bind _returnvalue (`GameplayStatics.GetActorOfClass` "/Game/GameFiles/InnerFocus/BP_InnerFocusComponent.BP_InnerFocusComponent_C" :!label _label_5))
    (if (`/Game/GameFiles/InnerFocus/BP_InnerFocusComponent.CanExit?` _returnvalue)
      (if (not (`self.IsPlacingPinString?`))
        (message `/Game/GameFiles/GameBlueprints/BPI_GameInstance.Set Is In Inner Focus` (`GameplayStatics.GetGameInstance`) true)
        (`PlayerCameraManager.StartCameraFade` :`self` (`GameplayStatics.GetPlayerCameraManager` 0) :`ToAlpha` 1.0 :`Duration` 1.0 :`bHoldWhenFinished` true)
        (`/Game/GameFiles/InnerFocus/UI/W_IF_Controls.Fade Off` (`self.Controls Widget`))
        (`KismetSystemLibrary.Delay` 1.0)
        (bind _returnvalue_2 (`GameplayStatics.GetActorOfClass` "/Game/GameFiles/InnerFocus/BP_InnerFocusComponent.BP_InnerFocusComponent_C"))
        (`/Game/GameFiles/InnerFocus/BP_InnerFocusComponent.Close Inner Focus` _returnvalue_2)
        (`PlayerCameraManager.StartCameraFade` :`self` (`GameplayStatics.GetPlayerCameraManager` 0) :`FromAlpha` 1.0 :`Duration` 1.0 :`bHoldWhenFinished` true)
        (message `/Game/GameFiles/GameBlueprints/BPI_GameInstance.Set Is In Inner Focus` (`GameplayStatics.GetGameInstance`) false)
        (`WidgetBlueprintLibrary.SetInputMode_GameOnly` (`GameplayStatics.GetPlayerController` 0))
        (`GameplayStatics.SetViewportMouseCaptureMode` "CapturePermanently_IncludingInitialMouseDown")
        (`self.Clear Evidence On Board`)))))

(event `InputAction|Inner Focus` :consume false
  (params (Key :type "Key Structure"))
  ;[1 1 1] Exit inner focus
  (:`Pressed`
    (goto _label_5)))

(event `Clear Evidence On Board`
  ;[1 1 1] Add and clear evidence on board
  (bind _outactors (`GameplayStatics.GetAllActorsOfClass` "/Game/GameFiles/InnerFocus/Evidence/BP_IF_Evidence_Master.BP_IF_Evidence_Master_C"))
  (for _array_element _outactors
    (`self.K2_DestroyActor` _array_element)))

(event `Key|X`
  (params (Key :type "Key Structure"))
  (bind _controls_widget (`self.Controls Widget`))
  ;[1 1 1] Toggle controls
  (:`Pressed`
    (`/Engine/EditorBlueprintResources/StandardMacros.FlipFlop`
      (:`A`
        (`/Game/GameFiles/InnerFocus/UI/W_IF_Controls.Hide Controls` _controls_widget))
      (:`B`
        (`/Game/GameFiles/InnerFocus/UI/W_IF_Controls.Show Controls` _controls_widget)))))

(event `Load Evidence On Board`
  ;[1 1 1] Add and clear evidence on board
  (bind _evidence_on_board (message `/Game/GameFiles/GameBlueprints/BPI_GameInstance.Get Evidence On Board` (`GameplayStatics.GetGameInstance`)))
  (for (_array_element _array_index) _evidence_on_board
    (`|SpawnActorFromClass` "/Game/GameFiles/InnerFocus/Evidence/BP_IF_Evidence_Master.BP_IF_Evidence_Master_C" (`|GetArrayItem` (`self.Evidence Spawn Transforms`) _array_index) "Undefined" "MultiplyWithRoot" null _array_element _array_index null))
  (`KismetSystemLibrary.Delay` 0.2)
  (bind _outactors (`GameplayStatics.GetAllActorsOfClass` "/Game/GameFiles/InnerFocus/Evidence/BP_IF_Evidence_Master.BP_IF_Evidence_Master_C"))
  (for _array_element_2 _outactors
    (`self.K2_AttachToComponent` _array_element_2 (`self.Board`) "None" "KeepWorld" "KeepWorld" "KeepWorld" true)))

(event `Hide Polaroids`
  ;[1 1 1] Hide/show polaroids
  (bind _outactors (`GameplayStatics.GetAllActorsOfClass` "/Game/GameFiles/InnerFocus/Evidence/BP_IF_Evidence_Master.BP_IF_Evidence_Master_C"))
  (for _array_element _outactors
    (`self.SetActorHiddenInGame` _array_element true)))

(event `Show Polaroids`
  ;[1 1 1] Hide/show polaroids
  (bind _outactors (`GameplayStatics.GetAllActorsOfClass` "/Game/GameFiles/InnerFocus/Evidence/BP_IF_Evidence_Master.BP_IF_Evidence_Master_C"))
  (for _array_element _outactors
    (`self.SetActorHiddenInGame` _array_element false)))

(fn `Get Clicked Location`
  (bind (_worldlocation _worlddirection) (`PlayerController.DeprojectMousePositionToWorld` (`GameplayStatics.GetPlayerController` 0)))
  (bind (_outhit _returnvalue) (`KismetSystemLibrary.LineTraceSingle` :`Start` _worldlocation :`End` (+ _worldlocation (* _worlddirection 2000.0)) :`TraceChannel` "TraceTypeQuery1" :`bIgnoreSelf` false))
  (if _returnvalue
    (set `self.TempPinStringStartLoc` (`KismetMathLibrary.InverseTransformLocation` (`self.GetTransform`) (`.Location` (`GameplayStatics.BreakHitResult` _outhit))))))

(fn `Spawn First Pin String REF`
  (params (Location :type "Vector Structure") (`Cable REF` :type "CableComponent Object Reference"))
  (bind _pin_string_id (`self.Pin String ID`))
  (bind _returnvalue (`KismetArrayLibrary.Array_IsEmpty` (`self.Pin String ID`)))
  (bind _returnvalue_2 (+ (`|GetArrayItem` _pin_string_id (- (`KismetArrayLibrary.Array_Length` _pin_string_id) 1)) 0.9))
  (bind _returnvalue_3 (`KismetMathLibrary.SelectFloat` 1.0 _returnvalue_2 _returnvalue))
  (`BlueprintMapLibrary.Map_Add` (`self.Cable REF`) _returnvalue_3 `Cable REF`)
  (`|SpawnActorFromClass` "/Game/GameFiles/InnerFocus/BP_PinStringREF.BP_PinStringREF_C" (`KismetMathLibrary.MakeTransform` (`KismetMathLibrary.MakeVector` Location_X -5681.782 Location_Z)) "Undefined" "MultiplyWithRoot" null _returnvalue_3 null)
  (if _returnvalue
    (`KismetArrayLibrary.Array_Add` (`self.Pin String ID`) 1.0)
    (else
      (`KismetArrayLibrary.Array_Add` (`self.Pin String ID`) _returnvalue_2))))

(fn `Spawn Second Pin String REF`
  (params (Location :type "Vector Structure"))
  (returns (ReturnValue :type "/Game/GameFiles/InnerFocus/BP_PinStringREF Object Reference"))
  (bind _pin_string_id (`self.Pin String ID`))
  (bind _returnvalue (+ (`|GetArrayItem` _pin_string_id (- (`KismetArrayLibrary.Array_Length` _pin_string_id) 1)) 0.1))
  (bind _returnvalue_2 (`|SpawnActorFromClass` "/Game/GameFiles/InnerFocus/BP_PinStringREF.BP_PinStringREF_C" (`KismetMathLibrary.MakeTransform` (`KismetMathLibrary.MakeVector` Location_X -5681.782 Location_Z)) "Undefined" "MultiplyWithRoot" null _returnvalue null))
  (`KismetArrayLibrary.Array_Add` (`self.Pin String ID`) _returnvalue)
  (return _returnvalue_2))

(fn `UserConstructionScript`)