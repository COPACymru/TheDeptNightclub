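; Camera actor for Inner Focus mode, where the player examines the evidence board, opened by a MaleCharacter event.
; Opening switches view and input from the character, loads BP_IF_MasterBoard's evidence and controls, and shows a first-time tutorial; closing restores the character if CanExit.
; WASD pans through Delay-based polling loops and the wheel zooms, both within hard-coded world bounds.
; Space resets the camera, X toggles controls help, and a timeline handles board focus.
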(event `self.ReceiveBeginPlay`
  (bind _asmale_character (cast `/Game/GameFiles/Characters/Male/MaleCharacter` (`GameplayStatics.GetPlayerCharacter` 0)))
  (add `/Game/GameFiles/Characters/Male/MaleCharacter.Enter Inner Focus` _asmale_character (delegate `Open Inner Focus`)))

(event `Open Inner Focus`
  (bind _returnvalue (`GameplayStatics.GetPlayerController` 0))
  (`PlayerController.SetViewTargetWithBlend` (`GameplayStatics.GetPlayerController` 0) self 0.0 "VTBlend_Linear" 0.0 false)
  (`PlayerCameraManager.StopAllCameraShakes` (`GameplayStatics.GetPlayerCameraManager` 0) true)
  (set `PlayerController.bShowMouseCursor` true (`GameplayStatics.GetPlayerController` 0))
  (bind _returnvalue_2 (`GameplayStatics.GetActorOfClass` "/Game/GameFiles/InnerFocus/BP_IF_MasterBoard.BP_IF_MasterBoard_C"))
  (`self.EnableInput` _returnvalue_2 _returnvalue)
  (`self.EnableInput` _returnvalue)
  (`self.DisableInput` (`GameplayStatics.GetPlayerCharacter` 0) _returnvalue)
  (message `/Game/GameFiles/GameBlueprints/BPI_GameInstance.Set Can Pause` (`GameplayStatics.GetGameInstance`) false)
  (`KismetSystemLibrary.Delay` 1.0)
  (`PlayerCameraManager.StartCameraFade` :`self` (`GameplayStatics.GetPlayerCameraManager` 0) :`FromAlpha` 1.0 :`Duration` 1.0 :`bHoldWhenFinished` true)
  (bind _returnvalue_3 (`GameplayStatics.GetActorOfClass` "/Game/GameFiles/InnerFocus/BP_IF_MasterBoard.BP_IF_MasterBoard_C"))
  (`UserWidget.AddToViewport` (`/Game/GameFiles/InnerFocus/BP_IF_MasterBoard.Controls Widget` _returnvalue_3) 0)
  (`/Game/GameFiles/InnerFocus/BP_IF_MasterBoard.Load Evidence On Board` _returnvalue_3)
  (`/Engine/EditorBlueprintResources/StandardMacros.DoOnce` false
    (:`Completed`
      (bind _returnvalue_4 (`|CreateWidget` "/Game/GameFiles/InnerFocus/UI/W_InnerFocusMasterTut.W_InnerFocusMasterTut_C"))
      (`UserWidget.AddToViewport` _returnvalue_4 0)
      (`WidgetBlueprintLibrary.SetInputMode_UIOnlyEx` _returnvalue _returnvalue_4) ; Prevents the need for double clicking the tutorial
    )))

(event `Close Inner Focus`
  (bind _returnvalue (`GameplayStatics.GetPlayerController` 0))
  (if (`self.CanExit?`)
    (`PlayerController.SetViewTargetWithBlend` (`GameplayStatics.GetPlayerController` 0) (`GameplayStatics.GetPlayerCharacter` 0) 0.0 "VTBlend_Linear" 0.0 false)
    (set `PlayerController.bShowMouseCursor` false (`GameplayStatics.GetPlayerController` 0))
    (`self.EnableInput` (`GameplayStatics.GetPlayerCharacter` 0) _returnvalue)
    (bind _returnvalue_2 (`GameplayStatics.GetActorOfClass` "/Game/GameFiles/InnerFocus/BP_IF_MasterBoard.BP_IF_MasterBoard_C"))
    (`self.DisableInput` _returnvalue_2 _returnvalue)
    (`self.DisableInput` _returnvalue)
    (message `/Game/GameFiles/GameBlueprints/BPI_GameInstance.Set Can Pause` (`GameplayStatics.GetGameInstance`) true)
    (`KismetSystemLibrary.Delay` 1.0)))

(event `Key|W`
  (params (Key :type "Key Structure"))
  (bind (_returnvalue_x _returnvalue_y _returnvalue_z) (`KismetMathLibrary.BreakVector` (`self.K2_GetActorLocation`)))
  ;[1 1 1] Move up and left
  (:`Pressed`
    (if (`self.CanMoveCamera?`)
      (`self.K2_SetActorLocation` (`KismetMathLibrary.MakeVector` _returnvalue_x _returnvalue_y (`KismetMathLibrary.FClamp` (+ _returnvalue_z 1.0) -622.0 -547.0)) :!label _label)
      (`KismetSystemLibrary.Delay` 0.01)
      (if (`PlayerController.IsInputKeyDown` (`GameplayStatics.GetPlayerController` 0) "W")
        (goto _label)))))

(event `Key|S`
  (params (Key :type "Key Structure"))
  (bind (_returnvalue_x _returnvalue_y _returnvalue_z) (`KismetMathLibrary.BreakVector` (`self.K2_GetActorLocation`)))
  ;[1 1 1] Move up and left
  (:`Pressed`
    (if (`self.CanMoveCamera?`)
      (`self.K2_SetActorLocation` (`KismetMathLibrary.MakeVector` _returnvalue_x _returnvalue_y (`KismetMathLibrary.FClamp` (- _returnvalue_z 1.0) -622.0 -547.0)) :!label _label_2)
      (`KismetSystemLibrary.Delay` 0.01)
      (if (`PlayerController.IsInputKeyDown` (`GameplayStatics.GetPlayerController` 0) "S")
        (goto _label_2)))))

(event `Key|A`
  (params (Key :type "Key Structure"))
  (bind (_returnvalue_x _returnvalue_y _returnvalue_z) (`KismetMathLibrary.BreakVector` (`self.K2_GetActorLocation`)))
  ;[1 1 1] Move left and right
  (:`Pressed`
    (if (`self.CanMoveCamera?`)
      (`self.K2_SetActorLocation` (`KismetMathLibrary.MakeVector` (`KismetMathLibrary.FClamp` (+ _returnvalue_x 1.0) -343.0 -210.0) _returnvalue_y _returnvalue_z) :!label _label_3)
      (`KismetSystemLibrary.Delay` 0.01)
      (if (`PlayerController.IsInputKeyDown` (`GameplayStatics.GetPlayerController` 0) "A")
        (goto _label_3)))))

(event `Key|D`
  (params (Key :type "Key Structure"))
  (bind (_returnvalue_x _returnvalue_y _returnvalue_z) (`KismetMathLibrary.BreakVector` (`self.K2_GetActorLocation`)))
  ;[1 1 1] Move left and right
  (:`Pressed`
    (if (`self.CanMoveCamera?`)
      (`self.K2_SetActorLocation` (`KismetMathLibrary.MakeVector` (`KismetMathLibrary.FClamp` (- _returnvalue_x 1.0) -343.0 -210.0) _returnvalue_y _returnvalue_z) :!label _label_4)
      (`KismetSystemLibrary.Delay` 0.01)
      (if (`PlayerController.IsInputKeyDown` (`GameplayStatics.GetPlayerController` 0) "D")
        (goto _label_4)))))

(event `Focus On Board`
  ;[1 1 1] Focus on board
  (bind (_direction _move_track) (`Timeline|Focus On Board T` :!label _label_5)
    (:`Update`
      (`self.K2_SetActorLocation` (`KismetMathLibrary.VLerp` (-273.0 -5616.0 -620.0) (-273.0 -5397.0 -587.0) _move_track)))))

(event `Unfocus Board`
  ;[1 1 1] Focus on board
  (goto _label_5 :!via `Reverse`))

(event `Key|SpaceBar`
  (params (Key :type "Key Structure"))
  ;[1 1 1] Reset camera location
  (:`Pressed`
    (`self.K2_SetActorLocation` (-273.0 -5397.0 -587.0) :!label _label_6)))

(event `Key|MouseScrollUp`
  (params (Key :type "Key Structure"))
  (bind (_returnvalue_x _returnvalue_y _returnvalue_z) (`KismetMathLibrary.BreakVector` (`self.K2_GetActorLocation`)))
  ;[1 1 1] Zoom camera in and out
  (:`Pressed`
    (if (`self.CanMoveCamera?`)
      (`self.K2_SetActorLocation` (`KismetMathLibrary.MakeVector` _returnvalue_x (`KismetMathLibrary.FClamp` (+ _returnvalue_y 10.0) -5397.0 -5167.0) _returnvalue_z)))))

(event `Reset camera`
  ;[1 1 1] Reset camera location
  (goto _label_6))

(event `Key|MouseScrollDown`
  (params (Key :type "Key Structure"))
  (bind (_returnvalue_x _returnvalue_y _returnvalue_z) (`KismetMathLibrary.BreakVector` (`self.K2_GetActorLocation`)))
  ;[1 1 1] Zoom camera in and out
  (:`Pressed`
    (if (`self.CanMoveCamera?`)
      (`self.K2_SetActorLocation` (`KismetMathLibrary.MakeVector` _returnvalue_x (`KismetMathLibrary.FClamp` (- _returnvalue_y 10.0) -5397.0 -5167.0) _returnvalue_z)))))

(event `Key|X`
  (params (Key :type "Key Structure"))
  ;[1 1 1] Toggle controls
  (:`Pressed`
    (`/Engine/EditorBlueprintResources/StandardMacros.FlipFlop`
      (:`A`
        (bind _returnvalue (`GameplayStatics.GetActorOfClass` "/Game/GameFiles/InnerFocus/BP_IF_MasterBoard.BP_IF_MasterBoard_C"))
        (`/Game/GameFiles/InnerFocus/UI/W_IF_Controls.Hide Controls` (`/Game/GameFiles/InnerFocus/BP_IF_MasterBoard.Controls Widget` _returnvalue)))
      (:`B`
        (bind _returnvalue_2 (`GameplayStatics.GetActorOfClass` "/Game/GameFiles/InnerFocus/BP_IF_MasterBoard.BP_IF_MasterBoard_C"))
        (`/Game/GameFiles/InnerFocus/UI/W_IF_Controls.Show Controls` (`/Game/GameFiles/InnerFocus/BP_IF_MasterBoard.Controls Widget` _returnvalue_2))))))

(fn `UserConstructionScript`)