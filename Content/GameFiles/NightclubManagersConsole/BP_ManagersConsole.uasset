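; BP_ManagersConsole is an interactable nightclub manager's computer that opens a screen-space desktop UI for the player.
; On BeginPlay it creates and stores desktop, mail inbox and web browser widgets.
; Interact toggles the session: opening shows the desktop, enables the console's input and the cursor.
; Closing removes the current widget, returns input to the interactor and restores game-only input mode.
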(event `self.ReceiveBeginPlay`
  (bind _returnvalue (`|CreateWidget` "/Game/GameFiles/NightclubManagersConsole/W_ConsoleDesktop.W_ConsoleDesktop_C"))
  (set `self.W_Desktop` _returnvalue)
  (bind _returnvalue_2 (`|CreateWidget` "/Game/GameFiles/NightclubManagersConsole/Mail/W_MailInbox.W_MailInbox_C"))
  (set `self.W_Mail` _returnvalue_2)
  (bind _returnvalue_3 (`|CreateWidget` "/Game/GameFiles/NightclubManagersConsole/W_WebBrowser.W_WebBrowser_C"))
  (set `self.W_Web Browser` _returnvalue_3))

(fn `Interact`
  (params (Interactor :type "Character Object Reference") (`Camera Trans Time` :type "Float (double-precision)"))
  (returns (`Did Interact?` :type Boolean))
  (bind _returnvalue (`GameplayStatics.GetPlayerController` 0))
  (bind _returnvalue_2 (`GameplayStatics.GetPlayerController` 0))
  (bind _w_desktop (`self.W_Desktop`))
  (if (`self.IsInteracting?`)
    (`Widget.RemoveFromParent` (`self.Current Widget`))
    (set `self.IsInteracting?` false)
    (`self.EnableInput` Interactor _returnvalue)
    (`self.DisableInput` _returnvalue)
    (set `PlayerController.bShowMouseCursor` false _returnvalue_2)
    (`WidgetBlueprintLibrary.SetInputMode_GameOnly` _returnvalue_2)
    (else
      (`UserWidget.AddToViewport` _w_desktop 0)
      (set `self.Current Widget` _w_desktop)
      (set `self.IsInteracting?` true)
      (`self.DisableInput` null _returnvalue)
      (`self.EnableInput` _returnvalue)
      (set `self.Inspector` null)
      (set `PlayerController.bShowMouseCursor` true _returnvalue_2)))
  (return true))

(fn `UserConstructionScript`)