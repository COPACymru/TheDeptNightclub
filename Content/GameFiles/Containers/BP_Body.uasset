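; Searchable body container that lets the player inspect clue items and mark them as evidence.
; Interact toggles a container widget, input and view target between player and body, unlocking KeyID 1 lockers on entry.
; A timeline lerps selected items to an inspection point, where gated mouse input rotates them and the wheel changes focal length.
; X matches the item's ClueID to BP_NEE_MASTER actors, logs it as evidence and removes its widget entry.
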(event `self.ReceiveBeginPlay`
  (bind _returnvalue (`|CreateWidget` "/Game/GameFiles/Containers/UI/W_Container.W_Container_C" null (`self.Items`) (`self.Container Name ENG`) (`self.Container Name CYM`) self (`self.ItemsBP`)))
  (set `self.Container Widget` _returnvalue))

(event `Key|LeftShift`
  (params (Key :type "Key Structure"))
  (:`Pressed`
    (`/Game/GameFiles/GameBlueprints/InteractInterface.Interact` (`self.Interactor`))))

(event `InputAction|Interact`
  (params (Key :type "Key Structure")))

(event `Key|X`
  (params (Key :type "Key Structure"))
  (bind _container_widget (`self.Container Widget`))
  ;[1 1 1] Mark clue as evidence
  (:`Pressed`
    (bind _selected_item (`self.Selected Item`)
      (:`then`
        (bind _outactors (`GameplayStatics.GetAllActorsOfClass` "/Game/GameFiles/Blueprints/Clues/NoneEssentialEvidence/BP_NEE_MASTER.BP_NEE_MASTER_C"))
        (for _array_element _outactors
          (if (`KismetTextLibrary.EqualEqual_TextText` (`/Game/GameFiles/Blueprints/Clues/NoneEssentialEvidence/BP_NEE_MASTER.Clue ID` _array_element) (`/Game/GameFiles/Blueprints/Clues/NoneEssentialEvidence/BP_NEE_MASTER.Clue ID` _selected_item))
            (message `/Game/GameFiles/GameBlueprints/BPI_GameInstance.Add To Firebug Evidence` (`GameplayStatics.GetGameInstance`) (`/Game/GameFiles/Blueprints/Clues/NoneEssentialEvidence/BP_NEE_MASTER.Evidence Info` _array_element))
            (set `self.Sensitivity` (`/Game/GameFiles/Blueprints/Clues/NoneEssentialEvidence/BP_NEE_MASTER.Container Sensitivity` _array_element))
            (`/Game/GameFiles/Blueprints/Clues/NoneEssentialEvidence/BP_NEE_MASTER.Is Clue Marked As Evidence` _array_element)
            ;;[1 1 1] Remove item from drawer
            (`PanelWidget.RemoveChild` (`/Game/GameFiles/Containers/UI/W_Container.VerticalBox_71` _container_widget) (`BlueprintMapLibrary.Map_Find` (`/Game/GameFiles/Containers/UI/W_Container.ActiveItems` _container_widget) (`self.Selected Item`)))
            (`self.Put Down Item`)
            (bind _returnvalue (`|CreateWidget` "/Game/GameFiles/UI/Prompts/AddedToEvidence.AddedToEvidence_C"))
            (`UserWidget.AddToViewport` _returnvalue 0)
            (set `CineCameraComponent.CurrentFocalLength` 30.0 (`self.CineCamera`))
            (break)))
        (set `self.Selected Item` null))
      (:`else`))))

(event `/Game/GameFiles/Containers/BPI_Containers.Set Selected Item`
  (params (Item :type "/Game/GameFiles/Blueprints/Clues/NoneEssentialEvidence/BP_NEE_MASTER Object Reference"))
  ;[1 1 1] Set clue
  (if (not (`TimelineComponent.IsPlaying` (`self.Pickup Item`)))
    (if (`self.IsViewingItem?`)
      (`self.Put Down Item`)
      (`KismetSystemLibrary.Delay` 0.5))
    (bind _output_get (set `self.Selected Item` Item))
    (set `self.Cached Selected Item` _output_get)
    (set `self.Selected Item Initial Transform` (`KismetMathLibrary.MakeTransform` (`self.K2_GetActorLocation` _output_get) (`self.K2_GetActorRotation` _output_get)))
    (set `self.Rot To Use` (struct))
    (bind (_direction _movement_track) (`Timeline|Pickup Item` :!label _label)
      (:`Update`
        (`self.K2_SetActorTransform` (`self.Cached Selected Item`) (`KismetMathLibrary.TLerp` (`self.Selected Item Initial Transform`) (`KismetMathLibrary.MakeTransform` (`SceneComponent.K2_GetComponentLocation` (`self.ChildActor`)) (`self.Rot To Use`)) _movement_track) false false))
      (:`Finished`
        (switch `ETimelineDirection` _direction
          (:`Forward`
            (set `self.IsViewingItem?` true))
          (:`Backward`
            (set `self.IsViewingItem?` false)))))))

(event `Put Down Item`
  ;[1 1 1] Set clue
  (set `self.Rot To Use` (`self.K2_GetActorRotation` (`self.Cached Selected Item`)))
  (goto _label :!via `Reverse`))

(event `InputAxisKey|MouseX`
  (params (AxisValue :type "Float (single-precision)"))
  (bind _sensitivity (`self.Sensitivity`))
  ;[1 1 1] Rotate clue
  (`/Engine/EditorBlueprintResources/StandardMacros.Gate` true :!label _label_2
    (:`Exit`
      (`self.K2_SetActorRotation` (`self.Cached Selected Item`) (`KismetMathLibrary.ComposeRotators` (`self.K2_GetActorRotation` (`self.Cached Selected Item`)) (`KismetMathLibrary.MakeRotator` (* AxisValue _sensitivity) (* (stale `InputAxisKey|MouseY` AxisValue) _sensitivity))) false))))

(event `InputAxisKey|MouseY`
  (params (AxisValue :type "Float (single-precision)"))
  ;[1 1 1] Rotate clue
  (goto _label_2))

(event `InputAction|Inspect` :consume false
  (params (Key :type "Key Structure"))
  ;[1 1 1] Rotate clue
  (:`Pressed`
    (goto _label_2 :!via `Open`))
  (:`Released`
    (goto _label_2 :!via `Close`)))

(event `self.Sphere.OnComponentBeginOverlap`
  (params (OverlappedComponent :type "PrimitiveComponent Object Reference") (OtherActor :type "Actor Object Reference") (OtherComp :type "PrimitiveComponent Object Reference") (OtherBodyIndex :type Integer) (bFromSweep :type Boolean) (SweepResult :type "HitResult Structure (by ref)"))
  ;[1 1 1] Interaction
  (if (`self.ActorHasTag` OtherActor "Player")
    (message `/Game/GameFiles/GameBlueprints/InteractInterface.Set Interaction Type` OtherActor true)
    (`SceneComponent.SetVisibility` (`self.Widget`) true false)))

(event `Key|MouseScrollUp`
  (params (Key :type "Key Structure"))
  (bind _cinecamera (`self.CineCamera`))
  ;[1 1 1] Zoom in/out
  (:`Pressed`
    (set `CineCameraComponent.CurrentFocalLength` (`KismetMathLibrary.FClamp` (+ (`CineCameraComponent.CurrentFocalLength` _cinecamera) 7.0) 30.0 200.0) _cinecamera)))

(event `self.Sphere.OnComponentEndOverlap`
  (params (OverlappedComponent :type "PrimitiveComponent Object Reference") (OtherActor :type "Actor Object Reference") (OtherComp :type "PrimitiveComponent Object Reference") (OtherBodyIndex :type Integer))
  ;[1 1 1] Interaction
  (if (`self.ActorHasTag` OtherActor "Player")
    (`SceneComponent.SetVisibility` (`self.Widget`) false false)))

(event `Key|MouseScrollDown`
  (params (Key :type "Key Structure"))
  (bind _cinecamera (`self.CineCamera`))
  ;[1 1 1] Zoom in/out
  (:`Pressed`
    (set `CineCameraComponent.CurrentFocalLength` (`KismetMathLibrary.FClamp` (- (`CineCameraComponent.CurrentFocalLength` _cinecamera) 7.0) 30.0 200.0) _cinecamera)))

(fn `Interact`
  (params (Interactor :type "Character Object Reference") (`Camera Trans Time` :type "Float (double-precision)"))
  (returns (`Did Interact?` :type Boolean))
  (bind _returnvalue (`GameplayStatics.GetPlayerController` 0))
  (bind _returnvalue_2 (`GameplayStatics.GetPlayerController` 0))
  (bind _container_widget (`self.Container Widget`))
  (bind _interactor (`local.Interactor`))
  (bind _widget (`self.Widget`))
  (if (`self.IsInteracting?`)
    (`Widget.RemoveFromParent` _container_widget)
    (`WidgetBlueprintLibrary.SetInputMode_GameOnly` _returnvalue)
    (set `PlayerController.bShowMouseCursor` false _returnvalue)
    (`self.EnableInput` Interactor _returnvalue)
    (`self.DisableInput` _returnvalue)
    (set `self.IsInteracting?` false)
    (`SceneComponent.SetVisibility` _widget true false)
    (`PlayerController.SetViewTargetWithBlend` _returnvalue_2 (`local.Interactor`) 0.0 "VTBlend_Linear" 0.0 false)
    (`self.SetActorHiddenInGame` _interactor false)
    (if (`self.IsViewingItem?`)
      (`self.Put Down Item`)
      (return true))
    (else
      (`UserWidget.AddToViewport` _container_widget 0)
      (`WidgetBlueprintLibrary.SetInputMode_GameAndUIEx` _returnvalue _container_widget "DoNotLock" false)
      (set `PlayerController.bShowMouseCursor` true _returnvalue)
      (`self.EnableInput` _returnvalue)
      (`self.DisableInput` Interactor _returnvalue)
      (set `self.IsInteracting?` true)
      (set `self.Interactor` Interactor)
      (`SceneComponent.SetVisibility` _widget false false)
      (`PlayerController.SetViewTargetWithBlend` _returnvalue_2 self 0.0 "VTBlend_Linear" 0.0 false)
      (`self.SetActorHiddenInGame` _interactor true)
      (bind _outactors (`GameplayStatics.GetAllActorsOfClass` "/Game/GameFiles/Containers/BP_Locker.BP_Locker_C"))
      (for _array_element _outactors
        (if (and (`/Game/GameFiles/Containers/BP_Locker.IsLocked?` _array_element) (== (`/Game/GameFiles/Containers/BP_Locker.Key ID` _array_element) 1))
          (set `/Game/GameFiles/Containers/BP_Locker.IsLocked?` false _array_element)))
      (`PlayerCameraManager.StopAllCameraShakes` (`GameplayStatics.GetPlayerCameraManager` 0) true)
      (return true))))

(fn `UserConstructionScript`)