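; Interactable CCTV console actor where the player sits at a desk and reviews nightclub footage leading to Alex's murder by Gasmask.
; Interact swaps input and view and starts a sit-down sequence, while widgets drive cameras, timestamps, static and time-skip prompts.
; Timed skips advance crowds, audio and scripted sequences, hiding present-day clues in past footage.
; EndCCTV restores clues, moves Dan and streams the tunnels; post-QTE interaction plays the ending.
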(event `Put Gasmask On Monitor`
  (bind _outactors (`GameplayStatics.GetAllActorsOfClassWithTag` "/Script/Engine.StaticMeshActor" "Monitor"))
  (for _array_element _outactors
    (`PrimitiveComponent.SetMaterial` (`StaticMeshActor.StaticMeshComponent` _array_element) 0 "/Game/GameFiles/Blueprints/CCTV/MATS/GasmaskCloseup_MAT.GasmaskCloseup_MAT")))

(event `Gasmask Talks To Morgan On Screen`
  (bind _outactors (`GameplayStatics.GetAllActorsOfClassWithTag` "/Script/Engine.StaticMeshActor" "MiddleMonitor"))
  (for _array_element _outactors
    (`PrimitiveComponent.SetMaterial` (`StaticMeshActor.StaticMeshComponent` _array_element) 0 null)
    (break)))

(event `Toggle Clues`
  ;[1 1 1] Toggle clue visibility
  (bind _isa (`/Engine/EditorBlueprintResources/StandardMacros.FlipFlop`)
    (:`A`
      _)
    (:`B`
      _))
  (bind _outactors (`GameplayStatics.GetAllActorsOfClass` "/Game/GameFiles/Blueprints/Clues/TutorialClueBP.TutorialClueBP_C"))
  (for _array_element _outactors
    (`self.SetActorHiddenInGame` _array_element _isa))
  (bind _outactors_2 (`GameplayStatics.GetAllActorsOfClassWithTag` "/Script/Engine.DecalActor" "Blood"))
  (for _array_element_2 _outactors_2
    (`self.SetActorHiddenInGame` _array_element_2 _isa))
  (bind _outactors_3 (`GameplayStatics.GetAllActorsOfClass` "/Game/GameFiles/Blueprints/Clues/NoneEssentialEvidence/MasterNEE.MasterNEE_C"))
  (for _array_element_3 _outactors_3
    (`self.SetActorHiddenInGame` _array_element_3 _isa)))

(event `self.ReceiveBeginPlay`
  (bind _returnvalue (`|CreateWidget` "/Game/GameFiles/UI/Prompts/ViewCCTV.ViewCCTV_C"))
  (bind _output_get (set `self.ViewSuspectsPrompt` _returnvalue))
  (`UserWidget.AddToViewport` _output_get 0)
  (bind _returnvalue_2 (`|CreateWidget` "/Game/GameFiles/Blueprints/CCTV/CCTV_Widget.CCTV_Widget_C"))
  (set `self.CCTV Widget` _returnvalue_2)
  (bind _returnvalue_3 (`|CreateWidget` "/Game/GameFiles/UI/Prompts/W_SKipAhead.W_SKipAhead_C"))
  (bind _output_get_2 (set `self.Time Skip Widget` _returnvalue_3))
  (`UserWidget.AddToViewport` _output_get_2 0)
  (`|ExecutionSequence`
    (:`then_0`
      (bind _outactors (`GameplayStatics.GetAllActorsOfClass` "/Game/GameFiles/Characters/ClubDancers/BP_ClubDancer.BP_ClubDancer_C"))
      (for _array_element _outactors
        (`self.SetActorHiddenInGame` _array_element true)))
    (:`then_1`
      (bind _outactors_2 (`GameplayStatics.GetAllActorsOfClass` "/Game/GameFiles/Blueprints/ClubLights/BP_ClubLights.BP_ClubLights_C"))
      (for _array_element_2 _outactors_2
        (`self.SetActorHiddenInGame` _array_element_2 true)))))

(event `Close Log In`
  (bind _returnvalue (`GameplayStatics.GetPlayerCharacter` 0))
  (bind _returnvalue_2 (`GameplayStatics.GetPlayerController` 0))
  (set `self.IsInteracting?` false)
  (`self.EnableInput` _returnvalue _returnvalue_2)
  (`self.DisableInput` _returnvalue_2)
  (set `PlayerController.bShowMouseCursor` false _returnvalue_2)
  (`WidgetBlueprintLibrary.SetInputMode_GameOnly` _returnvalue_2)
  (`PlayerController.SetViewTargetWithBlend` _returnvalue_2 _returnvalue 0.0 "VTBlend_Linear" 0.0 false)
  (bind _returnvalue_3 (`GameplayStatics.GetActorOfClass` "/Game/GameFiles/Characters/Dan/BP_Dan.BP_Dan_C"))
  (`self.SetActorHiddenInGame` _returnvalue_3 false)
  (`self.SetActorHiddenInGame` (`GameplayStatics.GetPlayerCharacter` 0) false)
  (`|ExecutionSequence`
    (:`then_0`
      (bind _outactors (`GameplayStatics.GetAllActorsOfClass` "/Game/GameFiles/Characters/ClubDancers/BP_ClubDancer.BP_ClubDancer_C"))
      (for _array_element _outactors
        (`self.SetActorHiddenInGame` _array_element true)))
    (:`then_1`
      (bind _outactors_2 (`GameplayStatics.GetAllActorsOfClass` "/Game/GameFiles/Blueprints/ClubLights/BP_ClubLights.BP_ClubLights_C"))
      (for _array_element_2 _outactors_2
        (`self.SetActorHiddenInGame` _array_element_2 true)))))

(event `self.Box.OnComponentBeginOverlap`
  (params (OverlappedComponent :type "PrimitiveComponent Object Reference") (OtherActor :type "Actor Object Reference") (OtherComp :type "PrimitiveComponent Object Reference") (OtherBodyIndex :type Integer) (bFromSweep :type Boolean) (SweepResult :type "HitResult Structure (by ref)"))
  ;[1 1 1] Display prompt
  (if (`self.ActorHasTag` OtherActor "Player")
    (message `/Game/GameFiles/GameBlueprints/InteractInterface.Set Interaction Type` OtherActor true)
    (`SceneComponent.SetVisibility` (`self.Widget`) true false)))

(event `self.Box.OnComponentEndOverlap`
  (params (OverlappedComponent :type "PrimitiveComponent Object Reference") (OtherActor :type "Actor Object Reference") (OtherComp :type "PrimitiveComponent Object Reference") (OtherBodyIndex :type Integer))
  ;[1 1 1] Display prompt
  (if (`self.ActorHasTag` OtherActor "Player")
    (message `/Game/GameFiles/GameBlueprints/InteractInterface.Set Interaction Type` OtherActor false)
    (`SceneComponent.SetVisibility` (`self.Widget`) false false)))

(event `Get CCTV Widget`
  (bind _returnvalue (`GameplayStatics.GetActorOfClass` "/Game/GameFiles/Characters/Tutorial/TutorialAttacker.TutorialAttacker_C"))
  (set `/Game/GameFiles/Characters/Tutorial/TutorialAttacker.CCTV Widget` (`self.CCTV Widget`) _returnvalue))

(event `Toggle CCTV Audio`
  ;[1 1 1] Toggle audio
  (`/Engine/EditorBlueprintResources/StandardMacros.FlipFlop`
    (:`A`
      (bind _returnvalue (`GameplayStatics.SpawnSound2D` "/Game/GameFiles/SFX/Club_CCTV_SFX.Club_CCTV_SFX" 1.0 1.0 0.0 null))
      (set `self.Club Audio` _returnvalue))
    (:`B`
      (`AudioComponent.Stop` (`self.Club Audio`)))))

(event `Start Time Skip Countdown`
  (params (Countdown :type "Float (double-precision)"))
  ;[1 1 1] Time skip countdown
  (`KismetSystemLibrary.Delay` Countdown)
  (set `self.CanSkipTime?` true)
  (`/Game/GameFiles/UI/Prompts/W_SKipAhead.Fade On` (`self.Time Skip Widget`)))

(event `Interact_Button`
  ;[1 1 1] Stop viewing
  (if (`self.CanSkipTime?`) :!label _label
    (switch `int` (`self.SkipsUsed`)
      (:`0`
        (`self.Time Skip 1`))
      (:`1`
        (`self.Time Skip 2`))
      (:`2`
        (`self.Time Skip 3`))
      (:`3`
        (`self.Cut To Live Feed`)))))

(event `InputAction|Interact`
  (params (Key :type "Key Structure"))
  ;[1 1 1] Stop viewing
  (:`Pressed`
    (goto _label)))

(event `Jump Audio`
  ;[1 1 1] Jump audio
  (`AudioComponent.Stop` (`self.Club Audio`))
  (bind _returnvalue (`GameplayStatics.SpawnSound2D` "/Game/GameFiles/SFX/HalfClubAudio.HalfClubAudio" 1.0 1.0 0.0 null))
  (set `self.Club Audio` _returnvalue))

(event `Time Skip 1`
  (`/Game/GameFiles/Blueprints/CCTV/CCTV_Widget.Set CCTV Time` (`self.CCTV Widget`) (`KismetMathLibrary.MakeDateTime` 2022 1 22 1 42))
  (set `self.CanSkipTime?` false)
  (set `self.SkipsUsed` 1)
  (`/Game/GameFiles/UI/Prompts/W_SKipAhead.Fade Off` (`self.Time Skip Widget`))
  (`/Game/GameFiles/Blueprints/CCTV/CCTV_Widget.Play Static` (`self.CCTV Widget`))
  (`self.Jump Audio`)
  (`self.Play Crowd Half`)
  (`self.Start Time Skip Countdown` 5.0))

(event `Time Skip 2`
  (`/Game/GameFiles/Blueprints/CCTV/CCTV_Widget.Set CCTV Time` (`self.CCTV Widget`) (`KismetMathLibrary.MakeDateTime` 2022 1 22 2 13))
  (set `self.CanSkipTime?` false)
  (set `self.SkipsUsed` 2)
  (`/Game/GameFiles/UI/Prompts/W_SKipAhead.Fade Off` (`self.Time Skip Widget`))
  (`/Game/GameFiles/Blueprints/CCTV/CCTV_Widget.Play Static` (`self.CCTV Widget`))
  (`self.Toggle CCTV Audio`)
  (`self.Play Crowd Empty`)
  ;[1 1 1] Shannon and Alex interact (Shannon leaves and Alex goes to sit at the bar)
  (`self.Play CCTV Sequence 1 ED`)
  (`self.Enable CCTV Grain`)
  (`/Game/GameFiles/Blueprints/CCTV/CCTV_Widget.Hide Camera Select` (`self.CCTV Widget`))
  (set `PlayerController.bShowMouseCursor` false (`GameplayStatics.GetPlayerController` 0))
  (`KismetSystemLibrary.Delay` 12.0)
  (`/Game/GameFiles/Blueprints/CCTV/CCTV_Widget.Play Static` (`self.CCTV Widget`))
  (`/Game/GameFiles/Blueprints/CCTV/CCTV_Widget.Open Camera Behind Bar` (`self.CCTV Widget`))
  (`/Game/GameFiles/Blueprints/CCTV/CCTV_Widget.Set CCTV Time` (`self.CCTV Widget`) (`KismetMathLibrary.MakeDateTime` 2022 1 22 3 29))
  ;[1 1 1] Gasmask comes out from right and sits next to Alex - they talk
  (`self.Play CCTV Sequence 2 ED`)
  (`KismetSystemLibrary.Delay` 23.0)
  (set `self.CanSkipTime?` true)
  (`/Game/GameFiles/UI/Prompts/W_SKipAhead.Fade On` (`self.Time Skip Widget`)))

(event `Time Skip 3`
  ;[1 1 1] Gasmask kills Alex
  (`/Game/GameFiles/Blueprints/CCTV/CCTV_Widget.Set CCTV Time` (`self.CCTV Widget`) (`KismetMathLibrary.MakeDateTime` 2022 1 22 2 27))
  (set `self.CanSkipTime?` false)
  (set `self.SkipsUsed` 3)
  (`/Game/GameFiles/UI/Prompts/W_SKipAhead.Fade Off` (`self.Time Skip Widget`))
  (`/Game/GameFiles/Blueprints/CCTV/CCTV_Widget.Open Nightclub Floor 4` (`self.CCTV Widget`))
  (`self.Play CCTV Sequence 3 ED`)
  (`KismetSystemLibrary.Delay` 7.63)
  (`self.End CCTV`))

(event `Cut To Live Feed`
  (`/Game/GameFiles/Blueprints/CCTV/CCTV_Widget.Set CCTV Time` (`self.CCTV Widget`) (`KismetMathLibrary.MakeDateTime` 2022 1 22 4 17))
  (set `self.CanSkipTime?` false)
  (set `self.SkipsUsed` 4)
  (`/Game/GameFiles/Blueprints/CCTV/CCTV_Widget.Play Static` (`self.CCTV Widget`))
  (`self.Show Clues`)
  (bind _returnvalue (`GameplayStatics.GetActorOfClass` "/Game/GameFiles/Blueprints/QTE/QTE_Component_CCTV.QTE_Component_CCTV_C"))
  (`/Game/GameFiles/Blueprints/QTE/QTE_Component_CCTV.Start Music New` _returnvalue))

(event `Gasmask Talks To Morgan`
  (params (Duration :type "Float (single-precision)"))
  ;[1 1 1] END GAME
  (`KismetSystemLibrary.Delay` Duration)
  (bind _returnvalue (`|CreateWidget` "/Game/GameFiles/UI/TitleSequence/TitleSequence.TitleSequence_C"))
  (`UserWidget.AddToViewport` _returnvalue 0)
  (`KismetSystemLibrary.Delay` 7.0)
  (bind _asdepartment_game_instance (cast `/Game/GameFiles/GameBlueprints/DepartmentGameInstance` (`GameplayStatics.GetGameInstance`)))
  (message `/Game/UltimateMenu/Blueprints/Data/Interfaces/Interface_UMS_GameInstance.Display_MenuContent` _asdepartment_game_instance "NewEnumerator5" "NewEnumerator0")
  (bind _returnvalue_2 (`|CreateWidget` "/Game/GameFiles/UI/W_Black.W_Black_C"))
  (`UserWidget.AddToViewport` _returnvalue_2 -1))

(event `End CCTV`
  ;[1 1 1] End CCTV
  (set `self.WatchingCCTV?` false)
  (`self.Disable CCTV Grain`)
  (`/Game/GameFiles/Blueprints/CCTV/CCTV_Widget.Play Static` (`self.CCTV Widget`))
  (`|ExecutionSequence`
    (:`then_0`
      (bind _returnvalue (`GameplayStatics.GetActorOfClass` "/Game/GameFiles/Blueprints/CCTV/BP_SitDownREF.BP_SitDownREF_C"))
      (`self.SetActorHiddenInGame` _returnvalue true)
      (`Widget.RemoveFromParent` (`self.CCTV Widget`))
      (`KismetSystemLibrary.Delay` 0.2)
      (`self.Interact` (`self.Inspector`))
      (bind _returnvalue_2 (`GameplayStatics.GetActorOfClass` "/Game/GameFiles/Blueprints/Doors/BP_NightclubCellarDoor.BP_NightclubCellarDoor_C"))
      (set `/Game/GameFiles/Blueprints/Doors/BP_NightclubCellarDoor.HasWatchedCCTV?` true _returnvalue_2)
      (bind _returnvalue_3 (`GameplayStatics.GetActorOfClass` "/Game/GameFiles/Characters/Dan/BP_Dan.BP_Dan_C"))
      (`|AIMoveTo` _returnvalue_3 (0.0 0.0 0.0) _returnvalue_3
        (:`OnSuccess`
          (set `/Game/GameFiles/Characters/Dan/BP_Dan.IsInFinalSequence?` true _returnvalue_3)
          (`self.K2_SetActorLocationAndRotation` _returnvalue_3 (802.0 4500.0 -125.499961) (struct :`Yaw` -90.0) false false)
          (`/Engine/EditorBlueprintResources/StandardMacros.DoOnce` false
            (:`Completed`
              (`GameplayStatics.PlaySound2D` "/Game/GameFiles/VoiceLines/Tutorial/Hughes/English/FinalSequence/Hughes_Next_Steps_Cue.Hughes_Next_Steps_Cue" 1.0 1.0 0.0 null null) ; "Excellent work mate"
              (bind _returnvalue_4 (`|CreateWidget` "/Game/GameFiles/UI/Subtitles/Master/W_Subtitles.W_Subtitles_C" null (make `DataTableRowHandle` "/Game/GameFiles/UI/Subtitles/SubDT_HughesNextSteps_ENG.SubDT_HughesNextSteps_ENG" "1")))
              (`UserWidget.AddToViewport` _returnvalue_4 0)
              (`KismetSystemLibrary.Delay` 2.0)
              (`GameplayStatics.LoadStreamLevel` "NightclubTunnels_Level" true)
              (`KismetSystemLibrary.Delay` 30.0)
              (if (not (`self.FoundDan?`))
                (`GameplayStatics.PlaySound2D` "/Game/GameFiles/VoiceLines/Tutorial/Hughes/English/10032024/Hughes_VO_Fire_Exit_Out_Back_Cue.Hughes_VO_Fire_Exit_Out_Back_Cue" 1.0 1.0 0.0 null null)
                (bind _returnvalue_5 (`|CreateWidget` "/Game/GameFiles/UI/Subtitles/Master/W_Subtitles.W_Subtitles_C" null (make `DataTableRowHandle` "/Game/GameFiles/UI/Subtitles/SubDT_HughesFireExit_ENG.SubDT_HughesFireExit_ENG" "1")))
                (`UserWidget.AddToViewport` _returnvalue_5 0)))))))
    (:`then_1`
      (bind _outactors (`GameplayStatics.GetAllActorsOfClass` "/Game/GameFiles/Blueprints/Clues/TutorialClueBP.TutorialClueBP_C" :!label _label_2))
      (for _array_element _outactors
        (`self.SetActorHiddenInGame` _array_element false))
      (bind _outactors_2 (`GameplayStatics.GetAllActorsOfClassWithTag` "/Script/Engine.DecalActor" "Blood"))
      (for _array_element_2 _outactors_2
        (`self.SetActorHiddenInGame` _array_element_2 false))
      (bind _outactors_3 (`GameplayStatics.GetAllActorsOfClass` "/Game/GameFiles/Blueprints/Clues/NoneEssentialEvidence/MasterNEE.MasterNEE_C"))
      (for _array_element_3 _outactors_3
        (`self.SetActorHiddenInGame` _array_element_3 false)))))

(event `Show Clues`
  ;[1 1 1] End CCTV
  (goto _label_2))

(event `Hide Clues`
  (bind _outactors (`GameplayStatics.GetAllActorsOfClass` "/Game/GameFiles/Blueprints/Clues/TutorialClueBP.TutorialClueBP_C"))
  (for _array_element _outactors
    (`self.SetActorHiddenInGame` _array_element true))
  (bind _outactors_2 (`GameplayStatics.GetAllActorsOfClassWithTag` "/Script/Engine.DecalActor" "Blood"))
  (for _array_element_2 _outactors_2
    (`self.SetActorHiddenInGame` _array_element_2 true))
  (bind _outactors_3 (`GameplayStatics.GetAllActorsOfClass` "/Game/GameFiles/Blueprints/Clues/NoneEssentialEvidence/MasterNEE.MasterNEE_C"))
  (for _array_element_3 _outactors_3
    (`self.SetActorHiddenInGame` _array_element_3 true)))

(event `Log In`
  ;[1 1 1] Log in
  (bind _returnvalue (`GameplayStatics.GetActorOfClass` "/Game/GameFiles/NightclubManagersConsole/BP_ManagersConsole.BP_ManagersConsole_C"))
  (bind _w_desktop (`/Game/GameFiles/NightclubManagersConsole/BP_ManagersConsole.W_Desktop` _returnvalue))
  (`UserWidget.AddToViewport` _w_desktop 0)
  (set `/Game/GameFiles/NightclubManagersConsole/BP_ManagersConsole.Current Widget` _w_desktop _returnvalue)
  (set `self.LoggedIn?` true))

(event `Open CCTV`
  (bind _cctv_widget (`self.CCTV Widget`))
  ;[1 1 1] Open CCTV
  (`self.Show Clues`)
  (bind _returnvalue (`GameplayStatics.GetActorOfClass` "/Game/GameFiles/Blueprints/CCTV/BP_SitDownREF.BP_SitDownREF_C"))
  (`self.SetActorHiddenInGame` _returnvalue false)
  (set `self.OpenedCCTV?` true)
  (`UserWidget.AddToViewport` _cctv_widget 0)
  (`/Game/GameFiles/Blueprints/CCTV/CCTV_Widget.Show Camera Select` _cctv_widget)
  (`Widget.SetIsEnabled` (`/Game/GameFiles/Blueprints/CCTV/CCTV_Widget.PastFootage` _cctv_widget) true)
  (bind _outactors (`GameplayStatics.GetAllActorsOfClass` "/Game/GameFiles/Blueprints/CCTV/CCTV_BP.CCTV_BP_C"))
  (for _array_element _outactors
    (if (== (`/Game/GameFiles/Blueprints/CCTV/CCTV_BP.Camera ID` _array_element) 5)
      (`PlayerController.SetViewTargetWithBlend` (`GameplayStatics.GetPlayerController` 0) _array_element 0.0 "VTBlend_Linear" 0.0 false)
      (break)))
  (set `self.WatchingCCTV?` true)
  (`KismetSystemLibrary.Delay` 7.0)
  (if (not (`/Game/GameFiles/Blueprints/CCTV/CCTV_Widget.WatchingPastFootage?` (`self.CCTV Widget`)))
    (`/Engine/EditorBlueprintResources/StandardMacros.DoOnce` false
      (:`Completed`
        (`GameplayStatics.PlaySound2D` "/Game/GameFiles/VoiceLines/Tutorial/Morgan/English/CCTV_Sequence/New/only_really_need_the_last_couple_of_hours_Cue.only_really_need_the_last_couple_of_hours_Cue" 1.0 1.0 0.0 null null)
        (bind _returnvalue_2 (`|CreateWidget` "/Game/GameFiles/UI/Subtitles/Master/W_Subtitles.W_Subtitles_C" null (make `DataTableRowHandle` "/Game/GameFiles/UI/Subtitles/SubDT_LastCoupleHours_ENG.SubDT_LastCoupleHours_ENG" "1")))
        (`UserWidget.AddToViewport` _returnvalue_2 0)))))

(event `Watch Past CCTV`
  (`self.Start Time Skip Countdown` 5.0)
  (`self.Hide Clues`)
  (`self.Toggle CCTV Audio`)
  (`self.Play Crowd Full`)
  (bind _returnvalue (`GameplayStatics.GetActorOfClass` "/Game/GameFiles/Characters/Dan/BP_Dan.BP_Dan_C"))
  (`self.SetActorHiddenInGame` _returnvalue true)
  (`/Game/GameFiles/Blueprints/CCTV/CCTV_Widget.Play Static` (`self.CCTV Widget`))
  (bind _returnvalue_2 (`GameplayStatics.GetActorOfClass` "/Game/GameFiles/Blueprints/CCTV/BP_SitDownREF.BP_SitDownREF_C"))
  (`self.SetActorHiddenInGame` _returnvalue_2 true))

(fn `Interact`
  (params (Interactor :type "Character Object Reference") (`Camera Trans Time` :type "Float (double-precision)"))
  (returns (`Did Interact?` :type Boolean))
  (bind _returnvalue (`GameplayStatics.GetPlayerController` 0))
  (bind _returnvalue_2 (`GameplayStatics.GetPlayerController` 0))
  (bind _returnvalue_3 (`GameplayStatics.GetPlayerController` 0))
  (bind _caninteract_ (`self.CanInteract?`))
  (bind _widget (`self.Widget`))
  (if (`self.IsInteracting?`)
    (if (`self.WatchingCCTV?`)
      _
      (elif _caninteract_
        (`SceneComponent.SetVisibility` _widget false false)
        (`self.Show Clues`)
        (set `self.SkipsUsed` 0)
        (`Widget.RemoveFromParent` (`self.CCTV Widget`))
        (set `self.IsInteracting?` false)
        (`self.EnableInput` Interactor _returnvalue_2)
        (`self.DisableInput` _returnvalue_2)
        (set `PlayerController.bShowMouseCursor` false _returnvalue_3)
        (`WidgetBlueprintLibrary.SetInputMode_GameOnly` _returnvalue_3)
        (`PlayerController.SetViewTargetWithBlend` _returnvalue_3 Interactor 0.0 "VTBlend_Linear" 0.0 false)
        (bind _returnvalue_4 (`GameplayStatics.GetActorOfClass` "/Game/GameFiles/Characters/Dan/BP_Dan.BP_Dan_C"))
        (`self.SetActorHiddenInGame` _returnvalue_4 false)
        (`self.SetActorHiddenInGame` (`GameplayStatics.GetPlayerCharacter` 0) false)
        (return true)))
    (elif _caninteract_
      (`SceneComponent.SetVisibility` _widget false false)
      (`self.Play CCTV Sequence Sit Down`)
      (set `self.IsInteracting?` true)
      (`self.DisableInput` Interactor _returnvalue_2)
      (`self.EnableInput` _returnvalue_2)
      (set `self.Inspector` Interactor)
      (set `PlayerController.bShowMouseCursor` true _returnvalue_3)
      (bind _returnvalue_5 (`GameplayStatics.GetActorOfClass` "/Game/GameFiles/Characters/Dan/BP_Dan.BP_Dan_C"))
      (`self.SetActorHiddenInGame` _returnvalue_5 false)
      (`self.SetActorHiddenInGame` (`GameplayStatics.GetPlayerCharacter` 0) true)
      (return true)
      (elif (`self.Completed QTE?`)
        (`self.DisableInput` Interactor _returnvalue)
        (`self.EnableInput` _returnvalue)
        (set `PlayerController.bShowMouseCursor` true _returnvalue)
        (bind _outactors (`GameplayStatics.GetAllActorsOfClass` "/Game/GameFiles/Blueprints/CCTV/CCTV_BP.CCTV_BP_C"))
        (for _array_element _outactors
          (if (== (`/Game/GameFiles/Blueprints/CCTV/CCTV_BP.Camera ID` _array_element) 13)
            (`PlayerController.SetViewTargetWithBlend` (`GameplayStatics.GetPlayerController` 0) _array_element 0.0 "VTBlend_Linear" 0.0 false)
            (break)))
        (`/Game/GameFiles/Blueprints/CCTV/CCTV_Widget.Disable All Buttons` (`self.CCTV Widget`))
        (`self.Play CCTV Sequence 4 ED`)
        (`self.Gasmask Talks To Morgan` 5.0)))))

(fn `UserConstructionScript`)