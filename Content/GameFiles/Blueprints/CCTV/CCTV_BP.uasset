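; CCTV camera actor whose Construction Script picks one of three meshes from CCTVMesh and repositions the Camera component to suit each model.
; The event graph holds remnants of a throttled feed updater: delay-only update events and a stop event that briefly clears ShouldLoop.
; BeginPlay is empty, the loop restarts are unreachable and the CameraID-to-render-target selection is unused, so this graph captures nothing.
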(event `Update Camera Feed`
  (params (FPS :type "Float (double-precision)"))
  (`KismetSystemLibrary.Delay` (/ 1.0 FPS)))

(event `CustomEvent`
  (params (FPS :type "Float (double-precision)"))
  (`KismetSystemLibrary.Delay` (/ 1.0 FPS)))

(event `Stop Updating Camera Feed`
  (set `self.ShouldLoop?` false)
  (`KismetSystemLibrary.RetriggerableDelay` (+ (/ 1.0 24.0) 0.2))
  (set `self.ShouldLoop?` true))

(event `self.ReceiveBeginPlay`)

(fn `UserConstructionScript`
  (bind _camera (`self.Camera`))
  (bind _staticmesh (`self.StaticMesh`))
  (switch `/Game/GameFiles/Blueprints/CCTV/CCTV_Mesh_ENUM` (`self.CCTV Mesh`)
    (:`NewEnumerator0`
      (`StaticMeshComponent.SetStaticMesh` _staticmesh "/Game/QA_Office/Meshes/SM_CCTV_1.SM_CCTV_1")
      (`SceneComponent.K2_SetRelativeTransform` _camera (`KismetMathLibrary.MakeTransform` (0.0 0.0 -10.0) (struct :`Pitch` -90.0)) false false))
    (:`NewEnumerator1`
      (`StaticMeshComponent.SetStaticMesh` _staticmesh "/Game/QA_Office/Meshes/SM_CCTV_2.SM_CCTV_2")
      (`SceneComponent.K2_SetRelativeTransform` _camera (`KismetMathLibrary.MakeTransform` (6.91767 0.0 -10.233283) (struct :`Pitch` -20.0)) false false))
    (:`NewEnumerator2`
      (`StaticMeshComponent.SetStaticMesh` _staticmesh "/Game/ParkingGarage/Meshes/SM_CCTVCameras_Down.SM_CCTVCameras_Down")
      (`SceneComponent.K2_SetRelativeTransform` _camera (`KismetMathLibrary.MakeTransform` (36.926674 0.0 1.83105) (struct :`Pitch` -20.0)) false false))))