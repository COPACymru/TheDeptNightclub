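; Scripted event hub for the CCTV QTE sequence, handling its audio and monitor-screen changes.
; Music events play a start sting and panic alarm, then fade into a loop and out with an end sting; others play voice-over lines.
; Monitor events find tagged StaticMeshActors and swap their materials.
; The gasmask monologue event flashes static with noise, fires CallPlayGasmaskTalksED, then hands off to CCTV_Interaction.
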(event `self.ReceiveBeginPlay`
  (bind _asmale_character (cast `/Game/GameFiles/Characters/Male/MaleCharacter` (`GameplayStatics.GetPlayerCharacter` 0)))
  (set `self.Morgan` _asmale_character))

(event `Start Music New`
  (bind _returnvalue (`GameplayStatics.SpawnSound2D` "/Game/GameFiles/Music/Door_Music_Start.Door_Music_Start" 1.0 1.0 0.0 null))
  (set `self.Start Music` _returnvalue)
  (bind _returnvalue_2 (`GameplayStatics.SpawnSound2D` "/Game/GameFiles/SFX/POLICE_PANIC_WAV.POLICE_PANIC_WAV" 1.0 1.0 0.0 null))
  (set `self.Panic Alarm` _returnvalue_2)
  (`KismetSystemLibrary.Delay` 5.5)
  (`AudioComponent.FadeOut` (`self.Start Music`) 1.0 0.0 "Linear")
  (bind _returnvalue_3 (`GameplayStatics.SpawnSound2D` "/Game/GameFiles/Music/Door_Music_Loop.Door_Music_Loop" 1.0 1.0 0.0 null))
  (bind _output_get (set `self.Loop Music` _returnvalue_3))
  (`AudioComponent.Stop` _output_get)
  (`AudioComponent.FadeIn` _output_get 1.0 1.0 0.0 "Linear"))

(event `QTE Music End`
  (`GameplayStatics.PlaySound2D` "/Game/GameFiles/Music/Door_Music_End.Door_Music_End" 1.0 1.0 0.0 null null)
  (`AudioComponent.FadeOut` (`self.Loop Music`) 1.0 0.0 "Linear"))

(event `End Panic Alarm`
  (`AudioComponent.Stop` (`self.Panic Alarm`)))

(event `Hughes's Death Monitor`
  (bind _outactors (`GameplayStatics.GetAllActorsOfClassWithTag` "/Script/Engine.StaticMeshActor" "MonitorHughes"))
  (for _array_element _outactors
    (`PrimitiveComponent.SetMaterial` (`StaticMeshActor.StaticMeshComponent` _array_element) 0 "/Game/GameFiles/Blueprints/CCTV/MATS/CCTV_HughesDead.CCTV_HughesDead")))

(event `DanVO 1`
  ;[1 1 1] Dan VO
  (`GameplayStatics.PlaySound2D` "/Game/GameFiles/VoiceLines/Tutorial/Morgan/English/Tutorial_Audio_Morgan_STOP_POLICE_STOP_ENGV2.Tutorial_Audio_Morgan_STOP_POLICE_STOP_ENGV2" 1.0 1.0 0.0 null null))

(event `Dan VO 2`
  ;[1 1 1] Dan VO
  (`GameplayStatics.PlaySound2D` "/Game/GameFiles/VoiceLines/Tutorial/Morgan/English/Tutorial_Audio_Morgan_Suspect_Making_Off_ENG.Tutorial_Audio_Morgan_Suspect_Making_Off_ENG" 1.0 1.0 0.0 null null))

(event `GasmaskMonolougeMonitor`
  (bind _outactors (`GameplayStatics.GetAllActorsOfClassWithTag` "/Script/Engine.StaticMeshActor" "MiddleMonitor"))
  (for _array_element _outactors
    (bind _staticmeshcomponent (`StaticMeshActor.StaticMeshComponent` _array_element))
    (`PrimitiveComponent.SetMaterial` _staticmeshcomponent 0 "/Game/GameFiles/Blueprints/CCTV/MATS/CCTV_Static_MAT.CCTV_Static_MAT")
    (`GameplayStatics.PlaySound2D` "/Game/GameFiles/SFX/Static_Sound_Effect__White_Noise_.Static_Sound_Effect__White_Noise_" 1.0 1.0 0.0 null null)
    (`KismetSystemLibrary.Delay` 0.2)
    (`PrimitiveComponent.SetMaterial` _staticmeshcomponent 0 null))
  (`self.PlayGasmaskTalks ED`)
  (bind _returnvalue (`GameplayStatics.GetActorOfClass` "/Game/GameFiles/Blueprints/CCTV/CCTV_Interaction.CCTV_Interaction_C"))
  (`/Game/GameFiles/Blueprints/CCTV/CCTV_Interaction.Gasmask Talks To Morgan` _returnvalue 65.416))

(event `Dan VO 3`
  ;[1 1 1] Dan VO
  (`GameplayStatics.PlaySound2D` "/Game/GameFiles/VoiceLines/Tutorial/Morgan/Welsh/Morgan_Cymraeg_DAN_STAY_WITH_ME_MATE.Morgan_Cymraeg_DAN_STAY_WITH_ME_MATE" 1.0 1.0 0.0 null null))

(event `GasmaskMonolouge Sequence`)

(event `Change Middle Monitor`
  (bind _outactors (`GameplayStatics.GetAllActorsOfClassWithTag` "/Script/Engine.StaticMeshActor" "MiddleMonitor"))
  (for _array_element _outactors
    (`PrimitiveComponent.SetMaterial` (`StaticMeshActor.StaticMeshComponent` _array_element) 0 "/Game/GameFiles/Blueprints/CCTV/MATS/CCTV_RT5_Mat.CCTV_RT5_Mat")))

(fn `UserConstructionScript`)