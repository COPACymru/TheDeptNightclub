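; BP_ClubLights is a club-style spotlight actor that continuously fades between random colours.
; On BeginPlay it picks start and target colours from the LightColours array and plays the ChangeColour timeline to lerp the SpotLight colour between them.
; When the timeline finishes, it waits briefly, makes the target the new start colour, picks another random target and replays, looping indefinitely.
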(event `self.ReceiveBeginPlay`
  (bind _light_colours (`self.Light Colours`))
  (bind _output (`|GetArrayItem` _light_colours (`KismetMathLibrary.RandomInteger` (`KismetArrayLibrary.Array_Length` _light_colours))))
  (set `self.Old Colour` _output)
  (set `self.New Colour` _output :!label _label)
  (bind (_direction _colour_track) (`Timeline|Change Colour` :!via `PlayFromStart`)
    (:`Update`
      (`LightComponent.SetLightColor` (`self.SpotLight`) (`KismetMathLibrary.LinearColorLerp` (`self.Old Colour`) (`self.New Colour`) _colour_track) true))
    (:`Finished`
      (`KismetSystemLibrary.Delay` 0.1)
      (set `self.Old Colour` (`self.New Colour`))
      (goto _label))))

(fn `UserConstructionScript`)