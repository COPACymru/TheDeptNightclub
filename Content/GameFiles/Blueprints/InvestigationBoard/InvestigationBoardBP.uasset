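; InvestigationBoardBP is an interactable investigation board that opens a mission-pin board screen for the player.
; BeginPlay creates both widgets, and box overlaps play or reverse a timeline that fades the on-screen view-map prompt.
; Interact toggles the board widget, switching input mode and cursor, and unlocking missions on open or hiding pins on close.
; Actor input is enabled only while the board is open, letting Escape close it through Interact.
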(event `self.ReceiveBeginPlay`
  (bind _returnvalue (`|CreateWidget` "/Game/GameFiles/UI/Prompts/ViewMap.ViewMap_C"))
  (bind _output_get (set `self.ViewMap Prompt` _returnvalue))
  (`UserWidget.AddToViewport` _output_get 0)
  (bind _returnvalue_2 (`|CreateWidget` "/Game/GameFiles/Blueprints/InvestigationBoard/InvestigationBoard.InvestigationBoard_C" null self))
  (set `self.BoardWidget REF` _returnvalue_2))

(event `self.Box.OnComponentBeginOverlap`
  (params (OverlappedComponent :type "PrimitiveComponent Object Reference") (OtherActor :type "Actor Object Reference") (OtherComp :type "PrimitiveComponent Object Reference") (OtherBodyIndex :type Integer) (bFromSweep :type Boolean) (SweepResult :type "HitResult Structure (by ref)"))
  (bind (_direction _fade_track) (`Timeline|Fade Prompt` :!label _label)
    (:`Update`
      (`TextBlock.SetColorAndOpacity` (`/Game/GameFiles/UI/Prompts/ViewMap.TextBlock_0` (`self.ViewMap Prompt`)) (make `SlateColor` (make `LinearColor` 1.0 1.0 1.0 _fade_track))))))

(event `self.Box.OnComponentEndOverlap`
  (params (OverlappedComponent :type "PrimitiveComponent Object Reference") (OtherActor :type "Actor Object Reference") (OtherComp :type "PrimitiveComponent Object Reference") (OtherBodyIndex :type Integer))
  (goto _label :!via `Reverse`))

(event `Key|Escape`
  (params (Key :type "Key Structure"))
  (:`Pressed`
    (`self.Interact` null)))

(fn `Interact`
  (params (Interactor :type "Character Object Reference") (`Camera Trans Time` :type "Float (double-precision)"))
  (returns (`Did Interact?` :type Boolean))
  (bind _returnvalue (`GameplayStatics.GetPlayerController` 0))
  (bind _returnvalue_2 (`GameplayStatics.GetPlayerController` 0))
  (bind _boardwidget_ref (`self.BoardWidget REF`))
  (bind _boardwidget_ref_2 (`self.BoardWidget REF`))
  (if (`Widget.IsInViewport` (`self.BoardWidget REF`))
    (`Widget.RemoveFromParent` _boardwidget_ref_2)
    (`WidgetBlueprintLibrary.SetInputMode_GameOnly` _returnvalue_2)
    (set `PlayerController.bShowMouseCursor` false _returnvalue_2)
    (`/Game/GameFiles/Blueprints/InvestigationBoard/InvestigationBoard.Hide All Mission Pins` _boardwidget_ref)
    (`self.DisableInput` _returnvalue)
    (return true)
    (else
      (`UserWidget.AddToViewport` _boardwidget_ref_2 0)
      (`WidgetBlueprintLibrary.SetInputMode_GameAndUIEx` _returnvalue_2 _boardwidget_ref_2)
      (set `PlayerController.bShowMouseCursor` true _returnvalue_2)
      (`/Game/GameFiles/Blueprints/InvestigationBoard/InvestigationBoard.Unlock Missions` _boardwidget_ref)
      (`self.EnableInput` _returnvalue)
      (return true))))

(fn `UserConstructionScript`)