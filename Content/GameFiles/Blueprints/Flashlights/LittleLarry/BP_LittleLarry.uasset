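; BP_LittleLarry is a flashlight with a mesh and a rect light that can be toggled on and off.
; Toggling flips the ON flag and light visibility only while CanUse is true.
; Equipping the taser switches the light off and blocks toggling, and unequipping it allows use again without relighting.
; A separate event shows or hides the mesh, and the construction script syncs light visibility to ON.
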(event `Toggle Flashlight`
  (if (`self.CanUse?`)
    (bind _output_get (set `self.ON?` (not (`self.ON?`))))
    (`SceneComponent.SetVisibility` (`self.RectLight`) _output_get false)))

(event `Taser Equiped`
  (set `self.CanUse?` false)
  (if (`self.ON?`)
    (bind _output_get (set `self.ON?` false))
    (`SceneComponent.SetVisibility` (`self.RectLight`) _output_get false)))

(event `Taser Unequipped`
  (set `self.CanUse?` true))

(event `Show/Hide Mesh`
  (params (`Show?` :type Boolean))
  (`SceneComponent.SetVisibility` (`self.StaticMesh`) `Show?` false))

(fn `UserConstructionScript`
  (`SceneComponent.SetVisibility` (`self.RectLight`) (`self.ON?`) false))