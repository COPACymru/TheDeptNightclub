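; Taser item that fires a bolt projectile and roots its user in place for a few seconds.
; UseItem plays the taser sound, disables the User's movement and spawns BoltProjectile at BoltREF, then restores walking after a delay.
; A timeline pulses BottomLight from BeginPlay, replaying itself while ShouldFlash is true.
; Firing clears that flag so the pulse stops after its current cycle, and it restarts when the delay ends.
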(event `self.ReceiveBeginPlay`
  (`self.Flash Light`))

(event `/Game/GameFiles/GameBlueprints/ItemUseInterface.Use Item`
  (params (`Item Location` :type "Vector Structure") (User :type "Character Object Reference"))
  (bind _charactermovement (`Character.CharacterMovement` User))
  (bind (_returnvalue_location _returnvalue_rotation) (`KismetMathLibrary.BreakTransform` (`SceneComponent.K2_GetComponentToWorld` (`self.Bolt REF`))))
  (`GameplayStatics.PlaySoundAtLocation` "/Game/GameFiles/SFX/Taser_SFX.Taser_SFX" `Item Location` (struct) 1.0 1.0 0.0 null null null null)
  (`CharacterMovementComponent.DisableMovement` _charactermovement)
  (`|SpawnActorFromClass` "/Game/GameFiles/Blueprints/Combat/Taser/BoltProjectile.BoltProjectile_C" (`KismetMathLibrary.MakeTransform` _returnvalue_location _returnvalue_rotation) "Undefined" "OverrideRootScale" null null)
  (set `self.ShouldFlash?` false)
  (`KismetSystemLibrary.Delay` 5.0)
  (`CharacterMovementComponent.SetMovementMode` _charactermovement "MOVE_Walking" 0)
  (set `self.ShouldFlash?` true)
  (`self.Flash Light`))

(event `Flash Light`
  (bind (_direction _flash_track) (`Timeline|Flash Light T` :!via `PlayFromStart` :!label _label)
    (:`Update`
      (`LightComponent.SetIntensity` (`self.Bottom Light`) _flash_track))
    (:`Finished`
      (if (`self.ShouldFlash?`)
        (goto _label :!via `PlayFromStart`)))))

(fn `UserConstructionScript`)