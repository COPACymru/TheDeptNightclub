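; BP_UVLight is a UV lamp for the fingerprint minigame that reveals hidden fingerprints caught in its cone.
; Cone overlaps with components tagged Fingerprint unhide their owning actor, and ending the overlap hides it again.
; If the visibility flag still holds after a delay, a DoOnce calls FindFingerprint on the tech demo minigame actor.
; The construction script sets the spotlight intensity, and BeginPlay starts with the cone's collision disabled.
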(event `self.ReceiveBeginPlay`
  (`PrimitiveComponent.SetCollisionEnabled` (`self.Cone`) "NoCollision"))

(event `self.Cone.OnComponentBeginOverlap`
  (params (OverlappedComponent :type "PrimitiveComponent Object Reference") (OtherActor :type "Actor Object Reference") (OtherComp :type "PrimitiveComponent Object Reference") (OtherBodyIndex :type Integer) (bFromSweep :type Boolean) (SweepResult :type "HitResult Structure (by ref)"))
  ;[1 1 1] Show fingerprint under UV light
  (if (`ActorComponent.ComponentHasTag` OtherComp "Fingerprint")
    (`self.SetActorHiddenInGame` (`ActorComponent.GetOwner` OtherComp) false)
    (set `self.IsVisible?` true)
    (`KismetSystemLibrary.Delay` 8.0)
    (if (`self.IsVisible?`)
      (`/Engine/EditorBlueprintResources/StandardMacros.DoOnce` false
        (:`Completed`
          (bind _returnvalue (`GameplayStatics.GetActorOfClass` "/Game/GameFiles/Blueprints/Minigames/Fingerprint/BP_FingerprintMinigameTECH_DEMO_VERSION.BP_FingerprintMinigameTECH_DEMO_VERSION_C"))
          (`/Game/GameFiles/Blueprints/Minigames/Fingerprint/BP_FingerprintMinigameTECH_DEMO_VERSION.Find Fingerprint` _returnvalue))))))

(event `self.Cone.OnComponentEndOverlap`
  (params (OverlappedComponent :type "PrimitiveComponent Object Reference") (OtherActor :type "Actor Object Reference") (OtherComp :type "PrimitiveComponent Object Reference") (OtherBodyIndex :type Integer))
  ;[1 1 1] Show fingerprint under UV light
  (if (`ActorComponent.ComponentHasTag` OtherComp "Fingerprint")
    (`self.SetActorHiddenInGame` (`ActorComponent.GetOwner` OtherComp) true)
    (set `self.IsVisible?` false)))

(fn `UserConstructionScript`
  (`LightComponent.SetIntensity` (`self.SpotLight`) (`self.Intensity`)))