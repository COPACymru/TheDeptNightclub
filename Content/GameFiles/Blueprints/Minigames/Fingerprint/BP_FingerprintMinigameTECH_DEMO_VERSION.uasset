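; Tech-demo fingerprint minigame actor where the player inspects a weapon under UV light to find a fingerprint.
; Interact toggles the session, switching input, camera and music on entry and playing win/loss feedback on exit.
; Input drags to rotate, moves and zooms the weapon with matching camera focus, and toggles UV, while tutorial prompts advance alongside.
; Clicking runs a multi-trace for Fingerprint-tagged components, opening the extraction widget on a hit.
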(event Custom|Fade%20On%20Controls
  ;[1 1 1] Fade on/off minigame controls
  (bind _returnvalue (UserInterface|CreateWidget "/Game/GameFiles/Blueprints/Minigames/Fingerprint/UI/Images/W_Rotate.W_Rotate_C"))
  (bind _output_get (Variables|Default|SetRotate _returnvalue))
  (UserInterface|Viewport|AddtoViewport _output_get 0))

(event Custom|Find%20Fingerprint
  (Variables|Default|GetIsolate
    (:then)
    (:else
      (bind _returnvalue (UserInterface|CreateWidget "/Game/GameFiles/Blueprints/Minigames/Fingerprint/UI/Images/W_Click.W_Click_C"))
      (bind _output_get (Variables|Default|SetExtract _returnvalue))
      (UserInterface|Viewport|AddtoViewport _output_get 0)
      (CallFunction|CheckFadedOff true true true true false false))))

(event Custom|Hide%20Everything
  (Rendering|SetVisibility (Variables|Default|GetWeapon) false false)
  (CallFunction|HideControls))

(event Custom|Stop%20Minigame
  (CallFunction|Interact (Variables|Default|GetInspector) 0.0))

(event Custom|Fade%20Off%20Controls)

(event Custom|Hide%20Lights%20and%20fog
  ;[1 1 1] Hide lights
  (bind _outactors (Actor|GetAllActorsOfClasswithTag "/Script/Engine.PointLight" "UVroom"))
  (for _array_element _outactors
    (Rendering|SetVisibility (Variables|/Script/Engine.Light|GetLightComponent _array_element) false false))
  ;[1 1 1] Hide lights
  (bind _outactors_2 (Actor|GetAllActorsOfClasswithTag "/Script/Engine.SpotLight" "UVroom"))
  (for _array_element_2 _outactors_2
    (Rendering|SetVisibility (Variables|/Script/Engine.Light|GetLightComponent _array_element_2) false false))
  ;[1 1 1] Show UV background bars
  (Rendering|SetVisibility (Variables|Default|GetStaticMesh1) true false))

(event Custom|Pick%20Up%20Weapon
  (bind _weapon (Variables|Default|GetWeapon))
  ;[1 1 1] Pick up/put down weapon
  (bind (_direction _inspect_track) (Timeline|Timeline_2 Play)
    (:Update
      (Transformation|SetWorldLocation _weapon (Math|Vector|Lerp(Vector) (Variables|Default|GetStart%20Transform) (Variables|Default|GetEnd%20Transform) _inspect_track) false false)
      (Transformation|SetWorldRotation _weapon (Math|Rotator|Lerp(Rotator) "0, 0, 0" (Variables|Default|GetWeaponEndRot) _inspect_track true) false false))
    (:Finished
      (switch Utilities|FlowControl|Switch|SwitchonETimelineDirection _direction
        (:Forward
          (Variables|Default|SetIsInspecting? true))
        (:Backward
          (Variables|Default|SetIsInspecting? false))))))

(event Custom|Put%20Down%20Weapon
  (bind _weapon (Variables|Default|GetWeapon))
  ;[1 1 1] Pick up/put down weapon
  (bind (_direction _inspect_track) (Timeline|Timeline_2 Reverse)
    (:Update
      (Transformation|SetWorldLocation _weapon (Math|Vector|Lerp(Vector) (Variables|Default|GetStart%20Transform) (Variables|Default|GetEnd%20Transform) _inspect_track) false false)
      (Transformation|SetWorldRotation _weapon (Math|Rotator|Lerp(Rotator) "0, 0, 0" (Variables|Default|GetWeaponEndRot) _inspect_track true) false false))
    (:Finished
      (switch Utilities|FlowControl|Switch|SwitchonETimelineDirection _direction
        (:Forward
          (Variables|Default|SetIsInspecting? true))
        (:Backward
          (Variables|Default|SetIsInspecting? false))))))

(event Custom|Put%20Down%20UV
  ;[1 1 1] Pick up UV
  (bind (_direction _track) (Timeline|PickUp%20UV Reverse)
    (:Update
      (Transformation|SetRelativeLocation (Variables|Default|GetUV%20Light) (Math|Vector|Lerp(Vector) (Variables|Default|GetUV%20Location) "-15.000000,-15.000000,55.000000" _track) false false))
    (:Finished
      (switch Utilities|FlowControl|Switch|SwitchonETimelineDirection _direction
        (:Forward
          (Variables|Default|SetIsUVPickedUp? true))
        (:Backward
          (Variables|Default|SetIsUVPickedUp? false))))))

(event Custom|Turn%20Off%20UV%20Light
  ;[1 1 1] Toggle UV light
  (if (Variables|Default|GetIsUVPickedUp?)
    (Rendering|SetVisibility (Variables|/Game/GameFiles/Blueprints/Minigames/Fingerprint/BP_UVLight.BP_UVLight_C|GetSpotLight (stale Input|KeyboardEvents|F _asbp_uvlight)) false false)
    (Collision|SetCollisionEnabled (Variables|/Game/GameFiles/Blueprints/Minigames/Fingerprint/BP_UVLight.BP_UVLight_C|GetCone (stale Input|KeyboardEvents|F _asbp_uvlight)) "NoCollision")
    (Audio|PlaySound2D "/Game/GameFiles/Blueprints/Minigames/Fingerprint/SFX/UVLightOff_Cue.UVLightOff_Cue" 1.0 1.0 0.0 0 0)
    (bind _uv_loop (Variables|Default|GetUV%20Loop)
      (:then
        (Audio|Components|Audio|Stop _uv_loop))
      (:else))))

(event Custom|Reset%20DoOnce
  (bind _returnvalue (Transformation|GetActorLocation))
  (Utilities|FlowControl|Sequence
    (:then_0
      ;[1 1 1] Pick up UV
      (Utilities|FlowControl|DoOnce false) ; enters at Reset
    )
    (:then_1
      ;[1 1 1] Interact with weapon
      (Utilities|FlowControl|DoOnce false) ; enters at Reset
    )))

(event Custom|Hide%20Controls
  ;[1 1 1] Show/hide controls
)

(event EventBeginPlay
  (bind _returnvalue (UserInterface|CreateWidget "/Game/GameFiles/UI/Prompts/W_StartForensicExamination.W_StartForensicExamination_C"))
  (bind _output_get (Variables|Default|SetPrompt%20Widget _returnvalue))
  (UserInterface|Viewport|AddtoViewport _output_get 0)
  (Class|GameplayStatics|SetViewportMouseCaptureMode "CapturePermanently_IncludingInitialMouseDown")
  (bind _returnvalue_2 (UserInterface|CreateWidget "/Game/GameFiles/Blueprints/Minigames/Fingerprint/UI/W_FingerprintExtractionTECH_DEMO_VERSION.W_FingerprintExtractionTECH_DEMO_VERSION_C"))
  (Variables|Default|SetExtractionWidget _returnvalue_2))

(event Input|MouseEvents|MouseX
  (params (AxisValue :type Float%20%28single-precision%29))
  ;[1 1 1] Rotate weapon
  (Utilities|FlowControl|Gate true
    (:Exit
      (Transformation|SetRelativeRotation (Variables|Default|GetWeapon) (Math|Rotator|CombineRotators (Variables|/Script/Engine.SceneComponent|GetRelativeRotation (Variables|Default|GetWeapon)) (Math|Rotator|MakeRotator (* AxisValue 3.0) (* (stale Input|MouseEvents|MouseY AxisValue) -3.0) 0.0)) false false))))

(event Input|MouseEvents|MouseY
  (params (AxisValue :type Float%20%28single-precision%29))
  ;[1 1 1] Rotate weapon
  (Utilities|FlowControl|Gate true
    (:Exit
      (Transformation|SetRelativeRotation (Variables|Default|GetWeapon) (Math|Rotator|CombineRotators (Variables|/Script/Engine.SceneComponent|GetRelativeRotation (Variables|Default|GetWeapon)) (Math|Rotator|MakeRotator (* (stale Input|MouseEvents|MouseX AxisValue) 3.0) (* AxisValue -3.0) 0.0)) false false))))

(event Input|MouseEvents|LeftMouseButton
  (params (Key :type Key%20Structure))
  (bind _returnvalue (Game|GetPlayerController 0))
  (bind _fingerprint_border_0 (Variables|Default|GetFingerprint%20Border_0))
  (bind (_worldlocation _worlddirection) (Game|Player|ConvertMouseLocationToWorldSpace _returnvalue))
  (bind _relativelocation (Variables|/Script/Engine.SceneComponent|GetRelativeLocation _fingerprint_border_0))
  ;[1 1 1] Find fingerprint
  (:Pressed
    (bind _outhits (Collision|MultiLineTraceByChannel _worldlocation (+ _worldlocation (* _worlddirection 1.5e+03)) "TraceTypeQuery1" false 0 "None"))
    (for _array_element _outhits
      (if (Components|ComponentHasTag (.HitComponent (Collision|BreakHitResult _array_element)) "Fingerprint")
        (CallFunction|HideEverything)
        (Widget|RemovefromParent (Variables|Default|GetPrompt%20Widget))
        (UserInterface|Viewport|AddtoViewport (Variables|Default|GetExtractionWidget) 0)
        (Variables|Default|SetIsRemovingFingerprint? true)
        (Transformation|SetRelativeLocation _fingerprint_border_0 (Math|Vector|MakeVector (.x _relativelocation) (.y _relativelocation) 0.0) false false)
        (Audio|PlaySound2D "/Game/GameFiles/Blueprints/Minigames/Fingerprint/VO/MiniGame_Fingerprintfind_Cue.MiniGame_Fingerprintfind_Cue" 1.0 1.0 0.0 0 0)
        (bind _returnvalue_2 (UserInterface|CreateWidget "/Game/GameFiles/UI/Subtitles/Master/W_Subtitles.W_Subtitles_C" 0 (Utilities|Struct|MakeDataTableRowHandle "/Game/GameFiles/UI/Subtitles/SubDT_AhGreatFingerprint_ENG.SubDT_AhGreatFingerprint_ENG" "1")))
        (UserInterface|Viewport|AddtoViewport _returnvalue_2 0)
        (Utilities|FlowControl|Sequence
          (:then_0
            ;[1 1 1] WASD prompt
            (Utilities|FlowControl|Delay 3.0)
            (bind _returnvalue_3 (UserInterface|CreateWidget "/Game/GameFiles/Blueprints/Minigames/Fingerprint/UI/Images/W_Draw.W_Draw_C"))
            (bind _output_get (Variables|Default|SetIsolate _returnvalue_3))
            (UserInterface|Viewport|AddtoViewport _output_get 0)
            (CallFunction|CheckFadedOff true true true true true false))
          (:then_1
            (bind _extract (Variables|Default|GetExtract)
              (:then
                (Default|FadeOff _extract))
              (:else))))))))

(event Input|MouseEvents|LeftMouseButton
  (params (Key :type Key%20Structure))
  ;[1 1 1] Fade on/off minigame controls
  (:Pressed
    (bind _rotate (Variables|Default|GetRotate)
      (:then
        (Default|FadeOff _rotate)
        (Utilities|FlowControl|Sequence
          (:then_0
            (Utilities|FlowControl|Delay 2.0)
            (bind _returnvalue (UserInterface|CreateWidget "/Game/GameFiles/Blueprints/Minigames/Fingerprint/UI/Images/W_Zoom.W_Zoom_C"))
            (bind _output_get (Variables|Default|SetZoom _returnvalue))
            (UserInterface|Viewport|AddtoViewport _output_get 0)
            (CallFunction|CheckFadedOff true false false false false false))
          (:then_1
            (Variables|Default|SetRotate 0))))
      (:else))))

(event Input|KeyboardEvents|X
  (params (Key :type Key%20Structure))
  ;[1 1 1] Show/hide controls
)

(event Input|KeyboardEvents|F
  (params (Key :type Key%20Structure))
  ;[1 1 1] Toggle UV light
  (:Pressed
    (CallFunction|HideLightsandFog)
    (bind _asbp_uvlight (Utilities|Casting|CastToBP_UVLight (Variables|/Script/Engine.ChildActorComponent|GetChildActor (Variables|Default|GetUV%20Light))))
    (if (Rendering|IsVisible (Variables|/Game/GameFiles/Blueprints/Minigames/Fingerprint/BP_UVLight.BP_UVLight_C|GetSpotLight _asbp_uvlight))
      (Rendering|SetVisibility (Variables|/Game/GameFiles/Blueprints/Minigames/Fingerprint/BP_UVLight.BP_UVLight_C|GetSpotLight _asbp_uvlight) false false)
      (Collision|SetCollisionEnabled (Variables|/Game/GameFiles/Blueprints/Minigames/Fingerprint/BP_UVLight.BP_UVLight_C|GetCone _asbp_uvlight) "NoCollision")
      (Audio|PlaySound2D "/Game/GameFiles/Blueprints/Minigames/Fingerprint/SFX/UVLightOff_Cue.UVLightOff_Cue" 1.0 1.0 0.0 0 0)
      (bind _uv_loop (Variables|Default|GetUV%20Loop)
        (:then
          (Audio|Components|Audio|Stop _uv_loop))
        (:else))
      (else
        (Rendering|SetVisibility (Variables|/Game/GameFiles/Blueprints/Minigames/Fingerprint/BP_UVLight.BP_UVLight_C|GetSpotLight _asbp_uvlight) true false)
        (Collision|SetCollisionEnabled (Variables|/Game/GameFiles/Blueprints/Minigames/Fingerprint/BP_UVLight.BP_UVLight_C|GetCone _asbp_uvlight) "QueryAndPhysics")
        (Audio|PlaySound2D "/Game/GameFiles/Blueprints/Minigames/Fingerprint/SFX/UVLightOn_Cue.UVLightOn_Cue" 1.0 1.0 0.0 0 0)
        (bind _returnvalue (Audio|SpawnSound2D "/Game/GameFiles/Blueprints/Minigames/Fingerprint/SFX/UVLightOn_Loop_Cue.UVLightOn_Loop_Cue" 1.0 1.0 0.0 0))
        (Variables|Default|SetUV%20Loop _returnvalue)))))

(event Input|MouseEvents|MouseWheelUp
  (params (Key :type Key%20Structure))
  ;[1 1 1] Zoom
  (:Pressed
    (Transformation|AddRelativeLocation (Variables|Default|GetWeapon) "0.000000,0.000000,5.000000" false false)
    (Variables|/Script/CinematicCamera.CineCameraComponent|SetFocusSettings (Variables|Default|GetCineCamera) (Utilities|Struct|MakeCameraFocusSettings "Manual" (- (Math|Vector|VectorLength (Variables|/Script/Engine.SceneComponent|GetRelativeLocation (Variables|Default|GetCineCamera))) (Math|Vector|VectorLength (Variables|/Script/Engine.SceneComponent|GetRelativeLocation (Variables|Default|GetWeapon)))) "(ActorToTrack=None,RelativeOffset=(X=0.000000,Y=0.000000,Z=0.000000))" false 8.0 0.0))))

(event Input|MouseEvents|MouseWheelDown
  (params (Key :type Key%20Structure))
  ;[1 1 1] Zoom
  (:Pressed
    (Transformation|AddRelativeLocation (Variables|Default|GetWeapon) "0.000000,0.000000,-5.000000" false false)
    (Variables|/Script/CinematicCamera.CineCameraComponent|SetFocusSettings (Variables|Default|GetCineCamera) (Utilities|Struct|MakeCameraFocusSettings "Manual" (- (Math|Vector|VectorLength (Variables|/Script/Engine.SceneComponent|GetRelativeLocation (Variables|Default|GetCineCamera))) (Math|Vector|VectorLength (Variables|/Script/Engine.SceneComponent|GetRelativeLocation (Variables|Default|GetWeapon)))) "(ActorToTrack=None,RelativeOffset=(X=0.000000,Y=0.000000,Z=0.000000))" false 8.0 0.0))))

(event Input|KeyboardEvents|F
  (params (Key :type Key%20Structure))
  ;[1 1 1] Fade on/off minigame controls
  (:Pressed
    (bind _uv (Variables|Default|GetUV)
      (:then
        (Default|FadeOff _uv)
        (Variables|Default|SetUV 0))
      (:else))))

(event Input|KeyboardEvents|W
  (params (Key :type Key%20Structure))
  ;[1 1 1] Fade on/off minigame controls
  (:Pressed
    (bind _wasd (Variables|Default|GetWASD)
      (:then
        (Default|FadeOff _wasd)
        (Utilities|FlowControl|Sequence
          (:then_0
            (Utilities|FlowControl|Delay 3.0)
            (bind _returnvalue (UserInterface|CreateWidget "/Game/GameFiles/Blueprints/Minigames/Fingerprint/UI/Images/W_UV.W_UV_C"))
            (bind _output_get (Variables|Default|SetUV _returnvalue))
            (UserInterface|Viewport|AddtoViewport _output_get 0)
            (CallFunction|CheckFadedOff true true true false false false))
          (:then_1
            (Variables|Default|SetWASD 0))))
      (:else))))

(event Input|MouseEvents|LeftMouseButton
  (params (Key :type Key%20Structure))
  ;[1 1 1] Rotate weapon
  (:Pressed
    (Utilities|FlowControl|Gate true) ; enters at Open
  )
  (:Released
    (Utilities|FlowControl|Gate true) ; enters at Close
  ))

(event Input|KeyboardEvents|W
  (params (Key :type Key%20Structure))
  ;[1 1 1] Move UV light
)

(event Input|MouseEvents|LeftMouseButton
  (params (Key :type Key%20Structure))
  ;[1 1 1] Interact with weapon
)

(event Input|KeyboardEvents|S
  (params (Key :type Key%20Structure))
  ;[1 1 1] Move UV light
)

(event Input|KeyboardEvents|A
  (params (Key :type Key%20Structure))
  ;[1 1 1] Move UV light
)

(event Input|KeyboardEvents|D
  (params (Key :type Key%20Structure))
  ;[1 1 1] Move UV light
)

(event Input|KeyboardEvents|A
  (params (Key :type Key%20Structure))
  ;[1 1 1] Move weapon
  (:Pressed
    (Variables|Default|SetIsAHeld? true)
    (Transformation|AddRelativeLocation (Variables|Default|GetWeapon) "0.000000,1.000000,0.000000" false false :!label _label)
    (Utilities|FlowControl|Delay 0.01)
    (if (Variables|Default|GetIsAHeld?)
      (CallFunction|CheckWeaponIsinArea)
      (if true
        (goto _label)
        (else
          (Transformation|AddRelativeLocation (Variables|Default|GetWeapon) "0.000000,-1.000000,0.000000" false false)))))
  (:Released
    (Variables|Default|SetIsAHeld? false)))

(event Input|MouseEvents|MouseWheelUp
  (params (Key :type Key%20Structure))
  ;[1 1 1] Fade on/off minigame controls
  (:Pressed
    (bind _zoom (Variables|Default|GetZoom)
      (:then
        (Default|FadeOff _zoom)
        (Utilities|FlowControl|Sequence
          (:then_0
            (Utilities|FlowControl|Delay 3.0)
            (bind _returnvalue (UserInterface|CreateWidget "/Game/GameFiles/Blueprints/Minigames/Fingerprint/UI/Images/W_WASD.W_WASD_C"))
            (bind _output_get (Variables|Default|SetWASD _returnvalue))
            (UserInterface|Viewport|AddtoViewport _output_get 0)
            (CallFunction|CheckFadedOff true true false false false false))
          (:then_1
            (Variables|Default|SetZoom 0))))
      (:else))))

(event Input|KeyboardEvents|D
  (params (Key :type Key%20Structure))
  ;[1 1 1] Move weapon
  (:Pressed
    (Variables|Default|SetIsDHeld? true)
    (Transformation|AddRelativeLocation (Variables|Default|GetWeapon) "0.000000,-1.000000,0.000000" false false :!label _label)
    (Utilities|FlowControl|Delay 0.01)
    (if (Variables|Default|GetIsDHeld?)
      (CallFunction|CheckWeaponIsinArea)
      (if true
        (goto _label)
        (else
          (Transformation|AddRelativeLocation (Variables|Default|GetWeapon) "0.000000,1.000000,0.000000" false false)))))
  (:Released
    (Variables|Default|SetIsDHeld? false)))

(event Input|KeyboardEvents|Z
  (params (Key :type Key%20Structure))
  ;[1 1 1] Move UV light
  (:Pressed
    (if (Variables|Default|GetIsUVPickedUp?)
      (Variables|Default|SetIsZHeld? true)
      (Transformation|AddLocalOffset (Variables|Default|GetUV%20Light) "0.000000,0.000000,1.000000" false false :!label _label)
      (Utilities|FlowControl|Delay 0.01)
      (if (Variables|Default|GetIsZHeld?)
        (bind _is_in_area_z_ (CallFunction|CheckUVLightIsinArea))
        (if _is_in_area_z_
          (goto _label)
          (else
            (Transformation|AddLocalOffset (Variables|Default|GetUV%20Light) "0.000000,-1.000000,-1.000000" false false))))))
  (:Released
    (Variables|Default|SetIsZHeld? false)))

(event Input|KeyboardEvents|C
  (params (Key :type Key%20Structure))
  ;[1 1 1] Move UV light
  (:Pressed
    (if (Variables|Default|GetIsUVPickedUp?)
      (Variables|Default|SetIsCHeld? true)
      (Transformation|AddLocalOffset (Variables|Default|GetUV%20Light) "0.000000,0.000000,-1.000000" false false :!label _label)
      (Utilities|FlowControl|Delay 0.01)
      (if (Variables|Default|GetIsCHeld?)
        (bind _is_in_area_z_ (CallFunction|CheckUVLightIsinArea))
        (if _is_in_area_z_
          (goto _label)
          (else
            (Transformation|AddLocalOffset (Variables|Default|GetUV%20Light) "0.000000,0.000000,1.000000" false false))))))
  (:Released
    (Variables|Default|SetIsCHeld? false)))

(event Input|KeyboardEvents|W
  (params (Key :type Key%20Structure))
  ;[1 1 1] Move weapon
  (:Pressed
    (Variables|Default|SetIsWHeld? true)
    (Transformation|AddRelativeLocation (Variables|Default|GetWeapon) "-1.000000,0.000000,0.000000" false false :!label _label)
    (Utilities|FlowControl|Delay 0.01)
    (if (Variables|Default|GetIsWHeld?)
      (CallFunction|CheckWeaponIsinArea)
      (if true
        (goto _label)
        (else
          (Transformation|AddRelativeLocation (Variables|Default|GetWeapon) "1.000000,0.000000,0.000000" false false)))))
  (:Released
    (Variables|Default|SetIsWHeld? false)))

(event Input|KeyboardEvents|S
  (params (Key :type Key%20Structure))
  ;[1 1 1] Move weapon
  (:Pressed
    (Variables|Default|SetIsSHeld? true)
    (Transformation|AddRelativeLocation (Variables|Default|GetWeapon) "1.000000,0.000000,0.000000" false false :!label _label)
    (Utilities|FlowControl|Delay 0.01)
    (if (Variables|Default|GetIsSHeld?)
      (CallFunction|CheckWeaponIsinArea)
      (if true
        (goto _label)
        (else
          (Transformation|AddRelativeLocation (Variables|Default|GetWeapon) "-1.000000,0.000000,0.000000" false false)))))
  (:Released
    (Variables|Default|SetIsSHeld? false)))

(fn ConstructionScript
  (Transformation|SetRelativeTransform (Variables|Default|GetWeapon) (Variables|Default|GetWeapon%20Transform) false false))

(fn CheckUVLightIsinArea
  (bind _uv_light (Variables|Default|GetUV%20Light))
  (bind _relativelocation (Variables|/Script/Engine.SceneComponent|GetRelativeLocation _uv_light))
  (return (and (> (.x _relativelocation) -18.0) (< (.x _relativelocation) 34.0)) (and (> (.y _relativelocation) -5e+01) (< (.y _relativelocation) 5e+01)) (and (> (.z _relativelocation) 45.0) (< (.z _relativelocation) 9e+01))))

(fn CheckWeaponIsinArea
  (bind _weapon (Variables|Default|GetWeapon))
  (bind _relativelocation (Variables|/Script/Engine.SceneComponent|GetRelativeLocation _weapon))
  (return (and (> (.x _relativelocation) -36.0) (< (.x _relativelocation) 8.0)) (and (> (.y _relativelocation) -57.0) (< (.y _relativelocation) 53.0)) (and (> (.z _relativelocation) 45.0) (< (.z _relativelocation) 9e+01))))

(fn CheckFadedOff
  (params (Rotate :type Boolean) (Zoom :type Boolean) (WASD :type Boolean) (UV :type Boolean) (Extract :type Boolean) (Isolate :type Boolean))
  (Utilities|FlowControl|Sequence
    (:then_0
      (if Rotate
        (bind _rotate (Variables|Default|GetRotate)
          (:then
            (if (UserInterface|Viewport|IsinViewport _rotate)
              (Default|FadeOff (Variables|Default|GetRotate))
              (Variables|Default|SetRotate 0)))
          (:else))))
    (:then_1
      (if Zoom
        (bind _zoom (Variables|Default|GetZoom)
          (:then
            (if (UserInterface|Viewport|IsinViewport _zoom)
              (Default|FadeOff (Variables|Default|GetZoom))
              (Variables|Default|SetZoom 0)))
          (:else))))
    (:then_2
      (if WASD
        (bind _wasd (Variables|Default|GetWASD)
          (:then
            (if (UserInterface|Viewport|IsinViewport _wasd)
              (Default|FadeOff (Variables|Default|GetWASD))
              (Variables|Default|SetWASD 0)))
          (:else))))
    (:then_3
      (if UV
        (bind _uv (Variables|Default|GetUV)
          (:then
            (if (UserInterface|Viewport|IsinViewport _uv)
              (Default|FadeOff (Variables|Default|GetUV))
              (Variables|Default|SetUV 0)))
          (:else))))
    (:then_4
      (if Extract
        (bind _extract (Variables|Default|GetExtract)
          (:then
            (if (UserInterface|Viewport|IsinViewport _extract)
              (Default|FadeOff (Variables|Default|GetExtract))
              (Variables|Default|SetExtract 0)))
          (:else))))
    (:then_5
      (if Isolate
        (bind _isolate (Variables|Default|GetIsolate)
          (:then
            (if (UserInterface|Viewport|IsinViewport _isolate)
              (Default|FadeOff (Variables|Default|GetIsolate))
              (Variables|Default|SetIsolate 0)))
          (:else))))))

(fn Interact
  (params (Interactor :type Character%20Object%20Reference) (Camera%20Trans%20Time :type Float%20%28double-precision%29))
  (bind _returnvalue (Game|GetPlayerController 0))
  (bind _returnvalue_2 (Game|GetPlayerController 0))
  (if (Variables|Default|GetIsInteracting?)
    (Variables|Default|SetIsInteracting? false)
    (Input|EnableInput Interactor _returnvalue)
    (Input|DisableInput _returnvalue)
    (Audio|Components|Audio|FadeOut (Variables|Default|GetMusic) 2.0 0.0 "Linear" :!class /Script/Engine.AudioComponent)
    (Default|CallRestartMusic)
    (bind _returnvalue_3 (Actor|GetActorOfClass "/Game/GameFiles/Characters/Male/MaleCharacter.MaleCharacter_C"))
    (Audio|Components|Audio|Play (Variables|/Game/GameFiles/Characters/Male/MaleCharacter.MaleCharacter_C|GetPoliceRadio_Cue _returnvalue_3) 3e+01)
    (CallFunction|CheckFadedOff true true true true true true)
    (bind _returnvalue_4 (Actor|GetActorOfClass "/Game/GameFiles/Blueprints/CCTV/CCTV_Interaction.CCTV_Interaction_C"))
    (Variables|/Game/GameFiles/Blueprints/CCTV/CCTV_Interaction.CCTV_Interaction_C|SetIsInMinigame? _returnvalue_4 false)
    (Input|SetInputModeGameOnly _returnvalue_2 false)
    (CallFunction|FadeOffControls)
    (Variables|Default|SetWeaponEndRot (Transformation|GetWorldRotation (Variables|Default|GetWeapon)))
    (CallFunction|TurnOffUVLight)
    (switch int (Variables|Default|GetEnding)
      (:0
        (Audio|PlaySound2D "/Game/GameFiles/Blueprints/Minigames/Fingerprint/VO/MiniGameWin_Cue.MiniGameWin_Cue" 1.0 1.0 0.0 0 0)
        (bind _uv_loop (Variables|Default|GetUV%20Loop)
          (:then
            (Audio|Components|Audio|Stop _uv_loop))
          (:else
            _))
        (bind _returnvalue_5 (UserInterface|CreateWidget "/Game/GameFiles/UI/Subtitles/Master/W_Subtitles.W_Subtitles_C" 0 (Utilities|Struct|MakeDataTableRowHandle "/Game/GameFiles/UI/Subtitles/SubDT_MinigameWin_ENG.SubDT_MinigameWin_ENG" "1")))
        (UserInterface|Viewport|AddtoViewport _returnvalue_5 5))
      (:1
        (Audio|PlaySound2D "/Game/GameFiles/Blueprints/Minigames/Fingerprint/VO/MiniGameLoss_Cue.MiniGameLoss_Cue" 1.0 1.0 0.0 0 0)
        (bind _uv_loop_2 (Variables|Default|GetUV%20Loop)
          (:then
            (Audio|Components|Audio|Stop _uv_loop_2))
          (:else
            _))
        (bind _returnvalue_6 (UserInterface|CreateWidget "/Game/GameFiles/UI/Subtitles/Master/W_Subtitles.W_Subtitles_C" 0 (Utilities|Struct|MakeDataTableRowHandle "/Game/GameFiles/UI/Subtitles/SubDT_MinigameLoss_ENG.SubDT_MinigameLoss_ENG" "1")))
        (UserInterface|Viewport|AddtoViewport _returnvalue_6 5)))
    (bind _returnvalue_7 (Actor|GetActorOfClass "/Game/GameFiles/InnerFocus/BP_InnerFocusComponent.BP_InnerFocusComponent_C"))
    (Variables|/Game/GameFiles/InnerFocus/BP_InnerFocusComponent.BP_InnerFocusComponent_C|SetCanExit? _returnvalue_7 true)
    (return true)
    (else
      (Game|Player|SetViewTargetwithBlend (Game|GetPlayerController 0) self 0.0 "VTBlend_Linear" 0.0 false)
      (Rendering|SetVisibility (Variables|Default|GetWeapon) true false)
      (Default|CallFadeOutMusicMG)
      (bind _returnvalue_8 (Audio|SpawnSound2D "/Game/GameFiles/Blueprints/Minigames/Fingerprint/SFX/MusicLoopMiniGameV2_Cue.MusicLoopMiniGameV2_Cue" 1.0 1.0 0.0 0))
      (bind _output_get (Variables|Default|SetMusic _returnvalue_8))
      (Audio|Components|Audio|Stop _output_get)
      (Audio|Components|Audio|FadeIn _output_get 5.0 1.0 0.0 "Linear" :!class /Script/Engine.AudioComponent)
      (Audio|PlaySound2D "/Game/GameFiles/SFX/InnerFocus_option1_Cue.InnerFocus_option1_Cue" 1.0 1.0 0.0 0 0)
      (CameraFades|StartCameraFade :self (Game|GetPlayerCameraManager 0) :FromAlpha 1.0 :Duration 0.8 :bHoldWhenFinished true)
      (CallFunction|FadeonControls)
      (bind _returnvalue_9 (Actor|GetActorOfClass "/Game/GameFiles/Characters/Male/MaleCharacter.MaleCharacter_C"))
      (Audio|Components|Audio|Stop (Variables|/Game/GameFiles/Characters/Male/MaleCharacter.MaleCharacter_C|GetPoliceRadio_Cue _returnvalue_9))
      (Variables|Default|SetIsInteracting? true)
      (Input|DisableInput Interactor _returnvalue)
      (Input|EnableInput _returnvalue)
      (Variables|Default|SetInspector Interactor)
      (Variables|/Script/Engine.PlayerController|SetbShowMouseCursor _returnvalue_2 true)
      (bind _returnvalue_10 (Actor|GetActorOfClass "/Game/GameFiles/Blueprints/CCTV/CCTV_Interaction.CCTV_Interaction_C"))
      (Variables|/Game/GameFiles/Blueprints/CCTV/CCTV_Interaction.CCTV_Interaction_C|SetIsInMinigame? _returnvalue_10 true)
      (Variables|Default|SetWeaponEndRot "0, 0, 0")
      (CallFunction|ResetDoOnce)
      (Class|GameplayStatics|SetViewportMouseCaptureMode "CaptureDuringMouseDown")
      (bind _outactors (Actor|GetAllActorsOfClass "/Game/GameFiles/Blueprints/Minigames/Fingerprint/BP_CeilingLampFMG.BP_CeilingLampFMG_C"))
      (for _array_element _outactors
        (Default|ToggleLights _array_element))
      (Audio|PlaySound2D "/Game/GameFiles/Blueprints/Minigames/Fingerprint/SFX/Light_Switch.Light_Switch" 1.0 1.0 0.0 0 0)
      (return true))))