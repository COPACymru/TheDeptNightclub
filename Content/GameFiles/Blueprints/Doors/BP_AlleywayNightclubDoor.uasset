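; Interactable door between the downtown alley and, by its name, the nightclub, with an entry trigger toggling the player's interaction prompt.
; Interact unhides the player and swings the bar door open on a timeline.
; A one-shot exit trigger closes it, calls the letterbox, unloads the alley streaming level, then adds the first-person widget, enables camera switching and stops police atmosphere audio/messages.
; A subtitled Hughes radio dialogue chain is left unconnected.
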(event `self.Entry Box.OnComponentBeginOverlap`
  (params (OverlappedComponent :type "PrimitiveComponent Object Reference") (OtherActor :type "Actor Object Reference") (OtherComp :type "PrimitiveComponent Object Reference") (OtherBodyIndex :type Integer) (bFromSweep :type Boolean) (SweepResult :type "HitResult Structure (by ref)"))
  (if (`self.ActorHasTag` OtherActor "Player")
    (message `/Game/GameFiles/GameBlueprints/InteractInterface.Set Interaction Type` OtherActor true)
    (`SceneComponent.SetVisibility` (`self.Widget`) true false)))

(event `self.Entry Box.OnComponentEndOverlap`
  (params (OverlappedComponent :type "PrimitiveComponent Object Reference") (OtherActor :type "Actor Object Reference") (OtherComp :type "PrimitiveComponent Object Reference") (OtherBodyIndex :type Integer))
  (if (`self.ActorHasTag` OtherActor "Player")
    (message `/Game/GameFiles/GameBlueprints/InteractInterface.Set Interaction Type` OtherActor false)
    (`SceneComponent.SetVisibility` (`self.Widget`) false false)))

(event `Open Door`
  (`self.SetActorHiddenInGame` (`GameplayStatics.GetPlayerCharacter` 0) false)
  (bind (_direction _door_track) (`Timeline|Door Timeline` :!label _label)
    (:`Update`
      (`SceneComponent.K2_SetRelativeRotation` (`self.SM_BarDoor01`) (`KismetMathLibrary.MakeRotator` 0.0 0.0 (- _door_track 180.0)) false false))))

(event `Close Door`
  (goto _label :!via `Reverse`))

(event `self.Exit Box.OnComponentBeginOverlap`
  (params (OverlappedComponent :type "PrimitiveComponent Object Reference") (OtherActor :type "Actor Object Reference") (OtherComp :type "PrimitiveComponent Object Reference") (OtherBodyIndex :type Integer) (bFromSweep :type Boolean) (SweepResult :type "HitResult Structure (by ref)"))
  (`KismetSystemLibrary.Delay` 1.5)
  (`self.Close Door`)
  (`ActorComponent.K2_DestroyComponent` (`self.Exit Box`))
  (`self.Open Letterbox`)
  (`|ExecutionSequence`
    (:`then_0`
      ;[1 1 1] Unloading of the alley level
      (`KismetSystemLibrary.Delay` 1.25)
      (`GameplayStatics.UnloadStreamLevel` "Downtown_Alley_Level"))
    (:`then_1`
      (`KismetSystemLibrary.Delay` 3.0)
      (bind _returnvalue (`|CreateWidget` "/Game/GameFiles/UI/Prompts/FirstPerson.FirstPerson_C"))
      (`UserWidget.AddToViewport` _returnvalue 0)
      (bind _asmale_character (cast `/Game/GameFiles/Characters/Male/MaleCharacter` (`GameplayStatics.GetPlayerCharacter` 0)))
      (set `/Game/GameFiles/Characters/Male/MaleCharacter.CanChangeCamera?` true _asmale_character)
      (`KismetSystemLibrary.Delay` 5.0)
      (message `/Game/GameFiles/GameBlueprints/BPI_Player.Stop Police Atmos` _asmale_character))))

(fn `Interact`
  (params (Interactor :type "Character Object Reference") (`Camera Trans Time` :type "Float (double-precision)"))
  (returns (`Did Interact?` :type Boolean))
  (`self.Open Door`)
  (return true))

(fn `UserConstructionScript`)