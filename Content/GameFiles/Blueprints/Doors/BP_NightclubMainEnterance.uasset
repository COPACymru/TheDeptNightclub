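; Nightclub main entrance double door that opens on BeginPlay and drives the player's transition from the hallway into the club.
; A Timeline swings both leaves; a one-shot ExitBox overlap reverses it and swaps streamed levels.
; The same trigger fades music, plays Dan's subtitled line and starts his roaming, feeds evidence slots to the Inner Focus board, and enables sprint.
; Delayed retry loops issue radio-aware CCTV hints, waiting out dialogue.
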(event `self.ReceiveBeginPlay`
  (`self.Open Door`))

(event `Open Door`
  (bind (_direction _left_door _right_door) (`Timeline|Door Timeline` :!label _label)
    (:`Update`
      (`SceneComponent.K2_SetRelativeRotation` (`self.Door Left`) (`KismetMathLibrary.MakeRotator` 0.0 0.0 _left_door) false false)
      (`SceneComponent.K2_SetRelativeRotation` (`self.Door Right`) (`KismetMathLibrary.MakeRotator` 0.0 0.0 _right_door) false false))))

(event `Close Door`
  (goto _label :!via `Reverse`))

(event `self.Exit Box.OnComponentBeginOverlap`
  (params (OverlappedComponent :type "PrimitiveComponent Object Reference") (OtherActor :type "Actor Object Reference") (OtherComp :type "PrimitiveComponent Object Reference") (OtherBodyIndex :type Integer) (bFromSweep :type Boolean) (SweepResult :type "HitResult Structure (by ref)"))
  (`ActorComponent.K2_DestroyComponent` (`self.Exit Box`))
  (`|ExecutionSequence`
    (:`then_0`
      (`KismetSystemLibrary.Delay` 2.0)
      (bind _returnvalue (`GameplayStatics.GetActorOfClass` "/Game/GameFiles/Characters/Dan/BP_Dan.BP_Dan_C"))
      (`GameplayStatics.PlaySoundAtLocation` "/Game/GameFiles/VoiceLines/Tutorial/Hughes/English/Hughes_Vo_TookYouLongEnough_NoRadio_Cue.Hughes_Vo_TookYouLongEnough_NoRadio_Cue" (`self.K2_GetActorLocation` _returnvalue) (struct) 1.0 1.0 0.0 null null _returnvalue null)
      (`/Game/GameFiles/Characters/Dan/BP_Dan.Random Roam` _returnvalue)
      (bind _returnvalue_2 (`|CreateWidget` "/Game/GameFiles/UI/Subtitles/Master/W_Subtitles.W_Subtitles_C" null (make `DataTableRowHandle` "/Game/GameFiles/UI/Subtitles/SubDT_TookYouLongEnough_ENG.SubDT_TookYouLongEnough_ENG" "1")))
      (`UserWidget.AddToViewport` _returnvalue_2 0)
      (`KismetSystemLibrary.Delay` 2.0)
      (`GameplayStatics.LoadStreamLevel` "NightclubUpper_Level" true))
    (:`then_1`
      (`self.FadeOutMusic`)
      (`GameplayStatics.LoadStreamLevel` "Inner_Focus" true)
      (`KismetSystemLibrary.Delay` 2.0)
      (bind _slots (message `/Game/GameFiles/GameBlueprints/BPI_GameInstance.Get Inner Focus Evidecne Slots` (`GameplayStatics.GetGameInstance`)))
      (bind _returnvalue_3 (`GameplayStatics.GetActorOfClass` "/Game/GameFiles/InnerFocus/BP_IF_MasterBoard.BP_IF_MasterBoard_C"))
      (set `/Game/GameFiles/InnerFocus/BP_IF_MasterBoard.Evidence Spawn Transforms` _slots _returnvalue_3))
    (:`then_2`
      (`KismetSystemLibrary.Delay` 0.0)
      (`self.Close Door`)
      (`KismetSystemLibrary.Delay` 2.0)
      (`GameplayStatics.UnloadStreamLevel` "Hallway_V2"))
    (:`then_3`
      (`KismetSystemLibrary.Delay` 180.0)
      (bind _returnvalue_4 (`GameplayStatics.GetActorOfClass` "/Game/GameFiles/Blueprints/CCTV/CCTV_Interaction.CCTV_Interaction_C" :!label _label_2))
      (if (not (`/Game/GameFiles/Blueprints/CCTV/CCTV_Interaction.OpenedCCTV?` _returnvalue_4))
        (bind _returnvalue_5 (`GameplayStatics.GetActorOfClass` "/Game/GameFiles/Characters/Dan/BP_Dan.BP_Dan_C"))
        (if (`/Game/GameFiles/Characters/Dan/BP_Dan.Dialogue?` _returnvalue_5)
          (`KismetSystemLibrary.Delay` 2.0)
          (goto _label_2)
          (else
            (bind _useradio_ (`/Game/GameFiles/Characters/Dan/BP_Dan.Check Radio Distance` _returnvalue_5))
            (if _useradio_
              (`GameplayStatics.PlaySound2D` "/Game/GameFiles/VoiceLines/Tutorial/Hughes/English/CCTV_Prompt_Radio_2_Cue.CCTV_Prompt_Radio_2_Cue" 1.0 1.0 0.0 null null)
              (else
                (`GameplayStatics.PlaySound2D` "/Game/GameFiles/VoiceLines/Tutorial/Hughes/English/CCTV_Prompt_2_Cue.CCTV_Prompt_2_Cue" 1.0 1.0 0.0 null null)))
            (bind _returnvalue_6 (`|CreateWidget` "/Game/GameFiles/UI/Subtitles/Master/W_Subtitles.W_Subtitles_C" null (make `DataTableRowHandle` "/Game/GameFiles/UI/Subtitles/SubDT_HughesCCTVPrompt2_ENG.SubDT_HughesCCTVPrompt2_ENG" "1")))
            (`UserWidget.AddToViewport` _returnvalue_6 0)
            (`KismetSystemLibrary.Delay` 180.0)
            (bind _returnvalue_7 (`GameplayStatics.GetActorOfClass` "/Game/GameFiles/Blueprints/CCTV/CCTV_Interaction.CCTV_Interaction_C" :!label _label_3))
            (if (not (`/Game/GameFiles/Blueprints/CCTV/CCTV_Interaction.OpenedCCTV?` _returnvalue_7))
              (if (`/Game/GameFiles/Blueprints/CCTV/CCTV_Interaction.IsInMinigame?` _returnvalue_7) :!label _label_4
                (`KismetSystemLibrary.Delay` 10.0)
                (goto _label_4)
                (else
                  (bind _returnvalue_8 (`GameplayStatics.GetActorOfClass` "/Game/GameFiles/Characters/Dan/BP_Dan.BP_Dan_C"))
                  (if (`/Game/GameFiles/Characters/Dan/BP_Dan.Dialogue?` _returnvalue_8)
                    (`KismetSystemLibrary.Delay` 2.0)
                    (goto _label_3)
                    (else
                      (bind _useradio__2 (`/Game/GameFiles/Characters/Dan/BP_Dan.Check Radio Distance` _returnvalue_8))
                      (if _useradio__2
                        (`GameplayStatics.PlaySound2D` "/Game/GameFiles/VoiceLines/Tutorial/Hughes/English/CCTV_Prompt_Radio_3_Cue.CCTV_Prompt_Radio_3_Cue" 1.0 1.0 0.0 null null)
                        (else
                          (`GameplayStatics.PlaySound2D` "/Game/GameFiles/VoiceLines/Tutorial/Hughes/English/CCTV_Prompt_3_Cue.CCTV_Prompt_3_Cue" 1.0 1.0 0.0 null null)))
                      (bind _returnvalue_9 (`|CreateWidget` "/Game/GameFiles/UI/Subtitles/Master/W_Subtitles.W_Subtitles_C" null (make `DataTableRowHandle` "/Game/GameFiles/UI/Subtitles/SubDT_HughesCCTVPrompt3_ENG.SubDT_HughesCCTVPrompt3_ENG" "1")))
                      (`UserWidget.AddToViewport` _returnvalue_9 0))))))))))
    (:`then_4`
      (`KismetSystemLibrary.Delay` 0.0)
      (bind _asmale_character (cast `/Game/GameFiles/Characters/Male/MaleCharacter` (`GameplayStatics.GetPlayerCharacter` 0)))
      (set `/Game/GameFiles/Characters/Male/MaleCharacter.CanSprint?` true _asmale_character)
      (bind _returnvalue_10 (`|CreateWidget` "/Game/GameFiles/UI/Prompts/Sprint.Sprint_C"))
      (`UserWidget.AddToViewport` _returnvalue_10 0))))

(fn `UserConstructionScript`)