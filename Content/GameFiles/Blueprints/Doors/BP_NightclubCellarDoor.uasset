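; Nightclub cellar double door that, once the CCTV is watched, lets the player trigger a one-time conversation with Dan.
; The talk plays dialogue, audio and montage, then sets FoundDan on CCTV_Interaction.
; OpenDoor, not called here, swings both leaves by timeline, equips Dan's taser, enables the player's, slows both and switches music.
; Overlapping ExitBox removes both triggers, shows taser tutorial widgets, then reverses the timeline to close.
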(event `self.Entry Box.OnComponentBeginOverlap`
  (params (OverlappedComponent :type "PrimitiveComponent Object Reference") (OtherActor :type "Actor Object Reference") (OtherComp :type "PrimitiveComponent Object Reference") (OtherBodyIndex :type Integer) (bFromSweep :type Boolean) (SweepResult :type "HitResult Structure (by ref)"))
  (if (and (`self.HasWatchedCCTV?`) (`self.ActorHasTag` OtherActor "Player"))
    (message `/Game/GameFiles/GameBlueprints/InteractInterface.Set Interaction Type` OtherActor true)
    (`SceneComponent.SetVisibility` (`self.Widget`) true false)))

(event `self.Entry Box.OnComponentEndOverlap`
  (params (OverlappedComponent :type "PrimitiveComponent Object Reference") (OtherActor :type "Actor Object Reference") (OtherComp :type "PrimitiveComponent Object Reference") (OtherBodyIndex :type Integer))
  (if (and (`self.HasWatchedCCTV?`) (`self.ActorHasTag` OtherActor "Player"))
    (message `/Game/GameFiles/GameBlueprints/InteractInterface.Set Interaction Type` OtherActor false)
    (`SceneComponent.SetVisibility` (`self.Widget`) false false)))

(event `Talk To Dan`
  (`/Engine/EditorBlueprintResources/StandardMacros.DoOnce` false
    (:`Completed`
      (bind _returnvalue (`GameplayStatics.GetActorOfClass` "/Game/GameFiles/Characters/Dan/BP_Dan.BP_Dan_C"))
      (bind _ashughes_rain_coat_animation_blueprint (cast `/Game/RLContent/Hughes_Rain_Coat/Hughes_Rain_Coat_AnimationBlueprint` (`SkeletalMeshComponent.GetAnimInstance` (`/Game/GameFiles/Characters/Dan/BP_Dan.Body` _returnvalue))))
      (set `/Game/RLContent/Hughes_Rain_Coat/Hughes_Rain_Coat_AnimationBlueprint.IsTalking?` true _ashughes_rain_coat_animation_blueprint)
      (bind _dialoguecomponentv2 (`/Game/GameFiles/Characters/Dan/BP_Dan.DialogueComponentV2` _returnvalue))
      (`/Game/GameFiles/DialogueSystemV2/DialogueComponentV2.Start Conversation` _dialoguecomponentv2 13.6)
      (`GameplayStatics.PlaySound2D` "/Game/GameFiles/VoiceLines/Tutorial/Hughes/English/FinalSequence/Hughes_3_1_ExcellentWorkMate_Cue.Hughes_3_1_ExcellentWorkMate_Cue" 1.0 1.0 0.0 null null)
      (message `/Game/GameFiles/DialogueSystemV2/BPI_DialougeComponentV2.Play Anim Montage` _returnvalue "/Game/GameFiles/Characters/Dan/New/Hughes__3_1_NEW_Montage.Hughes__3_1_NEW_Montage")
      (`KismetSystemLibrary.Delay` 0.2)
      (set `/Game/GameFiles/DialogueSystemV2/UI/W_DialogueSystemV2.Interviewee Response` "Excellent work bud. It's a shame we can't get a positive ID on the killer. I reckon we should head back out the service exit to make sure the killers not still there. If he is and he hurts anyone else that's on us at this point." (`/Game/GameFiles/DialogueSystemV2/DialogueComponentV2.DialogueSystemWidget` _dialoguecomponentv2))
      (bind _returnvalue_2 (`GameplayStatics.GetActorOfClass` "/Game/GameFiles/Blueprints/CCTV/CCTV_Interaction.CCTV_Interaction_C"))
      (set `/Game/GameFiles/Blueprints/CCTV/CCTV_Interaction.FoundDan?` true _returnvalue_2))))

(event `self.Exit Box.OnComponentBeginOverlap`
  (params (OverlappedComponent :type "PrimitiveComponent Object Reference") (OtherActor :type "Actor Object Reference") (OtherComp :type "PrimitiveComponent Object Reference") (OtherBodyIndex :type Integer) (bFromSweep :type Boolean) (SweepResult :type "HitResult Structure (by ref)"))
  (if (`self.ActorHasTag` OtherActor "Player")
    (`ActorComponent.K2_DestroyComponent` (`self.Exit Box`))
    (`ActorComponent.K2_DestroyComponent` (`self.Entry Box`))
    (`KismetSystemLibrary.Delay` 0.5)
    (bind _returnvalue (`|CreateWidget` "/Game/GameFiles/UI/Prompts/EquipTaser.EquipTaser_C"))
    (`UserWidget.AddToViewport` _returnvalue 0)
    (`KismetSystemLibrary.Delay` 2.0)
    (bind _returnvalue_2 (`|CreateWidget` "/Game/GameFiles/UI/Prompts/AimTaser.AimTaser_C"))
    (`UserWidget.AddToViewport` _returnvalue_2 0)
    (`self.Close Door`)))

(event `Open Door`
  (bind _returnvalue (`GameplayStatics.GetActorOfClass` "/Game/GameFiles/Characters/Dan/BP_Dan.BP_Dan_C"))
  (`/Game/GameFiles/Characters/Dan/BP_Dan.Equip Taser` _returnvalue)
  (set `CharacterMovementComponent.MaxWalkSpeed` 115.0 (`Character.CharacterMovement` _returnvalue))
  (bind _returnvalue_2 (`GameplayStatics.GetActorOfClass` "/Game/GameFiles/Characters/Male/MaleCharacter.MaleCharacter_C"))
  (set `/Game/GameFiles/Characters/Male/MaleCharacter.CanSprint?` false _returnvalue_2)
  (set `/Game/GameFiles/Characters/Male/MaleCharacter.CanEquipTaser?` true _returnvalue_2)
  (set `CharacterMovementComponent.MaxWalkSpeed` 115.0 (`Character.CharacterMovement` _returnvalue_2))
  (bind _returnvalue_3 (`GameplayStatics.SpawnSound2D` "/Game/GameFiles/Music/Tunnel_Music_Loop_Cue.Tunnel_Music_Loop_Cue" 0.3 1.0 0.0 null false false))
  (set `self.HallwayMusic` _returnvalue_3)
  (bind _returnvalue_4 (`GameplayStatics.GetActorOfClass` "/Game/GameFiles/Blueprints/Doors/BP_NightclubMainEnterance.BP_NightclubMainEnterance_C"))
  (`/Game/GameFiles/Blueprints/Doors/BP_NightclubMainEnterance.FadeOutMusic` _returnvalue_4)
  (bind (_direction _right_door_track _left_door_track) (`Timeline|Timeline` :!label _label)
    (:`Update`
      (`SceneComponent.K2_SetRelativeRotation` (`self.Door Right`) (`KismetMathLibrary.MakeRotator` 0.0 0.0 _right_door_track) false false)
      (`SceneComponent.K2_SetRelativeRotation` (`self.Door Left`) (`KismetMathLibrary.MakeRotator` 0.0 0.0 _left_door_track) false false))))

(event `Close Door`
  (goto _label :!via `Reverse`))

(fn `Interact`
  (params (Interactor :type "Character Object Reference") (`Camera Trans Time` :type "Float (double-precision)"))
  (returns (`Did Interact?` :type Boolean))
  (if (`self.HasWatchedCCTV?`)
    (`/Engine/EditorBlueprintResources/StandardMacros.DoOnce` false
      (:`Completed`
        (`self.Talk To Dan`)
        (`SceneComponent.SetVisibility` (`self.Widget`) false false)
        (return true)))))

(fn `UserConstructionScript`)