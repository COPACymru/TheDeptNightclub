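; Nightclub CCTV door Blueprint that opens and closes on interaction and can launch a QTE sequence.
; Interact toggles DoorClosed and plays the door's skeletal animation forward or in reverse through play rate.
; StartQTE proceeds only while CCTV_Interaction's QTE is incomplete, hiding the player and disabling movement.
; It then calls CallPlayQTE and, after a short delay, moves the player to a hardcoded world location.
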(event `Start QTE`
  (bind _returnvalue (`GameplayStatics.GetActorOfClass` "/Game/GameFiles/Blueprints/CCTV/CCTV_Interaction.CCTV_Interaction_C"))
  (if (not (`/Game/GameFiles/Blueprints/CCTV/CCTV_Interaction.Completed QTE?` _returnvalue))
    (bind _asmale_character (cast `/Game/GameFiles/Characters/Male/MaleCharacter` (`GameplayStatics.GetPlayerCharacter` 0)))
    (`self.SetActorHiddenInGame` _asmale_character true)
    (`CharacterMovementComponent.SetMovementMode` (`Character.CharacterMovement` _asmale_character) "MOVE_None" 0)
    (`self.Play QTE`)
    (`KismetSystemLibrary.Delay` 1.0)
    (`self.K2_SetActorLocation` _asmale_character (2681.999998 6134.985991 1137.756724) false false)))

(event `self.Box.OnComponentBeginOverlap`
  (params (OverlappedComponent :type "PrimitiveComponent Object Reference") (OtherActor :type "Actor Object Reference") (OtherComp :type "PrimitiveComponent Object Reference") (OtherBodyIndex :type Integer) (bFromSweep :type Boolean) (SweepResult :type "HitResult Structure (by ref)")))

(fn `Interact`
  (params (Interactor :type "Character Object Reference") (`Camera Trans Time` :type "Float (double-precision)"))
  (returns (`Did Interact?` :type Boolean))
  (bind _sk_door (`self.SK_Door`))
  (if (`self.Door Closed`)
    (`SkeletalMeshComponent.PlayAnimation` _sk_door "/Game/QAInterrogationRoom/Meshes/SK_Door_Anim.SK_Door_Anim" false)
    (`SkeletalMeshComponent.SetPlayRate` _sk_door 1.0)
    (set `self.Door Closed` false)
    (else
      (`SkeletalMeshComponent.PlayAnimation` _sk_door "/Game/QAInterrogationRoom/Meshes/SK_Door_Anim.SK_Door_Anim" false)
      (`SkeletalMeshComponent.SetPlayRate` _sk_door -1.0)
      (set `self.Door Closed` true)))
  (return false))

(fn `UserConstructionScript`)