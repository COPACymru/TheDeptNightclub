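; Nightclub gate that lowers shut when CloseGate is called, playing closing and slam sounds.
; A Slam flag picks one of two timelines to drive the actor's height, though both updates read GateT2's track.
; Fence collision starts disabled and is re-enabled after a delay only on the non-slam path.
; An "Attacker" leaving the box during closing speeds up both timelines.
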(event `Close Gate`
  (params (`Slam?` :type Boolean))
  (bind (_returnvalue_x _returnvalue_y) (`KismetMathLibrary.BreakVector` (`self.K2_GetActorLocation`)))
  (`AudioComponent.Play` (`self.Metal_Gate_Closing_Isolated_Cue`) 0.0)
  (set `self.GateClosing?` true)
  (if `Slam?`
    (bind (_direction _gate_track) (`Timeline|Gate T`)
      (:`Update`
        (`self.K2_SetActorLocation` (`KismetMathLibrary.MakeVector` _returnvalue_x _returnvalue_y (`KismetMathLibrary.Lerp` 825.0 500.0 (stale _gate_track_2))) :!label _label))
      (:`Finished`
        (`AudioComponent.Play` (`self.Metal_Gate_Closed_Slam_Isolated_Cue`) 0.0 :!label _label_2)
        (`AudioComponent.Stop` (`self.Metal_Gate_Closing_Isolated_Cue`))))
    (else
      (`|ExecutionSequence`
        (:`then_0`
          (bind (_direction_2 _gate_track_2) (`Timeline|Gate T 2`)
            (:`Update`
              (goto _label))
            (:`Finished`
              (goto _label_2))))
        (:`then_1`
          (`KismetSystemLibrary.Delay` 7.0)
          (`PrimitiveComponent.SetCollisionEnabled` (`self.SM_Fence06`) "QueryAndPhysics"))))))

(event `self.ReceiveBeginPlay`
  (`PrimitiveComponent.SetCollisionEnabled` (`self.SM_Fence06`) "NoCollision")
  (`AudioComponent.Stop` (`self.Metal_Gate_Closing_Isolated_Cue`))
  (`AudioComponent.Stop` (`self.Metal_Gate_Closed_Slam_Isolated_Cue`)))

(event `self.Box.OnComponentEndOverlap`
  (params (OverlappedComponent :type "PrimitiveComponent Object Reference") (OtherActor :type "Actor Object Reference") (OtherComp :type "PrimitiveComponent Object Reference") (OtherBodyIndex :type Integer))
  (if (and (`self.ActorHasTag` OtherActor "Attacker") (`self.GateClosing?`))
    (`TimelineComponent.SetPlayRate` (`self.Gate T 2`) 10.0)
    (`TimelineComponent.SetPlayRate` (`self.Gate T`) 10.0)))

(fn `UserConstructionScript`)