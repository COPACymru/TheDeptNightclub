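; Master actor for a group of non-essential evidence (NEE) clues that the player inspects together from a cine camera.
; Interact toggles inspection, blending the view, fading the shared clue widget, swapping input and hiding the player, with optional one-shot radio dialogue.
; Next/previous events lerp camera transform and set focus per EvidenceInfo entry, skipping non-viewable clues and updating the widget.
; A configurable box or sphere volume drives the interact prompt.
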(event `self.ReceiveBeginPlay`
  (bind _sphere (`self.Sphere`))
  (bind _box (`self.Box`))
  (`KismetSystemLibrary.Delay` 1.0)
  (bind _returnvalue (`GameplayStatics.GetActorOfClass` "/Game/GameFiles/Blueprints/Clues/NoneEssentialEvidence/BP_NEE_Component.BP_NEE_Component_C"))
  (set `self.Clue Inspection Widget` (`/Game/GameFiles/Blueprints/Clues/NoneEssentialEvidence/BP_NEE_Component.Clue Inspection Widget` _returnvalue))
  (switch `/Game/GameFiles/Blueprints/Clues/NoneEssentialEvidence/CollisionTypeEnum` (`self.Collision Type`)
    (:`NewEnumerator0`
      (`PrimitiveComponent.SetCollisionEnabled` _box "NoCollision")
      (`SceneComponent.SetVisibility` _box false false)
      (`PrimitiveComponent.SetCollisionEnabled` _sphere "QueryAndPhysics")
      (`SceneComponent.SetVisibility` _sphere true false))
    (:`NewEnumerator1`
      (`PrimitiveComponent.SetCollisionEnabled` _box "QueryAndPhysics")
      (`SceneComponent.SetVisibility` _box true false)
      (`PrimitiveComponent.SetCollisionEnabled` _sphere "NoCollision")
      (`SceneComponent.SetVisibility` _sphere false false))))

(event `Fade UI On`
  (bind _clue_inspection_widget (`self.Clue Inspection Widget`))
  (bind _clue_inspection_widget_2 (`self.Clue Inspection Widget`))
  ;[1 1 1] Fade on and off inspection widget
  (`UserWidget.AddToViewport` _clue_inspection_widget_2 0)
  (`/Game/GameFiles/Blueprints/Clues/W_Tutorial_NEE_Bulk_Inspection.Enable Button` _clue_inspection_widget_2)
  (bind (_direction _fade_track) (`Timeline|Timeline` :!label _label)
    (:`Update`
      (`Widget.SetRenderOpacity` (`/Game/GameFiles/Blueprints/Clues/W_Tutorial_NEE_Bulk_Inspection.CanvasPanel_0` _clue_inspection_widget) _fade_track))
    (:`Finished`
      (switch `ETimelineDirection` _direction
        (:`Backward`
          (`Widget.RemoveFromParent` _clue_inspection_widget))))))

(event `Fade UI Off`
  ;[1 1 1] Fade on and off inspection widget
  (goto _label :!via `Reverse`))

(event `Key|LeftShift`
  (params (Key :type "Key Structure"))
  ;[1 1 1] Stop inspecting
  (:`Pressed`
    (`self.Interact` (`self.Inspector`))))

(event `Should View`
  (params (Condition :type Boolean))
  ;[1 1 1] Should view next/previous clue
  (if (not Condition)
    (`/Engine/EditorBlueprintResources/StandardMacros.DoOnce` false :!label _label_2
      (:`Completed`
        (for _array_element (`self.Evidence Info`)
          (if (`.ShouldView?_11_8AC1C0E3449352F8908F0F86C01364FD` (break `/Game/GameFiles/Blueprints/Clues/NoneEssentialEvidence/NEE_Bulk_STRUCT` _array_element))
            (set `self.Continue?` true)))
        (if (`self.Continue?`)
          (set `self.Continue?` false)
          (if (`self.Forwards?`)
            (`self.Next Index`)
            (`self.Go To Next NEE`)
            (else
              (`self.Previous Index`)
              (`self.Go To Previous NEE`)))
          (`KismetSystemLibrary.Delay` 0.2)
          (goto _label_2 :!via `Reset`))))))

(event `Set Active Clue`
  (bind _clue_inspection_widget (`self.Clue Inspection Widget`))
  (bind (_output_nee _output_cameratransform _output_camerafocusdistance _output_shouldview_) (break `/Game/GameFiles/Blueprints/Clues/NoneEssentialEvidence/NEE_Bulk_STRUCT` (`|GetArrayItem` (`self.Evidence Info`) (`self.Index`))))
  ;[1 1 1] Set active clue in widget
  (if _output_shouldview_
    (set `/Game/GameFiles/Blueprints/Clues/W_Tutorial_NEE_Bulk_Inspection.Clue Name` (`/Game/GameFiles/Blueprints/Clues/NoneEssentialEvidence/BP_NEE_MASTER.Clue Name` _output_nee) _clue_inspection_widget)
    (set `/Game/GameFiles/Blueprints/Clues/W_Tutorial_NEE_Bulk_Inspection.Clue Description` (`/Game/GameFiles/Blueprints/Clues/NoneEssentialEvidence/BP_NEE_MASTER.Clue Description` _output_nee) _clue_inspection_widget)
    (set `/Game/GameFiles/Blueprints/Clues/W_Tutorial_NEE_Bulk_Inspection.Clue ID` (`/Game/GameFiles/Blueprints/Clues/NoneEssentialEvidence/BP_NEE_MASTER.Clue ID` _output_nee) _clue_inspection_widget)
    (set `/Game/GameFiles/Blueprints/Clues/W_Tutorial_NEE_Bulk_Inspection.NEE Clue New` _output_nee _clue_inspection_widget)
    (`/Game/GameFiles/Blueprints/Clues/W_Tutorial_NEE_Bulk_Inspection.Is Evidence Found?` _clue_inspection_widget)))

(event `Go To Next NEE`
  (bind _returnvalue (== (`self.Index`) (- (`KismetArrayLibrary.Array_Length` (`self.Evidence Info`)) 1)))
  (bind (_output_nee _output_cameratransform _output_camerafocusdistance _output_shouldview_) (break `/Game/GameFiles/Blueprints/Clues/NoneEssentialEvidence/NEE_Bulk_STRUCT` (`|GetArrayItem` (`self.Evidence Info`) (`KismetMathLibrary.SelectInt` 0 (+ (`self.Index`) 1) _returnvalue))))
  ;[1 1 1] Go from the current camera location to the next in the array (or beginning of array if at the end)
  (set `self.Forwards?` true)
  (if _output_shouldview_
    (set `self.StartingCameraT` (`SceneComponent.GetRelativeTransform` (`self.CineCamera`)))
    (bind (_direction _camera_track) (`Timeline|Move Camera Next T` :!via `PlayFromStart`)
      (:`Update`
        (`SceneComponent.K2_SetRelativeTransform` (`self.CineCamera`) (`KismetMathLibrary.TLerp` (`self.StartingCameraT`) _output_cameratransform _camera_track) false false)
        (set `CineCameraComponent.FocusSettings` (make `CameraFocusSettings` "Manual" _output_camerafocusdistance) (`self.CineCamera`)))
      (:`Finished`
        (set `self.CacheIndex` (`self.Index`))
        (if _returnvalue :!label _label_3
          (set `self.Index` 0)
          (else
            (`/Engine/EditorBlueprintResources/StandardMacros.IncrementInt` (`self.Index`)
              (:`  `
                _))))
        (`self.Set Active Clue`)))
    (else
      (`self.Should View` _output_shouldview_))))

(event `Next Index`
  ;[1 1 1] Go from the current camera location to the next in the array (or beginning of array if at the end)
  (goto _label_3))

(event `Mark As Evidence`
  ;[1 1 1] Remove clue from bulk view
)

(event `Go To Previous NEE`
  (bind _returnvalue (== (`self.Index`) 0))
  (bind (_output_nee _output_cameratransform _output_camerafocusdistance _output_shouldview_) (break `/Game/GameFiles/Blueprints/Clues/NoneEssentialEvidence/NEE_Bulk_STRUCT` (`|GetArrayItem` (`self.Evidence Info`) (`KismetMathLibrary.SelectInt` (- (`KismetArrayLibrary.Array_Length` (`self.Evidence Info`)) 1) 0 _returnvalue))))
  ;[1 1 1] Go from the current camera location to the previous in the array (or end of array if at the beginning)
  (set `self.Forwards?` false)
  (if _output_shouldview_
    (set `self.StartingCameraT` (`SceneComponent.GetRelativeTransform` (`self.CineCamera`)))
    (bind (_direction _camera_track) (`Timeline|Move Camera Previous T` :!via `PlayFromStart`)
      (:`Update`
        (`SceneComponent.K2_SetRelativeTransform` (`self.CineCamera`) (`KismetMathLibrary.TLerp` (`self.StartingCameraT`) _output_cameratransform _camera_track) false false)
        (set `CineCameraComponent.FocusSettings` (make `CameraFocusSettings` "Manual" _output_camerafocusdistance) (`self.CineCamera`)))
      (:`Finished`
        (set `self.CacheIndex` (`self.Index`))
        (if _returnvalue :!label _label_4
          (set `self.Index` (- (`KismetArrayLibrary.Array_Length` (`self.Evidence Info`)) 1))
          (else
            (`/Engine/EditorBlueprintResources/StandardMacros.DecrementInt` (`self.Index`)
              (:`  `
                _))))
        (`self.Set Active Clue`)))
    (else
      (`self.Should View` _output_shouldview_))))

(event `Play Hughes Radio`
  (`KismetSystemLibrary.Delay` 4.0)
  (`GameplayStatics.PlaySound2D` "/Game/GameFiles/VoiceLines/Tutorial/Hughes/English/10032024/Hughes_Charlie_1_4_Show_Me_At_Scene_Cue.Hughes_Charlie_1_4_Show_Me_At_Scene_Cue" 1.0 1.0 0.0 null null)
  (bind _returnvalue (`|CreateWidget` "/Game/GameFiles/UI/Subtitles/Master/W_Subtitles.W_Subtitles_C" null (make `DataTableRowHandle` "/Game/GameFiles/UI/Subtitles/SubDT_Charlie44ArrivedHughes_ENG.SubDT_Charlie44ArrivedHughes_ENG" "1")))
  (`UserWidget.AddToViewport` _returnvalue 0)
  (`KismetSystemLibrary.Delay` 6.0)
  (`GameplayStatics.PlaySound2D` "/Game/GameFiles/VoiceLines/Tutorial/Hughes/English/10032024/Hughes_Charlie_1_4_Did_You_Recieve_My_last_Cue.Hughes_Charlie_1_4_Did_You_Recieve_My_last_Cue" 1.0 1.0 0.0 null null)
  (bind _returnvalue_2 (`|CreateWidget` "/Game/GameFiles/UI/Subtitles/Master/W_Subtitles.W_Subtitles_C" null (make `DataTableRowHandle` "/Game/GameFiles/UI/Subtitles/SubDT_Charlie14RecieveHughes_ENG.SubDT_Charlie14RecieveHughes_ENG" "1")))
  (`UserWidget.AddToViewport` _returnvalue_2 0)
  (`KismetSystemLibrary.Delay` 3.5)
  (`GameplayStatics.PlaySound2D` "/Game/GameFiles/VoiceLines/Tutorial/Hughes/English/10032024/Hughes_VO_Thing_Doesn_t_Work__Radio_Cue.Hughes_VO_Thing_Doesn_t_Work__Radio_Cue" 1.0 1.0 0.0 null null)
  (bind _returnvalue_3 (`|CreateWidget` "/Game/GameFiles/UI/Subtitles/Master/W_Subtitles.W_Subtitles_C" null (make `DataTableRowHandle` "/Game/GameFiles/UI/Subtitles/SubDT_ThingDoesntWorkHughes_ENG.SubDT_ThingDoesntWorkHughes_ENG" "1")))
  (`UserWidget.AddToViewport` _returnvalue_3 0))

(event `Previous Index`
  ;[1 1 1] Go from the current camera location to the previous in the array (or end of array if at the beginning)
  (goto _label_4))

(event `self.Box.OnComponentBeginOverlap`
  (params (OverlappedComponent :type "PrimitiveComponent Object Reference") (OtherActor :type "Actor Object Reference") (OtherComp :type "PrimitiveComponent Object Reference") (OtherBodyIndex :type Integer) (bFromSweep :type Boolean) (SweepResult :type "HitResult Structure (by ref)"))
  ;[1 1 1] Show/hide interact widget
  (if (and (`self.ActorHasTag` OtherActor "Player") (not (`self.MarkedAsEvidence?`)))
    (message `/Game/GameFiles/GameBlueprints/InteractInterface.Set Interaction Type` OtherActor true)
    (`SceneComponent.SetVisibility` (`self.Interact Widget`) true false)))

(event `self.Sphere.OnComponentBeginOverlap`
  (params (OverlappedComponent :type "PrimitiveComponent Object Reference") (OtherActor :type "Actor Object Reference") (OtherComp :type "PrimitiveComponent Object Reference") (OtherBodyIndex :type Integer) (bFromSweep :type Boolean) (SweepResult :type "HitResult Structure (by ref)"))
  ;[1 1 1] Show/hide interact widget
  (if (and (`self.ActorHasTag` OtherActor "Player") (not (`self.MarkedAsEvidence?`)))
    (message `/Game/GameFiles/GameBlueprints/InteractInterface.Set Interaction Type` OtherActor false)
    (`SceneComponent.SetVisibility` (`self.Interact Widget`) false false)))

(event `self.Sphere.OnComponentEndOverlap`
  (params (OverlappedComponent :type "PrimitiveComponent Object Reference") (OtherActor :type "Actor Object Reference") (OtherComp :type "PrimitiveComponent Object Reference") (OtherBodyIndex :type Integer))
  ;[1 1 1] Show/hide interact widget
  (message `/Game/GameFiles/GameBlueprints/InteractInterface.Set Interaction Type` OtherActor true)
  (`SceneComponent.SetVisibility` (`self.Interact Widget`) true false))

(event `self.Box.OnComponentEndOverlap`
  (params (OverlappedComponent :type "PrimitiveComponent Object Reference") (OtherActor :type "Actor Object Reference") (OtherComp :type "PrimitiveComponent Object Reference") (OtherBodyIndex :type Integer))
  ;[1 1 1] Show/hide interact widget
  (message `/Game/GameFiles/GameBlueprints/InteractInterface.Set Interaction Type` OtherActor false)
  (`SceneComponent.SetVisibility` (`self.Interact Widget`) false false))

(fn `Interact`
  (params (Interactor :type "Character Object Reference") (`Camera Trans Time` :type "Float (double-precision)"))
  (returns (`Did Interact?` :type Boolean))
  (bind _returnvalue (`GameplayStatics.GetPlayerController` 0))
  (bind _returnvalue_2 (`GameplayStatics.GetPlayerController` 0))
  (bind _returnvalue_3 (`GameplayStatics.GetPlayerController` 0))
  (bind _cinecamera (`self.CineCamera`))
  (bind _clue_inspection_widget (`self.Clue Inspection Widget`))
  (bind _clue_inspection_widget_2 (`self.Clue Inspection Widget`))
  (bind _interact_widget (`self.Interact Widget`))
  (bind _is_on_floor_ (`self.Is On Floor?`))
  (bind _output_nee (break `/Game/GameFiles/Blueprints/Clues/NoneEssentialEvidence/NEE_Bulk_STRUCT` (`|GetArrayItem` (`self.Evidence Info`))))
  (bind (_output_nee_2 _output_cameratransform _output_camerafocusdistance) (break `/Game/GameFiles/Blueprints/Clues/NoneEssentialEvidence/NEE_Bulk_STRUCT` (`|GetArrayItem` (`self.Evidence Info`))))
  (if (`self.Is Inspecting`)
    (`PlayerController.SetViewTargetWithBlend` _returnvalue_3 (`local.Interactor`) 0.5 "VTBlend_Linear" 0.0 false)
    (`self.Fade UI Off`)
    (`WidgetBlueprintLibrary.SetInputMode_GameOnly` _returnvalue_2)
    (set `PlayerController.bShowMouseCursor` false _returnvalue_2)
    (set `self.Is Inspecting` false)
    (`self.DisableInput` _returnvalue)
    (`self.EnableInput` Interactor _returnvalue)
    (`self.SetActorHiddenInGame` Interactor false)
    (message `/Game/GameFiles/GameBlueprints/InspectingInterface.IsInspecting?` Interactor false (`self.Is On Floor?`))
    (`SceneComponent.SetVisibility` _interact_widget true false)
    (message `/Game/GameFiles/GameBlueprints/BPI_GameInstance.Add Clue Widget To Screen` (`GameplayStatics.GetGameInstance`))
    (`self.SetActorHiddenInGame` (`local.Interactor`) false)
    (return true)
    (else
      (`CharacterMovementComponent.DisableMovement` (`Character.CharacterMovement` Interactor))
      (`PlayerController.SetViewTargetWithBlend` _returnvalue_3 self 0.5 "VTBlend_Linear" 0.0 false)
      (`self.Fade UI On`)
      (`WidgetBlueprintLibrary.SetInputMode_GameAndUIEx` _returnvalue_2 (`self.Clue Inspection Widget`) "DoNotLock" false)
      (set `PlayerController.bShowMouseCursor` true _returnvalue_2)
      (set `self.Is Inspecting` true)
      (set `/Game/GameFiles/Blueprints/Clues/W_Tutorial_NEE_Bulk_Inspection.Clue Name` (`/Game/GameFiles/Blueprints/Clues/NoneEssentialEvidence/BP_NEE_MASTER.Clue Name` _output_nee) _clue_inspection_widget)
      (set `/Game/GameFiles/Blueprints/Clues/W_Tutorial_NEE_Bulk_Inspection.Clue Description` (`/Game/GameFiles/Blueprints/Clues/NoneEssentialEvidence/BP_NEE_MASTER.Clue Description` _output_nee) _clue_inspection_widget)
      (set `/Game/GameFiles/Blueprints/Clues/W_Tutorial_NEE_Bulk_Inspection.Clue ID` (`/Game/GameFiles/Blueprints/Clues/NoneEssentialEvidence/BP_NEE_MASTER.Clue ID` _output_nee) _clue_inspection_widget)
      (set `self.Clue ID` (`KismetTextLibrary.Conv_NameToText` (`/Game/GameFiles/Blueprints/Clues/NoneEssentialEvidence/BP_NEE_MASTER.Item ID` _output_nee)))
      (`self.DisableInput` Interactor _returnvalue)
      (`self.EnableInput` _returnvalue)
      (set `self.Inspector` Interactor)
      (`/Game/GameFiles/Blueprints/Clues/W_Tutorial_NEE_Bulk_Inspection.Is Evidence Found?` (`self.Clue Inspection Widget`))
      (message `/Game/GameFiles/GameBlueprints/InspectingInterface.IsInspecting?` Interactor _is_on_floor_ _is_on_floor_)
      (`SceneComponent.SetVisibility` _interact_widget false false)
      (set `/Game/GameFiles/Blueprints/Clues/W_Tutorial_NEE_Bulk_Inspection.Clue` null _clue_inspection_widget_2)
      (set `/Game/GameFiles/Blueprints/Clues/W_Tutorial_NEE_Bulk_Inspection.NEEclue` null _clue_inspection_widget_2)
      (set `/Game/GameFiles/Blueprints/Clues/W_Tutorial_NEE_Bulk_Inspection.NEE Clue New` _output_nee_2 _clue_inspection_widget_2)
      (`SceneComponent.K2_SetRelativeTransform` _cinecamera _output_cameratransform false false)
      (set `CineCameraComponent.FocusSettings` (make `CameraFocusSettings` "Manual" _output_camerafocusdistance) _cinecamera)
      (set `/Game/GameFiles/Blueprints/Clues/W_Tutorial_NEE_Bulk_Inspection.Currently Viewed Bulk` self (`self.Clue Inspection Widget`))
      (message `/Game/GameFiles/GameBlueprints/BPI_GameInstance.Remove Clue Widget From Screen` (`GameplayStatics.GetGameInstance`))
      (`self.SetActorHiddenInGame` (`local.Interactor`) true)
      (if (`self.PlayHughesRadio?`)
        (`|ExecutionSequence`
          (:`then_0`
            (`/Engine/EditorBlueprintResources/StandardMacros.DoOnce` false
              (:`Completed`
                (`self.Play Hughes Radio`))))
          (:`then_1`
            (if (not (`self.MarkedAsEvidence?`)) :!label _label
              (message `/Game/GameFiles/GameBlueprints/BPI_GameInstance.Dan Load Check Distance` (`GameplayStatics.GetGameInstance`))
              (return true))))
        (else
          (goto _label))))))

(fn `UserConstructionScript`
  (bind _sphere (`self.Sphere`))
  (bind _box (`self.Box`))
  (`SceneComponent.K2_SetRelativeTransform` (`self.Sphere`) (`self.Sphere Collision Transform`) false false)
  (`SceneComponent.K2_SetRelativeTransform` (`self.Box`) (`self.Box Collision Transform`) false false)
  (switch `/Game/GameFiles/Blueprints/Clues/NoneEssentialEvidence/CollisionTypeEnum` (`self.Collision Type`)
    (:`NewEnumerator0`
      (`PrimitiveComponent.SetCollisionEnabled` _box "NoCollision")
      (`SceneComponent.SetVisibility` _box false false)
      (`PrimitiveComponent.SetCollisionEnabled` _sphere "QueryAndPhysics")
      (`SceneComponent.SetVisibility` _sphere true false))
    (:`NewEnumerator1`
      (`PrimitiveComponent.SetCollisionEnabled` _box "QueryAndPhysics")
      (`SceneComponent.SetVisibility` _box true false)
      (`PrimitiveComponent.SetCollisionEnabled` _sphere "NoCollision")
      (`SceneComponent.SetVisibility` _sphere false false))))