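; Master Blueprint for non-essential evidence clues that the player inspects and marks as evidence.
; At BeginPlay it translates text (English/Welsh) and picks name, description and meshes by killer type, which the construction script previews per variant.
; Interact toggles inspection: a fading UI, optional camera switch, and timeline pick-up with mouse rotate and zoom.
; Marking reveals the bag mesh; overlap shows the prompt, plus a difficulty-dependent outline, unless in a container or bulk.
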(event `self.ReceiveBeginPlay`
  ;[1 1 1] Get a reference to the inspection widget
  (`|ExecutionSequence`
    (:`then_0`
      (`KismetSystemLibrary.Delay` 5.0)
      (bind _clue_inspection_widget (message `/Game/GameFiles/GameBlueprints/BPI_GameInstance.Dan Get Clue Inspect Widget` (`GameplayStatics.GetGameInstance`)))
      (set `self.Clue Inspection Widget` _clue_inspection_widget))
    (:`then_1`
      ;[1 1 1] Call generate clue
      (`self.Translate Clues`)
      (`self.Generate Clue`)
      (`KismetSystemLibrary.Delay` 5.0)
      (set `self.Clue ID` (`KismetTextLibrary.Conv_NameToText` (`self.Item ID`))))
    (:`then_2`
      (set `self.Clue Start Location` (`SceneComponent.K2_GetComponentLocation` (`self.Clue Mesh`)))
      (`self.Get End Location`))))

(event `Fade UI On`
  (bind _clue_inspection_widget (`self.Clue Inspection Widget`))
  ;[1 1 1] Fade on and off inspection widget
  (`UserWidget.AddToViewport` (`self.Clue Inspection Widget`) 0)
  (`/Game/GameFiles/Blueprints/Clues/TutorialClueInspection.Enable Button` (`self.Clue Inspection Widget`))
  (bind (_direction _fade_track) (`Timeline|Timeline` :!label _label)
    (:`Update`
      (`Widget.SetRenderOpacity` (`/Game/GameFiles/Blueprints/Clues/TutorialClueInspection.Border_42` _clue_inspection_widget) _fade_track))
    (:`Finished`
      (switch `ETimelineDirection` _direction
        (:`Backward`
          (`Widget.RemoveFromParent` _clue_inspection_widget))))))

(event `Set Clue`
  (params (`Clue Name` :type Text) (`Clue Description` :type Text) (`Clue Mesh` :type "StaticMesh Object Reference") (`Bag Mesh` :type "StaticMesh Object Reference") (`Body Mesh` :type "SkeletalMesh Object Reference"))
  ;[1 1 1] Dynamically set clue
  (set `self.Clue Name` `Clue Name`)
  (set `self.Clue Description` `Clue Description`)
  (set `self.Clue Item` `Clue Mesh`)
  (set `self.Bag Item` `Bag Mesh`)
  (`StaticMeshComponent.SetStaticMesh` (`self.Clue Mesh`) (`self.Clue Item`))
  (`StaticMeshComponent.SetStaticMesh` (`self.Bag Mesh`) (`self.Bag Item`)))

(event `Translate Clues`
  ;[1 1 1] Translate clue
  (bind _language (message `/Game/GameFiles/GameBlueprints/BPI_GameInstance.Get Language` (`GameplayStatics.GetGameInstance`)))
  (switch `/Game/GameFiles/GameBlueprints/LanguageEnum` _language
    (:`NewEnumerator0`
      (set `self.Visionary Clue Name ENG` (`self.Visionary Clue Name ENG`))
      (set `self.Visionary Clue Description ENG` (`self.Visionary Clue Description ENG`))
      (set `self.Mission Oriented Clue Name ENG` (`self.Mission Oriented Clue Name ENG`))
      (set `self.Mission Oriented Clue Description ENG` (`self.Mission Oriented Clue Description ENG`))
      (set `self.Hedonistic Clue Name ENG` (`self.Hedonistic Clue Name ENG`))
      (set `self.Hedonistic Clue Description ENG` (`self.Hedonistic Clue Description ENG`))
      (set `self.Power Clue Name ENG` (`self.Power Clue Name ENG`))
      (set `self.Power Clue Description ENG` (`self.Power Clue Description ENG`)))
    (:`NewEnumerator1`
      (set `self.Visionary Clue Name ENG` (`self.Visionary Clue Name CYM`))
      (set `self.Visionary Clue Description ENG` (`self.Visionary Clue Description CYM`))
      (set `self.Mission Oriented Clue Name ENG` (`self.Mission Oriented Clue Name CYM`))
      (set `self.Mission Oriented Clue Description ENG` (`self.Mission Oriented Clue Description CYM`))
      (set `self.Hedonistic Clue Name ENG` (`self.Hedonistic Clue Name CYM`))
      (set `self.Hedonistic Clue Description ENG` (`self.Hedonistic Clue Description CYM`))
      (set `self.Power Clue Name ENG` (`self.Power Clue Name CYM`))
      (set `self.Power Clue Description ENG` (`self.Power Clue Description CYM`)))))

(event `Fade UI Off`
  ;[1 1 1] Fade on and off inspection widget
  (goto _label :!via `Reverse`))

(event `InputAction|Interact`
  (params (Key :type "Key Structure"))
  ;[1 1 1] Stop inspecting
  (:`Pressed`
    (`self.Interact` (`self.Inspector`))))

(event `Set Clue ID`
  ;[1 1 1] Set clue ID
  (set `self.Clue ID` (`KismetTextLibrary.Conv_StringToText` (`KismetStringLibrary.Split` (`KismetStringLibrary.Conv_NameToString` (`self.Item ID`)) "I"))))

(event `Generate Clue`
  ;[1 1 1] Generate clue based on killer type
  (bind _killer_type (message `/Game/GameFiles/GameBlueprints/BPI_GameInstance.Get Killer Type` (`GameplayStatics.GetGameInstance`)))
  (switch `/Game/GameFiles/Blueprints/Clues/KillerTypeEnum` _killer_type
    (:`NewEnumerator1`
      (`self.Set Clue` (`self.Visionary Clue Name ENG`) (`self.Visionary Clue Description ENG`) (`self.Visionary Clue Mesh`) (`self.Visionary Bag mesh`)))
    (:`NewEnumerator2`
      (`self.Set Clue` (`self.Mission Oriented Clue Name ENG`) (`self.Mission Oriented Clue Description ENG`) (`self.Mission Oriented Clue Mesh`) (`self.Mission Oriented Bag Mesh`)))
    (:`NewEnumerator3`
      (`self.Set Clue` (`self.Hedonistic Clue Name ENG`) (`self.Hedonistic Clue Description ENG`) (`self.Hedonistic Clue Mesh`) (`self.Hedonistic Bag Mesh`)))
    (:`NewEnumerator4`
      (`self.Set Clue` (`self.Power Clue Name ENG`) (`self.Power Clue Description ENG`) (`self.Power Clue Mesh`) (`self.Power Bag Mesh`)))))

(event `Is Clue Marked As Evidence - Master`
  ;[1 1 1] Is clue marked as evidence? - Master
  (`self.Is Clue Marked As Evidence`))

(event `Is Clue Marked As Evidence`
  ;[1 1 1] Is clue marked as evidence? - Mission 1
  (if (`self.MarkedAsEvidence?`)
    (if (`self.IsInBulk?`)
      (bind _returnvalue (`GameplayStatics.GetActorOfClass` "/Game/GameFiles/Blueprints/Clues/NoneEssentialEvidence/BP_NEE_Component.BP_NEE_Component_C"))
      (`/Game/GameFiles/Blueprints/Clues/W_Tutorial_NEE_Bulk_Inspection.Disable NEE Bulk` (`/Game/GameFiles/Blueprints/Clues/NoneEssentialEvidence/BP_NEE_Component.Clue Inspection Widget` _returnvalue))
      (else
        (`/Game/GameFiles/Blueprints/Clues/TutorialClueInspection.Disable Button` (`self.Clue Inspection Widget`))))
    (else
      (`/Engine/EditorBlueprintResources/StandardMacros.DoOnce` false
        (:`Completed`
          (set `self.MarkedAsEvidence?` true)
          (`SceneComponent.SetHiddenInGame` (`self.Clue Mesh`) (`self.Should Hide Clue?`) false)
          (`SceneComponent.SetHiddenInGame` (`self.Bag Mesh`) false false)
          (`GameplayStatics.PlaySound2D` (`self.Radio Confirmation To Play`) 1.0 1.0 0.0 null null)
          (if (`self.IsInBulk?`)
            (bind _returnvalue_2 (`GameplayStatics.GetActorOfClass` "/Game/GameFiles/Blueprints/Clues/NoneEssentialEvidence/BP_NEE_Component.BP_NEE_Component_C"))
            (`/Game/GameFiles/Blueprints/Clues/W_Tutorial_NEE_Bulk_Inspection.Disable "Mark As Evidence Button" NEE New` (`/Game/GameFiles/Blueprints/Clues/NoneEssentialEvidence/BP_NEE_Component.Clue Inspection Widget` _returnvalue_2))
            (else
              (`/Game/GameFiles/Blueprints/Clues/TutorialClueInspection.Disable "Mark As Evidence Button" NEE New` (`self.Clue Inspection Widget`)))))))))

(event `self.Sphere Collision.OnComponentBeginOverlap`
  (params (OverlappedComponent :type "PrimitiveComponent Object Reference") (OtherActor :type "Actor Object Reference") (OtherComp :type "PrimitiveComponent Object Reference") (OtherBodyIndex :type Integer) (bFromSweep :type Boolean) (SweepResult :type "HitResult Structure (by ref)"))
  ;[1 1 1] Show/hide object outline
  (if (and (`self.ActorHasTag` OtherActor "Player") (not (`self.MarkedAsEvidence?`)))
    (if (not (or (`self.In Container?`) (`self.IsInBulk?`)))
      (message `/Game/GameFiles/GameBlueprints/InteractInterface.Set Interaction Type` OtherActor true)
      (`SceneComponent.SetVisibility` (`self.Interact Widget`) true false)
      (bind _difficulty (message `/Game/GameFiles/GameBlueprints/BPI_GameInstance.Get Difficulty` (`GameplayStatics.GetGameInstance`)))
      (if (`|EnumEquality` _difficulty "NewEnumerator0")
        (`PrimitiveComponent.SetRenderCustomDepth` (`self.Clue Mesh`) true)))))

(event `self.Sphere Collision.OnComponentEndOverlap`
  (params (OverlappedComponent :type "PrimitiveComponent Object Reference") (OtherActor :type "Actor Object Reference") (OtherComp :type "PrimitiveComponent Object Reference") (OtherBodyIndex :type Integer))
  ;[1 1 1] Show/hide object outline
  (if (not (or (`self.In Container?`) (`self.IsInBulk?`)))
    (`SceneComponent.SetVisibility` (`self.Interact Widget`) false false)))

(event `Load Evidence Bag`
  ;[1 1 1] Is clue marked as evidence? - Mission 1
  (`SceneComponent.SetHiddenInGame` (`self.Clue Mesh`) (`self.Should Hide Clue?`) false)
  (`SceneComponent.SetHiddenInGame` (`self.Bag Mesh`) false false))

(event `InputAxisKey|MouseX`
  (params (AxisValue :type "Float (single-precision)"))
  ;[1 1 1] Rotate clue
  (`/Engine/EditorBlueprintResources/StandardMacros.Gate` true :!label _label_2
    (:`Exit`
      (if (`self.Can Pick Up?`)
        (`SceneComponent.K2_SetRelativeRotation` (`self.Clue Mesh`) (`KismetMathLibrary.ComposeRotators` (`SceneComponent.RelativeRotation` (`self.Clue Mesh`)) (`KismetMathLibrary.MakeRotator` (* AxisValue 1.0) (* (stale `InputAxisKey|MouseY` AxisValue) -1.0))) false false)))))

(event `Pick Up Clue`
  (params (`Can Pick Up?` :type Boolean))
  ;[1 1 1] Pick up/put down clue
  (if `Can Pick Up?`
    (bind (_direction _clue_track) (`Timeline|Timeline_0` :!label _label_3)
      (:`Update`
        (`SceneComponent.K2_SetWorldLocation` (`self.Clue Mesh`) (`KismetMathLibrary.VLerp` (`self.Clue Start Location`) (`self.Clue End Location`) _clue_track) false false)))))

(event `InputAxisKey|MouseY`
  (params (AxisValue :type "Float (single-precision)"))
  ;[1 1 1] Rotate clue
  (goto _label_2))

(event `Put Down Clue`
  (params (`Can Pick Up?` :type Boolean))
  ;[1 1 1] Pick up/put down clue
  (if `Can Pick Up?`
    (goto _label_3 :!via `Reverse`)))

(event `InputAction|Inspect` :consume false
  (params (Key :type "Key Structure"))
  ;[1 1 1] Rotate clue
  (:`Pressed`
    (goto _label_2 :!via `Open`))
  (:`Released`
    (goto _label_2 :!via `Close`)))

(event `Get End Location`
  (bind _cinecamera (`self.CineCamera`))
  (bind _returnvalue (`SceneComponent.K2_GetComponentLocation` _cinecamera))
  ;[1 1 1] Get end location for picking up clue
  (bind _outhit (`KismetSystemLibrary.LineTraceSingle` _returnvalue (+ _returnvalue (* (`SceneComponent.GetForwardVector` _cinecamera) (`self.Pick Up Amount`))) "TraceTypeQuery1"))
  (set `self.Clue End Location` (`.TraceEnd` (`GameplayStatics.BreakHitResult` _outhit))))

(event `Key|MouseScrollUp`
  (params (Key :type "Key Structure"))
  ;[1 1 1] Zoom in clue
  (:`Pressed`
    (if (`self.Can Pick Up?`)
      (`CameraComponent.SetFieldOfView` (`self.CineCamera`) (`KismetMathLibrary.FClamp` (+ (`CameraComponent.FieldOfView` (`self.CineCamera`)) 2.0) 70.0 90.0)))))

(event `Key|MouseScrollDown`
  (params (Key :type "Key Structure"))
  ;[1 1 1] Zoom in clue
  (:`Pressed`
    (if (`self.Can Pick Up?`)
      (`CameraComponent.SetFieldOfView` (`self.CineCamera`) (`KismetMathLibrary.FClamp` (- (`CameraComponent.FieldOfView` (`self.CineCamera`)) 2.0) 70.0 90.0)))))

(fn `Interact`
  (params (Interactor :type "Character Object Reference") (`Camera Trans Time` :type "Float (double-precision)"))
  (returns (`Did Interact?` :type Boolean))
  (bind _returnvalue (`GameplayStatics.GetPlayerController` 0))
  (bind _returnvalue_2 (`GameplayStatics.GetPlayerController` 0))
  (bind _returnvalue_3 (`GameplayStatics.GetPlayerController` 0))
  (bind _can_pick_up_ (`self.Can Pick Up?`))
  (bind _is_on_floor_ (`self.Is On Floor?`))
  (bind _clue_inspection_widget (`self.Clue Inspection Widget`))
  (bind _clue_inspection_widget_2 (`self.Clue Inspection Widget`))
  (bind _usecamera_ (`self.UseCamera?`))
  (bind _interactor (`local.Interactor`))
  (bind _interact_widget (`self.Interact Widget`))
  (bind _returnvalue_4 (`KismetTextLibrary.Conv_NameToText` (`self.Item ID`)))
  (if (or (`self.In Container?`) (`self.IsInBulk?`))
    _
    (elif (`self.Can Inspect?`)
      (if (`self.Is Inspecting`)
        (`self.Fade UI Off`)
        (`WidgetBlueprintLibrary.SetInputMode_GameOnly` _returnvalue_3)
        (set `PlayerController.bShowMouseCursor` false _returnvalue_3)
        (set `self.Is Inspecting` false)
        (`self.DisableInput` _returnvalue_2)
        (`self.EnableInput` Interactor _returnvalue_2)
        (`self.SetActorHiddenInGame` Interactor false)
        (message `/Game/GameFiles/GameBlueprints/InspectingInterface.IsInspecting?` Interactor false (`self.Is On Floor?`))
        (`SceneComponent.SetVisibility` _interact_widget false false)
        (`self.Put Down Clue` _can_pick_up_)
        (if _usecamera_
          (`PlayerController.SetViewTargetWithBlend` _returnvalue _interactor 0.0 "VTBlend_Linear" 0.0 false)
          (`self.SetActorHiddenInGame` _interactor false))
        (return true)
        (else
          (`CharacterMovementComponent.DisableMovement` (`Character.CharacterMovement` Interactor))
          (`self.Fade UI On`)
          (`WidgetBlueprintLibrary.SetInputMode_GameAndUIEx` _returnvalue_3 (`self.Clue Inspection Widget`) "DoNotLock" false)
          (set `PlayerController.bShowMouseCursor` true _returnvalue_3)
          (set `self.Is Inspecting` true)
          (set `/Game/GameFiles/Blueprints/Clues/TutorialClueInspection.Clue Name` (`self.Clue Name`) _clue_inspection_widget)
          (set `/Game/GameFiles/Blueprints/Clues/TutorialClueInspection.Clue Description` (`self.Clue Description`) _clue_inspection_widget)
          (set `/Game/GameFiles/Blueprints/Clues/TutorialClueInspection.Clue ID` _returnvalue_4 _clue_inspection_widget)
          (set `self.Clue ID` _returnvalue_4)
          (`self.DisableInput` Interactor _returnvalue_2)
          (`self.EnableInput` _returnvalue_2)
          (set `self.Inspector` Interactor)
          (`/Game/GameFiles/Blueprints/Clues/TutorialClueInspection.Is Evidence Found?` (`self.Clue Inspection Widget`))
          (message `/Game/GameFiles/GameBlueprints/InspectingInterface.IsInspecting?` Interactor _is_on_floor_ _is_on_floor_)
          (`SceneComponent.SetVisibility` _interact_widget false false)
          (set `/Game/GameFiles/Blueprints/Clues/TutorialClueInspection.Clue` null _clue_inspection_widget_2)
          (set `/Game/GameFiles/Blueprints/Clues/TutorialClueInspection.NEEclue` null _clue_inspection_widget_2)
          (set `/Game/GameFiles/Blueprints/Clues/TutorialClueInspection.NEE Clue New` self _clue_inspection_widget_2)
          (`self.Pick Up Clue` _can_pick_up_)
          (if _usecamera_
            (`PlayerController.SetViewTargetWithBlend` _returnvalue self 0.0 "VTBlend_Linear" 0.0 false)
            (`self.SetActorHiddenInGame` _interactor true))
          (`|ExecutionSequence`
            (:`then_0`
              (`PlayerCameraManager.StopAllCameraShakes` (`GameplayStatics.GetPlayerCameraManager` 0) true))
            (:`then_1`
              (if (== (`self.Item ID`) "AGPhone")
                (`GameplayStatics.PlaySound2D` "/Game/GameFiles/VoiceLines/Tutorial/Morgan/English/CCTV_Sequence/New/its_time_strange_Cue.its_time_strange_Cue" 1.0 1.0 0.0 null null)
                (bind _returnvalue_5 (`|CreateWidget` "/Game/GameFiles/UI/Subtitles/Master/W_Subtitles.W_Subtitles_C" null (make `DataTableRowHandle` "/Game/GameFiles/UI/Subtitles/SubDT_ItsTime_ENG.SubDT_ItsTime_ENG" "1")))
                (`UserWidget.AddToViewport` _returnvalue_5 0)
                (if (not (`self.MarkedAsEvidence?`))
                  (message `/Game/GameFiles/GameBlueprints/BPI_GameInstance.Dan Load Check Distance` (`GameplayStatics.GetGameInstance`))
                  (return true))))))))))

(fn `UserConstructionScript`
  (bind _visionary_bag_size (`self.Visionary Bag Size`))
  (bind _mission_oriented_bag_size (`self.Mission Oriented Bag Size`))
  (bind _visionary_clue_size (`self.Visionary Clue Size`))
  (bind _power_bag_size (`self.Power Bag Size`))
  (bind _power_clue_size (`self.Power Clue Size`))
  (bind _mission_oriented_clue_size (`self.Mission Oriented Clue Size`))
  (bind _hedonistic_clue_size (`self.Hedonistic Clue Size`))
  (bind _hedonistic_bag_size (`self.Hedonistic Bag Size`))
  ;[1 1 1] Set interact widget transform
  (`SceneComponent.K2_SetRelativeTransform` (`self.Interact Widget`) (`self.InteractionWidgetTransform`) false false)
  ;[1 1 1] Set preview for different killer types
  (switch `/Game/GameFiles/Blueprints/Clues/KillerTypeEnum` (`self.Preview Clue Variation`)
    (:`NewEnumerator1`
      ;[1 1 1] General clue details
      (`StaticMeshComponent.SetStaticMesh` (`self.Bag Mesh`) (`self.Visionary Bag Mesh`))
      (`StaticMeshComponent.SetStaticMesh` (`self.Clue Mesh`) (`self.Visionary Clue Mesh`))
      (`SceneComponent.SetRelativeScale3D` (`self.Clue Mesh`) (`KismetMathLibrary.MakeVector` _visionary_clue_size _visionary_clue_size _visionary_clue_size))
      (`SceneComponent.K2_SetRelativeRotation` (`self.Clue Mesh`) (`KismetMathLibrary.MakeRotator` (`self.Visionary Clue Rotation X`) (`self.Visionary Clue Rotation Y`) (`self.Visionary Clue Rotation Z`)) false false)
      (`SceneComponent.K2_SetRelativeTransform` (`self.Sphere Collision`) (`self.Visionary Collision Transform`) false false)
      (`SceneComponent.K2_SetRelativeLocation` (`self.Clue Mesh`) (`self.Visionary Clue Location`) false false)
      ;[1 1 1] Generate bag details
      (`SceneComponent.SetRelativeScale3D` (`self.Bag Mesh`) (`KismetMathLibrary.MakeVector` _visionary_bag_size _visionary_bag_size _visionary_bag_size))
      (`SceneComponent.K2_SetRelativeRotation` (`self.Bag Mesh`) (`KismetMathLibrary.MakeRotator` (`self.Visionary Bag Rotation X`) (`self.Visionary Bag Rotation Y`) (`self.Visionary Bag Rotation Z`)) false false)
      (`SceneComponent.K2_SetRelativeLocation` (`self.Bag Mesh`) (`self.Visionary Bag Location`) false false))
    (:`NewEnumerator2`
      (`StaticMeshComponent.SetStaticMesh` (`self.Bag Mesh`) (`self.Mission Oriented Bag Mesh`))
      (`StaticMeshComponent.SetStaticMesh` (`self.Clue Mesh`) (`self.Mission Oriented Clue Mesh`))
      (`SceneComponent.SetRelativeScale3D` (`self.Clue Mesh`) (`KismetMathLibrary.MakeVector` _mission_oriented_clue_size _mission_oriented_clue_size _mission_oriented_clue_size))
      (`SceneComponent.K2_SetRelativeRotation` (`self.Clue Mesh`) (`KismetMathLibrary.MakeRotator` (`self.Mission Oriented Clue Rotation X`) (`self.Mission Oriented Clue Rotation Y`) (`self.Mission Oriented Clue Rotation Z`)) false false)
      (`SceneComponent.K2_SetRelativeTransform` (`self.Sphere Collision`) (`self.Mission Oriented Collision Transform`) false false)
      (`SceneComponent.K2_SetRelativeLocation` (`self.Clue Mesh`) (`self.Mission Oriented Clue Location`) false false)
      (`SceneComponent.SetRelativeScale3D` (`self.Bag Mesh`) (`KismetMathLibrary.MakeVector` _mission_oriented_bag_size _mission_oriented_bag_size _mission_oriented_bag_size))
      (`SceneComponent.K2_SetRelativeRotation` (`self.Bag Mesh`) (`KismetMathLibrary.MakeRotator` (`self.Mission Oriented Bag Rotation X`) (`self.Mission Oriented Bag Rotation Y`) (`self.Mission Oriented Bag Rotation Z`)) false false)
      (`SceneComponent.K2_SetRelativeLocation` (`self.Bag Mesh`) (`self.Mission Oriented Bag Location`) false false))
    (:`NewEnumerator3`
      (`StaticMeshComponent.SetStaticMesh` (`self.Bag Mesh`) (`self.Hedonistic Bag Mesh`))
      (`StaticMeshComponent.SetStaticMesh` (`self.Clue Mesh`) (`self.Hedonistic Clue Mesh`))
      (`SceneComponent.SetRelativeScale3D` (`self.Clue Mesh`) (`KismetMathLibrary.MakeVector` _hedonistic_clue_size _hedonistic_clue_size _hedonistic_clue_size))
      (`SceneComponent.K2_SetRelativeRotation` (`self.Clue Mesh`) (`KismetMathLibrary.MakeRotator` (`self.Hedonistic Clue Rotation X`) (`self.Hedonistic Clue Rotation Y`) (`self.Hedonistic Clue Rotation Z`)) false false)
      (`SceneComponent.K2_SetRelativeTransform` (`self.Sphere Collision`) (`self.Hedonistic Collision Transform`) false false)
      (`SceneComponent.K2_SetRelativeLocation` (`self.Clue Mesh`) (`self.Hedonistic Clue Location`) false false)
      (`SceneComponent.SetRelativeScale3D` (`self.Bag Mesh`) (`KismetMathLibrary.MakeVector` _hedonistic_bag_size _hedonistic_bag_size _hedonistic_bag_size))
      (`SceneComponent.K2_SetRelativeRotation` (`self.Bag Mesh`) (`KismetMathLibrary.MakeRotator` (`self.Hedonistic Bag Rotation X`) (`self.Hedonistic Bag Rotation Y`) (`self.Hedonistic Bag Rotation Z`)) false false)
      (`SceneComponent.K2_SetRelativeLocation` (`self.Bag Mesh`) (`self.Hedonistic Bag Location`) false false))
    (:`NewEnumerator4`
      (`StaticMeshComponent.SetStaticMesh` (`self.Bag Mesh`) (`self.Power Bag Mesh`))
      (`StaticMeshComponent.SetStaticMesh` (`self.Clue Mesh`) (`self.Power Clue Mesh`))
      (`SceneComponent.SetRelativeScale3D` (`self.Clue Mesh`) (`KismetMathLibrary.MakeVector` _power_clue_size _power_clue_size _power_clue_size))
      (`SceneComponent.K2_SetRelativeRotation` (`self.Clue Mesh`) (`KismetMathLibrary.MakeRotator` (`self.Power Clue Rotation X`) (`self.Power Clue Rotation Y`) (`self.Power Clue Rotation Z`)) false false)
      (`SceneComponent.K2_SetRelativeTransform` (`self.Sphere Collision`) (`self.Power Collision Transform`) false false)
      (`SceneComponent.K2_SetRelativeLocation` (`self.Clue Mesh`) (`self.Power Clue Location`) false false)
      (`SceneComponent.SetRelativeScale3D` (`self.Bag Mesh`) (`KismetMathLibrary.MakeVector` _power_bag_size _power_bag_size _power_bag_size))
      (`SceneComponent.K2_SetRelativeRotation` (`self.Bag Mesh`) (`KismetMathLibrary.MakeRotator` (`self.Power Bag Rotation X`) (`self.Power Bag Rotation Y`) (`self.Power Bag Rotation Z`)) false false)
      (`SceneComponent.K2_SetRelativeLocation` (`self.Bag Mesh`) (`self.Power Bag Location`) false false))))