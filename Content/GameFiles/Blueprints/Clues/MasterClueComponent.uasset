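; Clue manager component that sets up each mission's clue lists, tracks found evidence and mirrors it into the game instance.
; On a mission's first load it shuffles each of six clue classes and destroys all but one actor, recording destroyed IDs.
; Marking evidence saves found flags, and BeginPlay restores state via per-slot, per-mission dispatch, though only save slot 1 is implemented.
; It also creates the clue inspection widget and can check whether all clues are found.
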(event `Save Clue Locations`
  ;[1 1 1] Save clue locations - Master
  (bind _current_save_slot (message `/Game/GameFiles/GameBlueprints/BPI_GameInstance.Get Current Save Slot` (`GameplayStatics.GetGameInstance`)))
  (switch `int` (- (`KismetStringLibrary.Conv_StringToInt` (`KismetStringLibrary.GetSubstring` _current_save_slot 4)) 1)
    (:`0`
      (`self.Save Clue Locations - Slot 1`))))

(event `Destroy Item`
  (params (`Item ID` :type "Name (by ref)"))
  ;[1 1 1] Set clue locations
  (`KismetArrayLibrary.Array_Add` (`self.DestroyedActors`) `Item ID`))

(event `Load Clue Locations`
  ;[1 1 1] Load clue locations - Master
  (bind _current_save_slot (message `/Game/GameFiles/GameBlueprints/BPI_GameInstance.Get Current Save Slot` (`GameplayStatics.GetGameInstance`)))
  (switch `int` (- (`KismetStringLibrary.Conv_StringToInt` (`KismetStringLibrary.GetSubstring` _current_save_slot 4)) 1)
    (:`0`
      (`self.Load Clue Locations - Slot 1`))))

(event `Save Clue Locations - Slot 1`
  ;[1 1 1] Save clue locations - Slot 1
  (bind _current_save_slot (message `/Game/GameFiles/GameBlueprints/BPI_GameInstance.Get Current Save Slot` (`GameplayStatics.GetGameInstance`)))
  (bind _returnvalue (`GameplayStatics.LoadGameFromSlot` _current_save_slot))
  (bind _assave_slot_1 (cast `/Game/GameFiles/SaveGames/SaveSlot1` _returnvalue))
  (bind _output_get (set `self.Save Slot 1` _assave_slot_1))
  (set `/Game/GameFiles/SaveGames/SaveSlot1.DestroyedActors` (`self.DestroyedActors`) _output_get)
  (`GameplayStatics.SaveGameToSlot` (`self.Save Slot 1`) ""))

(event `Load Clue Locations - Slot 1`
  ;[1 1 1] Load clue locations - Slot 1
  (bind _current_save_slot (message `/Game/GameFiles/GameBlueprints/BPI_GameInstance.Get Current Save Slot` (`GameplayStatics.GetGameInstance`)))
  (bind _returnvalue (`GameplayStatics.LoadGameFromSlot` _current_save_slot))
  (bind _assave_slot_1 (cast `/Game/GameFiles/SaveGames/SaveSlot1` _returnvalue))
  (bind _output_get (set `self.Save Slot 1` _assave_slot_1))
  (set `self.DestroyedActors` (`/Game/GameFiles/SaveGames/SaveSlot1.DestroyedActors` _output_get)))

(event `self.ReceiveBeginPlay`
  (`|ExecutionSequence`
    (:`then_0`
      ;[1 1 1] Create inspection widget
      (bind _returnvalue (`|CreateWidget` "/Game/GameFiles/Blueprints/Clues/ClueInspection.ClueInspection_C"))
      (bind _output_get (set `self.Clue Inspection Widget` _returnvalue))
      (`UserWidget.AddToViewport` _output_get 0)
      ;[1 1 1] Set up clues
      (`self.Set Up Clues Arrays`))
    (:`then_1`
      ;[1 1 1] Randomly spawn clues on the first time level load up
      (bind (_mission_1_loaded_ _mission_2_loaded_ _mission_3_loaded_ _mission_4_loaded_ _mission_5_loaded_) (message `/Game/GameFiles/GameBlueprints/BPI_GameInstance.Get Missions Loaded` (`GameplayStatics.GetGameInstance`)))
      (if (select `/Game/GameFiles/Blueprints/Clues/MissionEnum` (`self.Mission Select`) :`NewEnumerator0` _mission_1_loaded_ :`NewEnumerator1` _mission_2_loaded_ :`NewEnumerator2` _mission_3_loaded_ :`NewEnumerator3` _mission_4_loaded_ :`NewEnumerator4` _mission_5_loaded_)
        (`self.Load Clue Locations`)
        (`self.Load Clues Found - Master`)
        (else
          (`self.Load Clue Locations`)
          (`KismetSystemLibrary.Delay` 0.2)
          (`self.Randomly Spawn Clue 1`)
          (`self.Randomly Spawn Clue 2`)
          (`self.Randomly Spawn Clue 3`)
          (`self.Randomly Spawn Clue 4`)
          (`self.Randomly Spawn Clue 5`)
          (`self.Randomly Spawn Clue 6`)
          (`KismetSystemLibrary.Delay` 2.0)
          (`self.Save Clue Locations`))))))

(event `Set Up Clue Array - Police Station`
  ;[1 1 1] Set up clue arrays - Police Station
  (`self.Set Up Clue Array - Mission 1`)
  (`self.Set Up Clue Array - Mission 2`)
  (`self.Set Up Clue Array - Mission 3`)
  (`self.Set Up Clue Array - Mission 4`)
  (`self.Set Up Clue Array - Mission 5`))

(event `Randomly Spawn Clue 1`
  ;[1 1 1] Randomly spawn clue 1
  (bind _outactors (`GameplayStatics.GetAllActorsOfClass` "/Game/GameFiles/Blueprints/Clues/Clue1BP.Clue1BP_C"))
  (`KismetArrayLibrary.Array_Shuffle` _outactors)
  (bind _returnvalue (`KismetArrayLibrary.Array_Length` _outactors))
  (set `self.Clue 1 Total` _returnvalue)
  (for _index (range (+ (- _returnvalue 2) 1))
    (bind _output (`|GetArrayItem` _outactors _index))
    (`self.Destroy Item` (`/Game/GameFiles/Blueprints/Clues/Clue1BP.Item ID` _output))
    (`self.K2_DestroyActor` _output)
    (`/Engine/EditorBlueprintResources/StandardMacros.DecrementInt` (`self.Clue 1 Total`))))

(event `Mark Clue For Evidence - Mission 1`
  (params (`Clue Name` :type Text))
  ;[1 1 1] Mark clue as evidence - Mission 1
  (for (_array_element _array_index) (`self.Mission 1 Clues`)
    (if (`KismetTextLibrary.EqualEqual_TextText` _array_element `Clue Name`)
      (`KismetArrayLibrary.Array_Set` (`self.Mission 1 Clues Found`) _array_index true)
      ;;[1 1 1] Update game instance clues
      (bind (_clues _clues_found) (message `/Game/GameFiles/GameBlueprints/BPI_GameInstance.Get Mission 1 Clues Info` (`GameplayStatics.GetGameInstance`) :!label _label))
      (`KismetArrayLibrary.Array_Set` _clues_found _array_index true)
      (`self.Save Clues Found - Master`)))
  (goto _label))

(event `Set Up Clue Array - Mission 1`
  ;[1 1 1] Set up clue arrays - Mission 1
  (for _ (`self.Mission 1 Clues`)
    (`KismetArrayLibrary.Array_Add` (`self.Mission 1 Clues Found`)))
  ;[1 1 1] Set up clues in the game instance - Mission 1
  (bind (_clues _clues_found _pictures) (message `/Game/GameFiles/GameBlueprints/BPI_GameInstance.Get Mission 1 Clues Info` (`GameplayStatics.GetGameInstance`)))
  (for _array_element (`self.Mission 1 Clues`)
    (`KismetArrayLibrary.Array_Add` _clues _array_element))
  (for _array_element_2 (`self.Mission 1 Clues Found`)
    (`KismetArrayLibrary.Array_Add` _clues_found _array_element_2))
  (for _array_element_3 (`self.Mission 1 Clue Pictures`)
    (`KismetArrayLibrary.Array_Add` _pictures _array_element_3)))

(event `Load Clues Found - Master`
  ;[1 1 1] Load clues found - Master
  (bind _current_save_slot (message `/Game/GameFiles/GameBlueprints/BPI_GameInstance.Get Current Save Slot` (`GameplayStatics.GetGameInstance`)))
  (bind _output_get (set `self.Current Save Slot` _current_save_slot))
  (switch `int` (- (`KismetStringLibrary.Conv_StringToInt` (`KismetStringLibrary.GetSubstring` _output_get 4)) 1)
    (:`0`
      (`self.Load Clues Found - Slot 1`))))

(event `Set Up Clues Arrays`
  ;[1 1 1] Set up clue arrays  - Master
  (switch `/Game/GameFiles/Blueprints/Clues/MissionEnum` (`self.Mission Select`)
    (:`NewEnumerator5`
      (`self.Set Up Clue Array - Police Station`))
    (:`NewEnumerator0`
      (`self.Set Up Clue Array - Mission 1`))
    (:`NewEnumerator1`
      (`self.Set Up Clue Array - Mission 2`))
    (:`NewEnumerator2`
      (`self.Set Up Clue Array - Mission 3`))
    (:`NewEnumerator3`
      (`self.Set Up Clue Array - Mission 4`))
    (:`NewEnumerator4`
      (`self.Set Up Clue Array - Mission 5`))))

(event `Mark Clue For Evidence`
  (params (`Clue Name` :type Text))
  ;[1 1 1] Mark clue for evidence - Master
  (switch `/Game/GameFiles/Blueprints/Clues/MissionEnum` (`self.Mission Select`)
    (:`NewEnumerator0`
      (`self.Mark Clue For Evidence - Mission 1` `Clue Name`))
    (:`NewEnumerator1`
      (`self.Mark Clue For Evidence - Mission 2` `Clue Name`))
    (:`NewEnumerator2`
      (`self.Mark Clue For Evidence - Mission 3` `Clue Name`))
    (:`NewEnumerator3`
      (`self.Mark Clue For Evidence - Mission 4` `Clue Name`))
    (:`NewEnumerator4`
      (`self.Mark Clue For Evidence - Mission 5` `Clue Name`))))

(event `Randomly Spawn Clue 2`
  ;[1 1 1] Randomly spawn clue 2
  (bind _outactors (`GameplayStatics.GetAllActorsOfClass` "/Game/GameFiles/Blueprints/Clues/Clue2BP.Clue2BP_C"))
  (`KismetArrayLibrary.Array_Shuffle` _outactors)
  (bind _returnvalue (`KismetArrayLibrary.Array_Length` _outactors))
  (set `self.Clue 2 Total` _returnvalue)
  (for _index (range (+ (- _returnvalue 2) 1))
    (bind _output (`|GetArrayItem` _outactors _index))
    (`self.Destroy Item` (`/Game/GameFiles/Blueprints/Clues/Clue2BP.Item ID` _output))
    (`self.K2_DestroyActor` _output)
    (`/Engine/EditorBlueprintResources/StandardMacros.DecrementInt` (`self.Clue 2 Total`))))

(event `Set Up Clue Array - Mission 2`
  ;[1 1 1] Set up clue arrays - Mission 2
  (for _ (`self.Mission 2 Clues`)
    (`KismetArrayLibrary.Array_Add` (`self.Mission 2 Clues Found`)))
  ;[1 1 1] Set up clues in the game instance - Mission 2
  (bind (_clues _clues_found _pictures) (message `/Game/GameFiles/GameBlueprints/BPI_GameInstance.Get Mission 2 Clues Info` (`GameplayStatics.GetGameInstance`)))
  (for _array_element (`self.Mission 2 Clues`)
    (`KismetArrayLibrary.Array_Add` _clues _array_element))
  (for _array_element_2 (`self.Mission 2 Clues Found`)
    (`KismetArrayLibrary.Array_Add` _clues_found _array_element_2))
  (for _array_element_3 (`self.Mission 2 Clue Pictures`)
    (`KismetArrayLibrary.Array_Add` _pictures _array_element_3)))

(event `Mark Clue For Evidence - Mission 2`
  (params (`Clue Name` :type Text))
  ;[1 1 1] Mark clue as evidence - Mission 2
  (for (_array_element _array_index) (`self.Mission 2 Clues`)
    (if (`KismetTextLibrary.EqualEqual_TextText` _array_element `Clue Name`)
      (`KismetArrayLibrary.Array_Set` (`self.Mission 2 Clues Found`) _array_index true)
      ;;[1 1 1] Update game instance clues
      (bind (_clues _clues_found) (message `/Game/GameFiles/GameBlueprints/BPI_GameInstance.Get Mission 2 Clues Info` (`GameplayStatics.GetGameInstance`) :!label _label_2))
      (`KismetArrayLibrary.Array_Set` _clues_found _array_index true)
      (`self.Save Clues Found - Master`)))
  (goto _label_2))

(event `Set Up Clue Array - Mission 3`
  ;[1 1 1] Set up clue arrays - Mission 3
  (for _ (`self.Mission 3 Clues`)
    (`KismetArrayLibrary.Array_Add` (`self.Mission 3 Clues Found`)))
  ;[1 1 1] Set up clues in the game instance - Mission 3
  (bind (_clues _clues_found _pictures) (message `/Game/GameFiles/GameBlueprints/BPI_GameInstance.Get Mission 3 Clues Info` (`GameplayStatics.GetGameInstance`)))
  (for _array_element (`self.Mission 3 Clues`)
    (`KismetArrayLibrary.Array_Add` _clues _array_element))
  (for _array_element_2 (`self.Mission 3 Clues Found`)
    (`KismetArrayLibrary.Array_Add` _clues_found _array_element_2))
  (for _array_element_3 (`self.Mission 3 Clue Pictures`)
    (`KismetArrayLibrary.Array_Add` _pictures _array_element_3)))

(event `Randomly Spawn Clue 3`
  ;[1 1 1] Randomly spawn clue 3
  (bind _outactors (`GameplayStatics.GetAllActorsOfClass` "/Game/GameFiles/Blueprints/Clues/Clue3BP.Clue3BP_C"))
  (`KismetArrayLibrary.Array_Shuffle` _outactors)
  (bind _returnvalue (`KismetArrayLibrary.Array_Length` _outactors))
  (set `self.Clue 3 Total` _returnvalue)
  (for _index (range (+ (- _returnvalue 2) 1))
    (bind _output (`|GetArrayItem` _outactors _index))
    (`self.Destroy Item` (`/Game/GameFiles/Blueprints/Clues/Clue3BP.Item ID` _output))
    (`self.K2_DestroyActor` _output)
    (`/Engine/EditorBlueprintResources/StandardMacros.DecrementInt` (`self.Clue 3 Total`))))

(event `Load Clues Found - Slot 1`
  ;[1 1 1] Load clues found - Slot 1
  (switch `/Game/GameFiles/Blueprints/Clues/MissionEnum` (`self.Mission Select`)
    (:`NewEnumerator0`
      (`self.Load Clues Found - Slot 1 Mission 1`))
    (:`NewEnumerator1`
      (`self.Load Clues Found - Slot 1 Mission 2`))
    (:`NewEnumerator2`
      (`self.Load Clues Found - Slot 1 Mission 3`))
    (:`NewEnumerator3`
      (`self.Load Clues Found - Slot 1 Mission 4`))
    (:`NewEnumerator4`
      (`self.Load Clues Found - Slot 1 Mission 5`))))

(event `Set Up Clue Array - Mission 4`
  ;[1 1 1] Set up clue arrays - Mission 4
  (for _ (`self.Mission 4 Clues`)
    (`KismetArrayLibrary.Array_Add` (`self.Mission 4 Clues Found`)))
  ;[1 1 1] Set up clues in the game instance - Mission 4
  (bind (_clues _clues_found _pictures) (message `/Game/GameFiles/GameBlueprints/BPI_GameInstance.Get Mission 4 Clues Info` (`GameplayStatics.GetGameInstance`)))
  (for _array_element (`self.Mission 4 Clues`)
    (`KismetArrayLibrary.Array_Add` _clues _array_element))
  (for _array_element_2 (`self.Mission 4 Clues Found`)
    (`KismetArrayLibrary.Array_Add` _clues_found _array_element_2))
  (for _array_element_3 (`self.Mission 4 Clue Pictures`)
    (`KismetArrayLibrary.Array_Add` _pictures _array_element_3)))

(event `Save Clues Found - Master`
  ;[1 1 1] Save clues found - Master
  (bind _current_save_slot (message `/Game/GameFiles/GameBlueprints/BPI_GameInstance.Get Current Save Slot` (`GameplayStatics.GetGameInstance`)))
  (bind _output_get (set `self.Current Save Slot` _current_save_slot))
  (switch `int` (- (`KismetStringLibrary.Conv_StringToInt` (`KismetStringLibrary.GetSubstring` _output_get 4)) 1)
    (:`0`
      (`self.Save Clues Found - Slot 1`))
    (:`1`
      (`self.Save Clues Found - Slot 2`))
    (:`2`
      (`self.Save Clues Found - Slot 3`))
    (:`3`
      (`self.Save Clues Found - Slot 4`))
    (:`4`
      (`self.Save Clues Found - Slot 5`))))

(event `Randomly Spawn Clue 4`
  ;[1 1 1] Randomly spawn clue 4
  (bind _outactors (`GameplayStatics.GetAllActorsOfClass` "/Game/GameFiles/Blueprints/Clues/Clue4BP.Clue4BP_C"))
  (`KismetArrayLibrary.Array_Shuffle` _outactors)
  (bind _returnvalue (`KismetArrayLibrary.Array_Length` _outactors))
  (set `self.Clue 4 Total` _returnvalue)
  (for _index (range (+ (- _returnvalue 2) 1))
    (bind _output (`|GetArrayItem` _outactors _index))
    (`self.Destroy Item` (`/Game/GameFiles/Blueprints/Clues/Clue4BP.Item ID` _output))
    (`self.K2_DestroyActor` _output)
    (`/Engine/EditorBlueprintResources/StandardMacros.DecrementInt` (`self.Clue 4 Total`))))

(event `Mark Clue For Evidence - Mission 3`
  (params (`Clue Name` :type Text))
  ;[1 1 1] Mark clue as evidence - Mission 3
  (for (_array_element _array_index) (`self.Mission 3 Clues`)
    (if (`KismetTextLibrary.EqualEqual_TextText` _array_element `Clue Name`)
      (`KismetArrayLibrary.Array_Set` (`self.Mission 3 Clues Found`) _array_index true)
      ;;[1 1 1] Update game instance clues
      (bind (_clues _clues_found) (message `/Game/GameFiles/GameBlueprints/BPI_GameInstance.Get Mission 3 Clues Info` (`GameplayStatics.GetGameInstance`) :!label _label_3))
      (`KismetArrayLibrary.Array_Set` _clues_found _array_index true)
      (`self.Save Clues Found - Master`)))
  (goto _label_3))

(event `Set Up Clue Array - Mission 5`
  ;[1 1 1] Set up clue arrays - Mission 5
  (for _ (`self.Mission 5 Clues`)
    (`KismetArrayLibrary.Array_Add` (`self.Mission 5 Clues Found`)))
  ;[1 1 1] Set up clues in the game instance - Mission 5
  (bind (_clues _clues_found _pictures) (message `/Game/GameFiles/GameBlueprints/BPI_GameInstance.Get Mission 5 Clues Info` (`GameplayStatics.GetGameInstance`)))
  (for _array_element (`self.Mission 5 Clues`)
    (`KismetArrayLibrary.Array_Add` _clues _array_element))
  (for _array_element_2 (`self.Mission 5 Clues Found`)
    (`KismetArrayLibrary.Array_Add` _clues_found _array_element_2))
  (for _array_element_3 (`self.Mission 5 Clue Pictures`)
    (`KismetArrayLibrary.Array_Add` _pictures _array_element_3)))

(event `Load Clues Found - Slot 1 Mission 1`
  ;[1 1 1] Load clues found - Slot 1 Mission 1
  (bind _returnvalue (`GameplayStatics.LoadGameFromSlot` (`self.Current Save Slot`)))
  (bind _assave_slot_1 (cast `/Game/GameFiles/SaveGames/SaveSlot1` _returnvalue))
  (bind _output_get (set `self.Mission 1 Clues Found` (`/Game/GameFiles/SaveGames/SaveSlot1.Mission 1 Clues Found` _assave_slot_1)))
  (if (`KismetArrayLibrary.Array_IsEmpty` _output_get)
    (`self.Set Up Clues Arrays`)))

(event `Randomly Spawn Clue 5`
  ;[1 1 1] Randomly spawn clue 5
  (bind _outactors (`GameplayStatics.GetAllActorsOfClass` "/Game/GameFiles/Blueprints/Clues/Clue5BP.Clue5BP_C"))
  (`KismetArrayLibrary.Array_Shuffle` _outactors)
  (bind _returnvalue (`KismetArrayLibrary.Array_Length` _outactors))
  (set `self.Clue 5 Total` _returnvalue)
  (for _index (range (+ (- _returnvalue 2) 1))
    (bind _output (`|GetArrayItem` _outactors _index))
    (`self.Destroy Item` (`/Game/GameFiles/Blueprints/Clues/Clue5BP.Item ID` _output))
    (`self.K2_DestroyActor` _output)
    (`/Engine/EditorBlueprintResources/StandardMacros.DecrementInt` (`self.Clue 5 Total`))))

(event `Load Clues Found - Slot 1 Mission 2`
  ;[1 1 1] Load clues found - Slot 1 Mission 2
  (bind _returnvalue (`GameplayStatics.LoadGameFromSlot` (`self.Current Save Slot`)))
  (bind _assave_slot_1 (cast `/Game/GameFiles/SaveGames/SaveSlot1` _returnvalue))
  (bind _output_get (set `self.Mission 2 Clues Found` (`/Game/GameFiles/SaveGames/SaveSlot1.Mission 2 Clues Found` _assave_slot_1)))
  (if (`KismetArrayLibrary.Array_IsEmpty` _output_get)
    (`self.Set Up Clues Arrays`)))

(event `Save Clues Found - Slot 1`
  ;[1 1 1] Save clues found - Slot 1
  (switch `/Game/GameFiles/Blueprints/Clues/MissionEnum` (`self.Mission Select`)
    (:`NewEnumerator0`
      (`self.Save Clues Found - Slot 1 Mission 1`))
    (:`NewEnumerator1`
      (`self.Save Clues Found - Slot 1 Mission 2`))
    (:`NewEnumerator2`
      (`self.Save Clues Found - Slot 1 Mission 3`))
    (:`NewEnumerator3`
      (`self.Save Clues Found - Slot 1 Mission 4`))
    (:`NewEnumerator4`
      (`self.Save Clues Found - Slot 1 Mission 5`))))

(event `Save Clues Found - Slot 2`
  (switch `/Game/GameFiles/Blueprints/Clues/MissionEnum` (`self.Mission Select`)))

(event `Randomly Spawn Clue 6`
  ;[1 1 1] Randomly spawn clue 6
  (bind _outactors (`GameplayStatics.GetAllActorsOfClass` "/Game/GameFiles/Blueprints/Clues/Clue6BP.Clue6BP_C"))
  (`KismetArrayLibrary.Array_Shuffle` _outactors)
  (bind _returnvalue (`KismetArrayLibrary.Array_Length` _outactors))
  (set `self.Clue 6 Total` _returnvalue)
  (for _index (range (+ (- _returnvalue 2) 1))
    (bind _output (`|GetArrayItem` _outactors _index))
    (`self.Destroy Item` (`/Game/GameFiles/Blueprints/Clues/Clue6BP.Item ID` _output))
    (`self.K2_DestroyActor` _output)
    (`/Engine/EditorBlueprintResources/StandardMacros.DecrementInt` (`self.Clue 6 Total`))))

(event `Mark Clue For Evidence - Mission 4`
  (params (`Clue Name` :type Text))
  ;[1 1 1] Mark clue as evidence - Mission 4
  (for (_array_element _array_index) (`self.Mission 4 Clues`)
    (if (`KismetTextLibrary.EqualEqual_TextText` _array_element `Clue Name`)
      (`KismetArrayLibrary.Array_Set` (`self.Mission 4 Clues Found`) _array_index true)
      ;;[1 1 1] Update game instance clues
      (bind (_clues _clues_found) (message `/Game/GameFiles/GameBlueprints/BPI_GameInstance.Get Mission 4 Clues Info` (`GameplayStatics.GetGameInstance`) :!label _label_4))
      (`KismetArrayLibrary.Array_Set` _clues_found _array_index true)
      (`self.Save Clues Found - Master`)))
  (goto _label_4))

(event `Save Clues Found - Slot 3`)

(event `Save Clues Found - Slot 4`)

(event `Load Clues Found - Slot 1 Mission 3`
  ;[1 1 1] Load clues found - Slot 1 Mission 3
  (bind _returnvalue (`GameplayStatics.LoadGameFromSlot` (`self.Current Save Slot`)))
  (bind _assave_slot_1 (cast `/Game/GameFiles/SaveGames/SaveSlot1` _returnvalue))
  (bind _output_get (set `self.Mission 3 Clues Found` (`/Game/GameFiles/SaveGames/SaveSlot1.Mission 3 Clues Found` _assave_slot_1)))
  (if (`KismetArrayLibrary.Array_IsEmpty` _output_get)
    (`self.Set Up Clues Arrays`)))

(event `Save Clues Found - Slot 5`)

(event `Save Clues Found - Slot 1 Mission 1`
  ;[1 1 1] Save clues found - Slot 1 Mission 1
  (bind _returnvalue (`GameplayStatics.LoadGameFromSlot` (`self.Current Save Slot`)))
  (bind _assave_slot_1 (cast `/Game/GameFiles/SaveGames/SaveSlot1` _returnvalue))
  (set `/Game/GameFiles/SaveGames/SaveSlot1.Mission 1 Clues` (`self.Mission 1 Clues`) _assave_slot_1)
  (set `/Game/GameFiles/SaveGames/SaveSlot1.Mission 1 Clues Found` (`self.Mission 1 Clues Found`) _assave_slot_1)
  (set `/Game/GameFiles/SaveGames/SaveSlot1.Mission 1 Clue Pictures` (`self.Mission 1 Clue Pictures`) _assave_slot_1)
  (`GameplayStatics.SaveGameToSlot` _assave_slot_1 (`self.Current Save Slot`)))

(event `Load Clues Found - Slot 1 Mission 4`
  ;[1 1 1] Load clues found - Slot 1 Mission 4
  (bind _returnvalue (`GameplayStatics.LoadGameFromSlot` (`self.Current Save Slot`)))
  (bind _assave_slot_1 (cast `/Game/GameFiles/SaveGames/SaveSlot1` _returnvalue))
  (bind _output_get (set `self.Mission 4 Clues Found` (`/Game/GameFiles/SaveGames/SaveSlot1.Mission 4 Clues Found` _assave_slot_1)))
  (if (`KismetArrayLibrary.Array_IsEmpty` _output_get)
    (`self.Set Up Clues Arrays`)))

(event `Mark Clue For Evidence - Mission 5`
  (params (`Clue Name` :type Text))
  ;[1 1 1] Mark clue as evidence - Mission 5
  (for (_array_element _array_index) (`self.Mission 5 Clues`)
    (if (`KismetTextLibrary.EqualEqual_TextText` _array_element `Clue Name`)
      (`KismetArrayLibrary.Array_Set` (`self.Mission 5 Clues Found`) _array_index true)
      ;;[1 1 1] Update game instance clues
      (bind (_clues _clues_found) (message `/Game/GameFiles/GameBlueprints/BPI_GameInstance.Get Mission 5 Clues Info` (`GameplayStatics.GetGameInstance`) :!label _label_5))
      (`KismetArrayLibrary.Array_Set` _clues_found _array_index)
      (`self.Save Clues Found - Master`)))
  (goto _label_5))

(event `Save Clues Found - Slot 1 Mission 2`
  ;[1 1 1] Save clues found - Slot 1 Mission 2
  (bind _returnvalue (`GameplayStatics.LoadGameFromSlot` (`self.Current Save Slot`)))
  (bind _assave_slot_1 (cast `/Game/GameFiles/SaveGames/SaveSlot1` _returnvalue))
  (set `/Game/GameFiles/SaveGames/SaveSlot1.Mission 2 Clues` (`self.Mission 2 Clues`) _assave_slot_1)
  (set `/Game/GameFiles/SaveGames/SaveSlot1.Mission 2 Clues Found` (`self.Mission 2 Clues Found`) _assave_slot_1)
  (set `/Game/GameFiles/SaveGames/SaveSlot1.Mission 2 Clue Pictures` (`self.Mission 2 Clue Pictures`) _assave_slot_1)
  (`GameplayStatics.SaveGameToSlot` _assave_slot_1 (`self.Current Save Slot`)))

(event `Load Clues Found - Slot 1 Mission 5`
  ;[1 1 1] Load clues found - Slot 1 Mission 5
  (bind _returnvalue (`GameplayStatics.LoadGameFromSlot` (`self.Current Save Slot`)))
  (bind _assave_slot_1 (cast `/Game/GameFiles/SaveGames/SaveSlot1` _returnvalue))
  (bind _output_get (set `self.Mission 5 Clues Found` (`/Game/GameFiles/SaveGames/SaveSlot1.Mission 5 Clues Found` _assave_slot_1)))
  (if (`KismetArrayLibrary.Array_IsEmpty` _output_get)
    (`self.Set Up Clues Arrays`)))

(event `Save Clues Found - Slot 1 Mission 3`
  ;[1 1 1] Save clues found - Slot 1 Mission 3
  (bind _returnvalue (`GameplayStatics.LoadGameFromSlot` (`self.Current Save Slot`)))
  (bind _assave_slot_1 (cast `/Game/GameFiles/SaveGames/SaveSlot1` _returnvalue))
  (set `/Game/GameFiles/SaveGames/SaveSlot1.Mission 3 Clues` (`self.Mission 3 Clues`) _assave_slot_1)
  (set `/Game/GameFiles/SaveGames/SaveSlot1.Mission 3 Clues Found` (`self.Mission 3 Clues Found`) _assave_slot_1)
  (set `/Game/GameFiles/SaveGames/SaveSlot1.Mission 3 Clue Pictures` (`self.Mission 3 Clue Pictures`) _assave_slot_1)
  (`GameplayStatics.SaveGameToSlot` _assave_slot_1 (`self.Current Save Slot`)))

(event `Save Clues Found - Slot 1 Mission 4`
  ;[1 1 1] Save clues found - Slot 1 Mission 4
  (bind _returnvalue (`GameplayStatics.LoadGameFromSlot` (`self.Current Save Slot`)))
  (bind _assave_slot_1 (cast `/Game/GameFiles/SaveGames/SaveSlot1` _returnvalue))
  (set `/Game/GameFiles/SaveGames/SaveSlot1.Mission 4 Clues` (`self.Mission 4 Clues`) _assave_slot_1)
  (set `/Game/GameFiles/SaveGames/SaveSlot1.Mission 4 Clues Found` (`self.Mission 4 Clues Found`) _assave_slot_1)
  (set `/Game/GameFiles/SaveGames/SaveSlot1.Mission 4 Clue Pictures` (`self.Mission 4 Clue Pictures`) _assave_slot_1)
  (`GameplayStatics.SaveGameToSlot` _assave_slot_1 (`self.Current Save Slot`)))

(event `Save Clues Found - Slot 1 Mission 5`
  ;[1 1 1] Save clues found - Slot 1 Mission 5
  (bind _returnvalue (`GameplayStatics.LoadGameFromSlot` (`self.Current Save Slot`)))
  (bind _assave_slot_1 (cast `/Game/GameFiles/SaveGames/SaveSlot1` _returnvalue))
  (set `/Game/GameFiles/SaveGames/SaveSlot1.Mission 5 Clues` (`self.Mission 5 Clues`) _assave_slot_1)
  (set `/Game/GameFiles/SaveGames/SaveSlot1.Mission 5 Clues Found` (`self.Mission 5 Clues Found`) _assave_slot_1)
  (set `/Game/GameFiles/SaveGames/SaveSlot1.Mission 5 Clue Pictures` (`self.Mission 5 Clue Pictures`) _assave_slot_1)
  (`GameplayStatics.SaveGameToSlot` _assave_slot_1 (`self.Current Save Slot`)))

(fn `Check All Clues Found`
  (returns (`All Clues Found?` :type Boolean))
  (locals (`All Found?` :type Boolean :default true))
  (for _array_element (`self.Mission 1 Clues Found`)
    (if (not _array_element)
      (set `local.All Found?` false)))
  (if (`local.All Found?`)
    (for _array_element_2 (`self.Mission 2 Clues Found`)
      (if (not _array_element_2)
        (set `local.All Found?` false)))
    (if (`local.All Found?`)
      (for _array_element_3 (`self.Mission 3 Clues Found`)
        (if (not _array_element_3)
          (set `local.All Found?` false)))
      (if (`local.All Found?`)
        (for _array_element_4 (`self.Mission 4 Clues Found`)
          (if (not _array_element_4)
            (set `local.All Found?` false)))
        (if (`local.All Found?`)
          (for _array_element_5 (`self.Mission 5 Clues Found`)
            (if (not _array_element_5)
              (set `local.All Found?` false)))
          (if (`local.All Found?`)
            (return true)
            (else
              (return false)))
          (else
            (return false)))
        (else
          (return false)))
      (else
        (return false)))
    (else
      (return false))))

(fn `Check If Already Destroyed`
  (params (`Item ID` :type "Name (by ref)"))
  (returns (`Destroyed Already?` :type Boolean))
  (return (> (`KismetArrayLibrary.Array_Find` (`self.DestroyedActors`) `Item ID`) -1)))

(fn `UserConstructionScript`)