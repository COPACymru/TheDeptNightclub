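; Trigger volume that starts the nightclub final sequence cutscene when an actor tagged Player overlaps its box.
; The overlap calls PlayFinalSequenceCutscene, then hides Morgan (MaleCharacter) and Dan and disables player input on Morgan.
; It also fades out the hallway music owned by the nightclub cellar door, finding each affected actor by class lookup.
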(event `self.Box.OnComponentBeginOverlap`
  (params (OverlappedComponent :type "PrimitiveComponent Object Reference") (OtherActor :type "Actor Object Reference") (OtherComp :type "PrimitiveComponent Object Reference") (OtherBodyIndex :type Integer) (bFromSweep :type Boolean) (SweepResult :type "HitResult Structure (by ref)"))
  ;[1 1 1] Play cutscene, hide Morgan and Dan, remove player input
  (if (`self.ActorHasTag` OtherActor "Player")
    (`self.Play Final Sequence Cutscene`)
    (bind _returnvalue (`GameplayStatics.GetActorOfClass` "/Game/GameFiles/Characters/Male/MaleCharacter.MaleCharacter_C"))
    (`self.SetActorHiddenInGame` _returnvalue true)
    (`self.DisableInput` _returnvalue (`GameplayStatics.GetPlayerController` 0))
    (bind _returnvalue_2 (`GameplayStatics.GetActorOfClass` "/Game/GameFiles/Characters/Dan/BP_Dan.BP_Dan_C"))
    (`self.SetActorHiddenInGame` _returnvalue_2 true)
    (bind _returnvalue_3 (`GameplayStatics.GetActorOfClass` "/Game/GameFiles/Blueprints/Doors/BP_NightclubCellarDoor.BP_NightclubCellarDoor_C"))
    (`AudioComponent.FadeOut` (`/Game/GameFiles/Blueprints/Doors/BP_NightclubCellarDoor.HallwayMusic` _returnvalue_3) 3.0 0.0 "Linear")))

(fn `UserConstructionScript`)