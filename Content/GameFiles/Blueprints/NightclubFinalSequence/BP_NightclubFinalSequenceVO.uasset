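; BP_NightclubFinalSequenceVO is a trigger that plays a short voice-over exchange during the nightclub final sequence.
; On any Box overlap, it attaches the Hughes line to BP_Dan's mesh and shows its subtitle widget.
; Two seconds later it plays the 2D reply with a second DataTable-driven subtitle, then destroys itself.
; The overlap has no actor filter or re-entry guard.
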(event `self.Box.OnComponentBeginOverlap`
  (params (OverlappedComponent :type "PrimitiveComponent Object Reference") (OtherActor :type "Actor Object Reference") (OtherComp :type "PrimitiveComponent Object Reference") (OtherBodyIndex :type Integer) (bFromSweep :type Boolean) (SweepResult :type "HitResult Structure (by ref)"))
  (bind _returnvalue (`GameplayStatics.GetActorOfClass` "/Game/GameFiles/Characters/Dan/BP_Dan.BP_Dan_C"))
  (`GameplayStatics.SpawnSoundAttached` "/Game/GameFiles/VoiceLines/Tutorial/Hughes/English/10032024/Hughes_Charlie_Wouldntwanttogetlost_Cue.Hughes_Charlie_Wouldntwanttogetlost_Cue" (`Character.Mesh` _returnvalue) "None" (0.0 0.0 0.0) (struct) "KeepRelativeOffset" false 1.0 1.0 0.0 null null)
  (bind _returnvalue_2 (`|CreateWidget` "/Game/GameFiles/UI/Subtitles/Master/W_Subtitles.W_Subtitles_C" null (make `DataTableRowHandle` "/Game/GameFiles/UI/Subtitles/SubDT_HughesWouldntWannaGetLost_ENG.SubDT_HughesWouldntWannaGetLost_ENG" "1")))
  (`UserWidget.AddToViewport` _returnvalue_2 0)
  (`KismetSystemLibrary.Delay` 2.0)
  (`GameplayStatics.PlaySound2D` "/Game/GameFiles/VoiceLines/NewMorgan/you_can_say_that_again_Cue.you_can_say_that_again_Cue" 1.0 1.0 0.0 null null)
  (bind _returnvalue_3 (`|CreateWidget` "/Game/GameFiles/UI/Subtitles/Master/W_Subtitles.W_Subtitles_C" null (make `DataTableRowHandle` "/Game/GameFiles/UI/Subtitles/SubDT_YouCanSayThatAgain_ENG.SubDT_YouCanSayThatAgain_ENG" "1")))
  (`UserWidget.AddToViewport` _returnvalue_3 0)
  (`self.K2_DestroyActor`))

(fn `UserConstructionScript`)