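; Wall-clock style Blueprint that displays real-world time on hour, minute and second hand meshes with an audible tick.
; From BeginPlay, a one-second Delay loop reads UTC, adds an hour from April through October as approximate daylight saving, and sets each hand's roll.
; The hour hand also advances with the minutes.
; Each pass replays the audio, with a FlipFlop alternating its pitch for a tick-tock effect.
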(event `self.ReceiveBeginPlay`
  (bind (_returnvalue_year _returnvalue_month _returnvalue_day _returnvalue_hour _returnvalue_minute _returnvalue_second _returnvalue_millisecond) (`KismetMathLibrary.BreakDateTime` (`KismetMathLibrary.UtcNow`)))
  (bind (_returnvalue_year_2 _returnvalue_month_2) (`KismetMathLibrary.BreakDateTime` (`KismetMathLibrary.UtcNow`)))
  (bind _audio (`self.Audio`))
  (bind (_days _hours _minutes _seconds) (`KismetMathLibrary.BreakTimespan` (+ (`KismetMathLibrary.MakeTimespan` _returnvalue_day _returnvalue_hour _returnvalue_minute _returnvalue_second _returnvalue_millisecond) (`KismetMathLibrary.MakeTimespan` 0 (select `bool` (and (>= _returnvalue_month_2 4) (<= _returnvalue_month_2 10)) :`true` 1)))))
  (`SceneComponent.K2_SetRelativeRotation` (`self.SM_Clock_HourHand`) (`KismetMathLibrary.MakeRotator` (* (+ (* _hours 30.0) (/ (`KismetMathLibrary.Conv_IntToDouble` _minutes) 2.0)) -1.0)) false false :!label _label)
  (`SceneComponent.K2_SetRelativeRotation` (`self.SM_Clock_MinuteHand`) (`KismetMathLibrary.MakeRotator` (* _minutes -6.0)) false false)
  (`SceneComponent.K2_SetRelativeRotation` (`self.SM_Clock_SecondHand`) (`KismetMathLibrary.MakeRotator` (* _seconds -6.0)) false false)
  (`AudioComponent.Play` _audio 0.0)
  (`/Engine/EditorBlueprintResources/StandardMacros.FlipFlop`
    (:`A`
      (`AudioComponent.SetPitchMultiplier` _audio 1.25))
    (:`B`
      (`AudioComponent.SetPitchMultiplier` _audio 1.0)))
  (`KismetSystemLibrary.Delay` 1.0)
  (goto _label))

(fn `UserConstructionScript`)